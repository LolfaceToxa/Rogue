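; Replicated component that makes its owning actor hoverable and clickable, with a custom-depth outline and key-helper prompts that flag chests as containers.
; It binds cursor events on the owner's sphere component and updates prompts through BP_CombatPlayerActions.
; Mouse hover applies when unblocked or the inventory is open, while separate HoverStart/HoverEnd events serve third person.
; Clicking only toggles Selected, as the material color swap is unused.
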(event Custom|OnMouseHoverStart
  (params (TouchedComponent :type Primitive%20Component%20Object%20Reference))
  (bind _playeractions (Variables|Default|GetPlayerActions))
  (bind _playerkeyhelpers (Variables|/Game/Rogue/Blueprints/Core/Player/BP_CombatPlayerActions.BP_CombatPlayerActions_C|GetPlayerKeyHelpers _playeractions))
  (if (or (not (Variables|Default|GetMouseHoverBlocked?)) (Variables|Default|GetInvOpened?))
    (Rendering|SetRenderCustomDepth (Variables|Default|GetStaticMeshRef) true) ; outline around an object
    (Utilities|Casting|CastToBP_Chest (Components|GetOwner)
      (:then
        (Default|UpdateKeyHelpers _playerkeyhelpers true true true false))
      (:CastFailed
        (Default|UpdateKeyHelpers _playerkeyhelpers true false true false)))))

(event Custom|HoverStart
  (bind _playeractions (Variables|Default|GetPlayerActions))
  (bind _playerkeyhelpers (Variables|/Game/Rogue/Blueprints/Core/Player/BP_CombatPlayerActions.BP_CombatPlayerActions_C|GetPlayerKeyHelpers _playeractions))
  (Rendering|SetRenderCustomDepth (Variables|Default|GetStaticMeshRef) true) ; outline around an object
  (Utilities|Casting|CastToBP_Chest (Components|GetOwner)
    (:then
      (Default|UpdateKeyHelpers _playerkeyhelpers true true true false))
    (:CastFailed
      (Default|UpdateKeyHelpers _playerkeyhelpers true false true false))))

(event Custom|HoverEnd
  (Rendering|SetRenderCustomDepth (Variables|Default|GetStaticMeshRef) false) ; outline around an object
  (Default|UpdateKeyHelpers (Variables|/Game/Rogue/Blueprints/Core/Player/BP_CombatPlayerActions.BP_CombatPlayerActions_C|GetPlayerKeyHelpers (Variables|Default|GetPlayerActions)) false false true false))

(event Custom|OnMouseHoverEnd
  (params (TouchedComponent :type Primitive%20Component%20Object%20Reference))
  (if (or (not (Variables|Default|GetMouseHoverBlocked?)) (Variables|Default|GetInvOpened?))
    (Rendering|SetRenderCustomDepth (Variables|Default|GetStaticMeshRef) false) ; outline around an object
    (Default|UpdateKeyHelpers (Variables|/Game/Rogue/Blueprints/Core/Player/BP_CombatPlayerActions.BP_CombatPlayerActions_C|GetPlayerKeyHelpers (Variables|Default|GetPlayerActions)) false false true false)))

(event Custom|OnClicked
  (params (TouchedComponent :type Primitive%20Component%20Object%20Reference) (ButtonPressed :type Key%20Structure :default "None"))
  (bind _output_get (Variables|Default|SetSelected? (not (Variables|Default|GetSelected?)))))

(event EventBeginPlay
  (bind _returnvalue (Components|GetOwner))
  (Class|ActorComponent|SetIsReplicated true)
  (Variables|Default|SetStaticMeshRef (Actor|GetComponentbyClass _returnvalue "/Script/Engine.StaticMeshComponent"))
  (bind _assphere_collision (Utilities|Casting|CastToSphereComponent (Actor|GetComponentbyClass _returnvalue "/Script/Engine.SphereComponent")))
  (EventDispatchers|BindEventtoOnBeginCursorOver _assphere_collision (EventDispatchers|CreateEvent :!event Custom|OnMouseHoverStart))
  (EventDispatchers|BindEventtoOnEndCursorOver _assphere_collision (EventDispatchers|CreateEvent :!event Custom|OnMouseHoverEnd))
  (EventDispatchers|BindEventtoOnClicked _assphere_collision (EventDispatchers|CreateEvent :!event Custom|OnClicked))
  (bind _returnvalue_2 (Actor|GetActorOfClass "/Game/Rogue/Blueprints/Core/Player/BP_CombatPlayerActions.BP_CombatPlayerActions_C"))
  (Variables|Default|SetPlayerActions _returnvalue_2))