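; BP_Chest is a container actor with its own BPC inventory that opens and closes the container menu by click or forced third-person call.
; Opening closes any previous container, registers this inventory with the player, shows it and updates key hints.
; Clicks respect interaction range; the looping timer for auto-closing on distance is left unwired.
; Closing resets TouchCollision responses after a tiny delay so overlaps refresh.
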(event Custom|Event_OnChestOpened
  ;[1 1 1] Open/Close Chest
  (if (Variables|/Game/Inventory/BPC_Inventory.BPC_Inventory_C|GetNeedToUseInteractionRange? (Variables|Default|GetBPC_Inventory))
    _
    (else
      _))
  (bind _returnvalue (Actor|GetActorOfClass "/Game/Rogue/Blueprints/Core/Player/BP_PlayerActions.BP_PlayerActions_C"))
  (bind _playerinventory (Class|BPIInventoryPlayer|GetPlayerInventoryRef(Message) _returnvalue))
  (Default|UpdateKeyHelpers (Variables|/Game/Inventory/BPC_Inventory.BPC_Inventory_C|GetHUD _playerinventory) true true true false) ; bottom left corner keys
)

(event Custom|Event_OnClicked
  (params (TouchedActor :type Actor%20Object%20Reference) (ButtonPressed :type Key%20Structure :default "None"))
  ;[1 1 1] Open/Close Chest
  (bind _returnvalue (Actor|GetActorOfClass "/Game/Rogue/Blueprints/Core/Player/BP_PlayerActions.BP_PlayerActions_C"))
  (bind _playerinventory (Class|BPIInventoryPlayer|GetPlayerInventoryRef(Message) _returnvalue))
  (if (Variables|/Game/Inventory/UI/WB_PlayerInventoryHUD.WB_PlayerInventoryHUD_C|GetPlayerMenuIsContainer? (Variables|/Game/Inventory/BPC_Inventory.BPC_Inventory_C|GetHUD (Variables|Default|GetBPC_Inventory)))
    (Default|DestroyPlayerMenu (Variables|/Game/Inventory/BPC_Inventory.BPC_Inventory_C|GetHUD (Variables|Default|GetBPC_Inventory)))
    (Utilities|Time|ClearandInvalidateTimerbyHandle (Variables|InnerUsage|GetPlayerFarTimer))
    (CallFunction|ReInitChestCollision)
    (elif (or (Variables|/Game/Inventory/BPC_Inventory.BPC_Inventory_C|GetisTopDown? _playerinventory) (Variables|/Game/Inventory/BPC_Inventory.BPC_Inventory_C|GetisInventoryVisible? _playerinventory))
      (if (CallFunction|CanCharacterInteractwithItem (Variables|/Game/Inventory/BPC_Inventory.BPC_Inventory_C|GetInteractionRange (Variables|Default|GetBPC_Inventory)) (Utilities|GetPlayerLocation) (Transformation|GetActorLocation TouchedActor))
        (Utilities|IsValid (Variables|Default|GetBPC_Inventory)
          (:Is%20Valid
            (Utilities|FlowControl|Sequence
              (:then_0
                (bind _returnvalue_2 (Actor|GetActorOfClass "/Game/Rogue/Blueprints/Core/Player/BP_PlayerActions.BP_PlayerActions_C"))
                (bind _playerinventory_2 (Class|BPIInventoryPlayer|GetPlayerInventoryRef(Message) _returnvalue_2)) ; Close old before opening new(nesessary because there can be two chests)
                (Utilities|IsValid (Variables|/Game/Inventory/BPC_Inventory.BPC_Inventory_C|GetContainer%20Inventory%20Ref _playerinventory_2)
                  (:Is%20Valid
                    (Default|OnInventoryClosedEvent (Variables|/Game/Inventory/BPC_Inventory.BPC_Inventory_C|GetContainer%20Inventory%20Ref _playerinventory_2)))
                  (:Is%20Not%20Valid
                    _))
                (Variables|/Game/Inventory/BPC_Inventory.BPC_Inventory_C|SetContainer%20Inventory%20Ref _playerinventory_2 (Variables|Default|GetBPC_Inventory)) ; Each chest has its own inventory, so we update this value
              )
              (:then_1
                (Default|ShowContainer (Variables|/Game/Inventory/BPC_Inventory.BPC_Inventory_C|GetHUD (Variables|Default|GetBPC_Inventory)) (Variables|Default|GetBPC_Inventory))
                (Utilities|FlowControl|Sequence
                  (:then_0
                    (if (Variables|/Game/Inventory/BPC_Inventory.BPC_Inventory_C|GetNeedToUseInteractionRange? (Variables|Default|GetBPC_Inventory))
                      (EventDispatchers|BindEventtoPlayerMenuDestroyed (Variables|/Game/Inventory/BPC_Inventory.BPC_Inventory_C|GetHUD (Variables|Default|GetBPC_Inventory)) (EventDispatchers|CreateEvent :!event Custom|Event_OnMenuDestroyed)) ; If interaction range is enabled then we check how far player is from chest to close chest menu
                    ))
                  (:then_1
                    (Default|CallOnChestOpened) ; Trigger event in BPC_Inventory
                  ))))))))))

(event Custom|Event_OnMenuDestroyed
  ;[1 1 1] Open/Close Chest
  (Utilities|Time|ClearandInvalidateTimerbyHandle (Variables|InnerUsage|GetPlayerFarTimer))
  (bind _returnvalue (Actor|GetActorOfClass "/Game/Rogue/Blueprints/Core/Player/BP_PlayerActions.BP_PlayerActions_C"))
  (bind _playerinventory (Class|BPIInventoryPlayer|GetPlayerInventoryRef(Message) _returnvalue))
  (Variables|/Game/Inventory/BPC_Inventory.BPC_Inventory_C|SetisInventoryVisible? _playerinventory false))

(event Custom|Is%20Player%20Far%20From%20Chest
  (bind _bpc_inventory (Variables|Default|GetBPC_Inventory))
  ;[1 1 1] Open/Close Chest
  (if (Variables|/Game/Inventory/BPC_Inventory.BPC_Inventory_C|GetNeedToUseInteractionRange? _bpc_inventory)
    (if (not (CallFunction|CanCharacterInteractwithItem (Variables|/Game/Inventory/BPC_Inventory.BPC_Inventory_C|GetInteractionRange _bpc_inventory) (Utilities|GetPlayerLocation) (Transformation|GetActorLocation)))
      (Default|DestroyPlayerMenu (Variables|/Game/Inventory/BPC_Inventory.BPC_Inventory_C|GetHUD (Variables|Default|GetBPC_Inventory)))
      (Utilities|Time|ClearandInvalidateTimerbyHandle (Variables|InnerUsage|GetPlayerFarTimer))
      (bind _returnvalue (Actor|GetActorOfClass "/Game/Rogue/Blueprints/Core/Player/BP_PlayerActions.BP_PlayerActions_C"))
      (bind _playerinventory (Class|BPIInventoryPlayer|GetPlayerInventoryRef(Message) _returnvalue))
      (Variables|/Game/Inventory/BPC_Inventory.BPC_Inventory_C|SetisInventoryVisible? _playerinventory false))))

(event Custom|OpenChestForce
  ;[1 1 1] Open/Close Chest
  (bind _returnvalue (Actor|GetActorOfClass "/Game/Rogue/Blueprints/Core/Player/BP_PlayerActions.BP_PlayerActions_C"))
  (bind _playerinventory (Class|BPIInventoryPlayer|GetPlayerInventoryRef(Message) _returnvalue))
  (if (Variables|/Game/Inventory/UI/WB_PlayerInventoryHUD.WB_PlayerInventoryHUD_C|GetPlayerMenuIsContainer? (Variables|/Game/Inventory/BPC_Inventory.BPC_Inventory_C|GetHUD _playerinventory))
    (Default|DestroyPlayerMenu (Variables|/Game/Inventory/BPC_Inventory.BPC_Inventory_C|GetHUD (Variables|Default|GetBPC_Inventory)))
    (Utilities|Time|ClearandInvalidateTimerbyHandle (Variables|InnerUsage|GetPlayerFarTimer))
    (CallFunction|ReInitChestCollision)
    (else
      (Variables|InnerUsage|SetChestOpenedForce? true)
      (Utilities|IsValid (Variables|Default|GetBPC_Inventory)
        (:Is%20Valid
          (Utilities|FlowControl|Sequence
            (:then_0
              (bind _returnvalue_2 (Actor|GetActorOfClass "/Game/Rogue/Blueprints/Core/Player/BP_PlayerActions.BP_PlayerActions_C"))
              (bind _playerinventory_2 (Class|BPIInventoryPlayer|GetPlayerInventoryRef(Message) _returnvalue_2)) ; Close old before opening new(nesessary because there can be two chests)
              (Utilities|IsValid (Variables|/Game/Inventory/BPC_Inventory.BPC_Inventory_C|GetContainer%20Inventory%20Ref _playerinventory_2)
                (:Is%20Valid
                  (Default|OnInventoryClosedEvent (Variables|/Game/Inventory/BPC_Inventory.BPC_Inventory_C|GetContainer%20Inventory%20Ref _playerinventory_2)))
                (:Is%20Not%20Valid
                  _))
              (Variables|/Game/Inventory/BPC_Inventory.BPC_Inventory_C|SetContainer%20Inventory%20Ref _playerinventory_2 (Variables|Default|GetBPC_Inventory)) ; Each chest has its own inventory, so we update this value
            )
            (:then_1
              (Default|ShowContainer (Variables|/Game/Inventory/BPC_Inventory.BPC_Inventory_C|GetHUD (Variables|Default|GetBPC_Inventory)) (Variables|Default|GetBPC_Inventory))
              (Utilities|FlowControl|Sequence
                (:then_0
                  (if (Variables|/Game/Inventory/BPC_Inventory.BPC_Inventory_C|GetNeedToUseInteractionRange? (Variables|Default|GetBPC_Inventory))
                    (EventDispatchers|BindEventtoPlayerMenuDestroyed (Variables|/Game/Inventory/BPC_Inventory.BPC_Inventory_C|GetHUD (Variables|Default|GetBPC_Inventory)) (EventDispatchers|CreateEvent :!event Custom|Event_OnMenuDestroyed)) ; If interaction range is enabled then we check how far player is from chest to close chest menu
                  ))
                (:then_1
                  (Default|CallOnChestOpened) ; Trigger event in BPC_Inventory
                )))))))))

(event Custom|ReInitChestCollision
  (bind _touchcollision (Variables|Default|GetTouchCollision))
  ;[0.7792 0.638 0] Collision update
  (Collision|SetCollisionResponsetoAllChannels _touchcollision "ECR_Ignore")
  (Utilities|FlowControl|Delay 0.0001)
  (Collision|SetCollisionResponsetoChannel _touchcollision "ECC_Visibility" "ECR_Block")
  (Collision|SetCollisionResponsetoChannel _touchcollision "ECC_WorldStatic" "ECR_Overlap"))

(event EventBeginPlay
  ;[0.0298 0 1] Begin Play
  (EventDispatchers|BindEventtoOnClicked (EventDispatchers|CreateEvent :!event Custom|Event_OnClicked))
  (EventDispatchers|BindEventtoOnChestOpened (EventDispatchers|CreateEvent :!event Custom|Event_OnChestOpened)))

(fn ConstructionScript)

(fn CanCharacterInteractwithItem
  (params (InteractDistance :type Float%20%28double-precision%29) (Player%20Location :type Vector) (Item%20Location :type Vector))
  (return (<= (Math|Vector|VectorLength (- Player%20Location Item%20Location)) InteractDistance)))