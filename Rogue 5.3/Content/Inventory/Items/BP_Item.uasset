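; BP_Item is a world pickup for the inventory system, holding a DT_Item row ID and quantity.
; Cursor or player-gaze hover shows its name and selects it in the player's inventory component, so a key press can take it.
; A drag function line-traces the mouse to move it within range or takes it into the player or container grid under the cursor.
; The event nodes starting that timer-driven drag are disconnected.
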(event OnBeginCursorOver(TouchCollision)
  (params (TouchedComponent :type Primitive%20Component%20Object%20Reference))
  ;[1 1 1] Item interaction
  (bind _returnvalue (Actor|GetActorOfClass "/Game/Rogue/Blueprints/Core/Player/BP_PlayerActions.BP_PlayerActions_C"))
  (bind _playerinventory (Default|GetPlayerInventoryRef _returnvalue))
  (bind _output_get (Variables|Default|SetInvRef _playerinventory))
  (Utilities|IsValid _output_get
    (:Is%20Valid
      (bind _returnvalue_2 (Utilities|GetDataTableRow "/Game/Inventory/DT_Item.DT_Item" (.RowName (Utilities|Struct|BreakDataTableRowHandle (Variables|SettingsSetByBPCInventory|GetItemID))))
        (:then
          (Default|ShowMessage (Variables|/Game/Inventory/BPC_Inventory.BPC_Inventory_C|GetItemInfoMenu (Variables|Default|GetInvRef)) (Utilities|Text|ToText(String) (Utilities|String|EnumtoString (.Name (Utilities|Struct|BreakS_Item _returnvalue_2))))) ; Bottom middle item title
        )
        (:RowNotFound
          _))
      (Variables|InnerUsage|SetItemHovered? true)
      (Class|BPIInventoryItem|SelectItem(Message) (Variables|Default|GetInvRef) self (.RowName (Utilities|Struct|BreakDataTableRowHandle (Variables|SettingsSetByBPCInventory|GetItemID))) (Variables|SettingsSetbyBPCInventory|GetQuantity)) ; If item is hovered then it's selected and we let BPC_Inventory know about current selected item
    )))

(event OnEndCursorOver(TouchCollision)
  (params (TouchedComponent :type Primitive%20Component%20Object%20Reference))
  ;[1 1 1] Item interaction
  (bind _returnvalue (Actor|GetActorOfClass "/Game/Rogue/Blueprints/Core/Player/BP_PlayerActions.BP_PlayerActions_C"))
  (bind _playerinventory (Default|GetPlayerInventoryRef _returnvalue))
  (Variables|Default|SetInvRef _playerinventory)
  (Variables|InnerUsage|SetItemHovered? false)
  (if (not (Variables|InnerUsage|GetInItemDrag?))
    (bind _invref (Variables|Default|GetInvRef)
      (:then
        (bind _iteminfomenu (Variables|/Game/Inventory/BPC_Inventory.BPC_Inventory_C|GetItemInfoMenu _invref)
          (:then
            (Default|ShowMessage _iteminfomenu) ; Hide middle item title
          )
          (:else
            _))
        (Class|BPIInventoryItem|SelectItem(Message) (Variables|Default|GetInvRef) 0 "None") ; Don't have current selected item
      )
      (:else))))

(event OnClicked(TouchCollision)
  (params (TouchedComponent :type Primitive%20Component%20Object%20Reference) (ButtonPressed :type Key%20Structure))
  ;[1 1 1] Item interaction
)

(event OnReleased(TouchCollision)
  (params (TouchedComponent :type Primitive%20Component%20Object%20Reference) (ButtonReleased :type Key%20Structure))
  ;[1 1 1] Item interaction
)

(event Custom|TakeItemIntoInventory_ByKey
  (bind _invref (Variables|Default|GetInvRef))
  ;[1 1 1] Take by key
  (if (Variables|InnerUsage|GetItemHovered?)
    (Utilities|IsValid _invref
      (:Is%20Valid
        (Class|BPIInventoryItem|TakeUpItem(Message) _invref))
      (:Is%20Not%20Valid
        (Development|PrintString "Error: No inventory reference" true true "(R=1.000000,G=0.000000,B=0.031627,A=1.000000)")))))

(event Custom|OnEndPlayerGazeOver
  ;[1 1 1] Item interaction
  (Variables|InnerUsage|SetItemHovered? false)
  (if (not (Variables|InnerUsage|GetInItemDrag?))
    (bind _invref (Variables|Default|GetInvRef)
      (:then
        (bind _iteminfomenu (Variables|/Game/Inventory/BPC_Inventory.BPC_Inventory_C|GetItemInfoMenu _invref)
          (:then
            (Default|ShowMessage _iteminfomenu) ; Hide middle item title
          )
          (:else
            _))
        (Class|BPIInventoryItem|SelectItem(Message) (Variables|Default|GetInvRef) 0 "None") ; Don't have current selected item
      )
      (:else))))

(event Custom|InItemInteraction
  ;[1 1 1] Item interaction
)

(event Custom|OnBeginPlayerGazeOver
  ;[1 1 1] Item interaction
  (Utilities|IsValid (stale OnBeginCursorOver(TouchCollision) _output_get)
    (:Is%20Valid
      (bind _returnvalue (Utilities|GetDataTableRow "/Game/Inventory/DT_Item.DT_Item" (.RowName (Utilities|Struct|BreakDataTableRowHandle (Variables|SettingsSetByBPCInventory|GetItemID))))
        (:then
          (Default|ShowMessage (Variables|/Game/Inventory/BPC_Inventory.BPC_Inventory_C|GetItemInfoMenu (Variables|Default|GetInvRef)) (Utilities|Text|ToText(String) (Utilities|String|EnumtoString (.Name (Utilities|Struct|BreakS_Item _returnvalue))))) ; Bottom middle item title
        )
        (:RowNotFound
          _))
      (Variables|InnerUsage|SetItemHovered? true)
      (Class|BPIInventoryItem|SelectItem(Message) (Variables|Default|GetInvRef) self (.RowName (Utilities|Struct|BreakDataTableRowHandle (Variables|SettingsSetByBPCInventory|GetItemID))) (Variables|SettingsSetbyBPCInventory|GetQuantity)) ; If item is hovered then it's selected and we let BPC_Inventory know about current selected item
    )))

(event Custom|OnMouseReleased
  (params (Force? :type Boolean))
  ;[1 1 1] Item interaction
)

(event Custom|ReInitItemCollision
  (bind _touchcollision (Variables|Default|GetTouchCollision))
  ;[0.7792 0.638 0] Collision update
  (Collision|SetCollisionResponsetoAllChannels _touchcollision "ECR_Ignore")
  (Utilities|FlowControl|Delay 0.0001)
  (Collision|SetCollisionResponsetoChannel _touchcollision "ECC_Visibility" "ECR_Block")
  (Collision|SetCollisionResponsetoChannel _touchcollision "ECC_WorldStatic" "ECR_Overlap"))

(event EventBeginPlay
  (bind _returnvalue (Actor|GetActorOfClass "/Game/Rogue/Blueprints/Core/Player/BP_PlayerActions.BP_PlayerActions_C"))
  (bind _playerinventory (Default|GetPlayerInventoryRef _returnvalue))
  (Variables|Default|SetInvRef _playerinventory))

(fn ConstructionScript)

(fn SetItemLocationtoMouseLocation
  (bind _returnvalue (Game|GetPlayerController 0))
  (bind _invref (Variables|Default|GetInvRef))
  (bind _invref_2 (Variables|Default|GetInvRef))
  (bind _invref_3 (Variables|Default|GetInvRef))
  (bind _invref_4 (Variables|Default|GetInvRef))
  (bind _returnvalue_2 (Components|GetOwner _invref))
  (bind (_worldlocation _worlddirection) (Game|Player|ConvertMouseLocationToWorldSpace _returnvalue))
  (bind _container_inventory_ref (Variables|/Game/Inventory/BPC_Inventory.BPC_Inventory_C|GetContainer%20Inventory%20Ref _invref_3))
  (Utilities|IsValid _container_inventory_ref
    (:Is%20Valid
      (bind _playermenu (Variables|/Game/Inventory/UI/WB_PlayerHUD.WB_PlayerHUD_C|GetPlayerMenu (Variables|/Game/Inventory/BPC_Inventory.BPC_Inventory_C|GetHUD _container_inventory_ref))
        (:then
          (bind _aswb_container_inventory (Utilities|Casting|CastToWB_ContainerInventory _playermenu) ; Chest opened
            (:then
              (if (Utilities|GetMouseUnderUI (Variables|/Game/Inventory/UI/WB_ContainerInventory.WB_ContainerInventory_C|GetWB_InventoryGrid_Chest _aswb_container_inventory)) ; Above chest ui?
                (Utilities|FlowControl|DoOnce false :!label _label
                  (:Completed
                    (bind _success_ (CallFunction|TakeItemIntoInventory (Variables|/Game/Inventory/BPC_Inventory.BPC_Inventory_C|GetContainer%20Inventory%20Ref _invref_4)))
                    (if _success_
                      (CallFunction|OnMouseReleased false)
                      (else
                        (goto _label Reset)))))
                (elif (Utilities|GetMouseUnderUI (Variables|/Game/Inventory/UI/WB_ContainerInventory.WB_ContainerInventory_C|GetWB_InventoryGrid_Player _aswb_container_inventory)) ; Above player ui?
                  (Utilities|FlowControl|DoOnce false :!label _label_2
                    (:Completed
                      (bind _success__2 (CallFunction|TakeItemIntoInventory _invref_4))
                      (if _success__2
                        (CallFunction|OnMouseReleased false)
                        (else
                          (goto _label_2 Reset)))))
                  (else
                    (bind _playermenu_2 (Variables|/Game/Inventory/UI/WB_PlayerHUD.WB_PlayerHUD_C|GetPlayerMenu (Variables|/Game/Inventory/BPC_Inventory.BPC_Inventory_C|GetHUD _invref_3) :!label _label_3)
                      (:then
                        (bind _aswb_player_menu (Utilities|Casting|CastToWB_PlayerMenu _playermenu_2) ; Player inv opened
                          (:then
                            (if (Utilities|GetMouseUnderUI (Variables|/Game/Inventory/UI/WB_PlayerMenu.WB_PlayerMenu_C|GetWB_InventoryGrid _aswb_player_menu)) ; Above player ui?
                              (goto _label_2)
                              (else
                                _)))
                          (:CastFailed
                            _)))
                      (:else
                        _))
                    (if (or (Variables|/Game/Inventory/BPC_Inventory.BPC_Inventory_C|GetisTopDown? _invref_2) (Variables|/Game/Inventory/BPC_Inventory.BPC_Inventory_C|GetisInventoryVisible? _invref_2)) :!label _label_4 ; Drop item in the world
                      (bind (_outhit _returnvalue_3) (Collision|LineTraceForObjects _worldlocation (+ _worldlocation (* _worlddirection 10000)) (Utilities|Array|MakeArray "ObjectTypeQuery1") false 0 "None"))
                      (if _returnvalue_3
                        (if (Variables|/Game/Inventory/BPC_Inventory.BPC_Inventory_C|GetNeedToUseInteractionRange? (Variables|Default|GetInvRef))
                          (if (CallFunction|CanCharacterInteractwithItem (Variables|SettingssetbyBPC_Inventory|GetInteraction%20Range) (Utilities|GetPlayerLocation) (+ (* (.Normal (Collision|BreakHitResult _outhit)) 3e+01) (.Location (Collision|BreakHitResult _outhit))))
                            (Transformation|SetActorLocation (+ (* (.Normal (Collision|BreakHitResult _outhit)) 3e+01) (.Location (Collision|BreakHitResult _outhit))) false true :!label _label_5)
                            (CallFunction|InItemInteraction)
                            (else
                              (CallFunction|OnMouseReleased false) ; If item too far then just leave it on the last place where it was interactable
                            ))
                          (else
                            (goto _label_5))))
                      (else
                        (Transformation|SetActorLocation (+ (Transformation|GetActorLocation _returnvalue_2) (* (Transformation|GetActorForwardVector _returnvalue_2) 100)) false true)
                        (Variables|/Game/Inventory/BPC_Inventory.BPC_Inventory_C|SetSelectedItem (Variables|Default|GetInvRef) self)
                        (CallFunction|InItemInteraction)))))))
            (:CastFailed
              (goto _label_4))))
        (:else
          (goto _label_4))))
    (:Is%20Not%20Valid
      (goto _label_3))))

(fn CanCharacterInteractwithItem
  (params (InteractDistance :type Float%20%28double-precision%29) (Player%20Location :type Vector) (Item%20Location :type Vector))
  (return (<= (Math|Vector|VectorLength (- Player%20Location Item%20Location)) InteractDistance)))

(fn TakeItemIntoInventory
  (params (TakeIntoInvRef :type BPC%20Inventory%20Object%20Reference))
  (Utilities|IsValid TakeIntoInvRef
    (:Is%20Valid
      (Class|BPIInventoryItem|SelectItem(Message) TakeIntoInvRef self (.RowName (Utilities|Struct|BreakDataTableRowHandle (Variables|SettingsSetByBPCInventory|GetItemID))) (Variables|SettingsSetbyBPCInventory|GetQuantity)) ; Select item then take it
      (Class|BPIInventoryItem|TakeUpItem(Message) TakeIntoInvRef)
      (return true))
    (:Is%20Not%20Valid
      (Development|PrintString "Error in BP_Item->TakeItemIntoInventory: No inventory reference" true true "(R=1.000000,G=0.000000,B=0.031627,A=1.000000)")
      (return false))))