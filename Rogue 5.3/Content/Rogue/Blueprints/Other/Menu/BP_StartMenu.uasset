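; Start menu controller that loads or creates the "save1" save and spawns all menu widgets, most hidden until shown.
; A looping Delay chain streams L_Square in and out as backdrop while toggling the start widget's background.
; Inspect events swap hover item and talent tooltips for pinned, focusable versions, closing them when toggled again.
; Helpers award achievements with XP, notification and save, and return unlocked items and tier-filtered talents.
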(event Custom|CloseFullItemFocused
  (bind _fulliteminfo_focused (Variables|UI|GetFullItemInfo_Focused) ; Close old one
    (:then
      (Widget|RemovefromParent _fulliteminfo_focused)
      (Variables|UI|SetFullItemInfo_Focused 0)
      (Variables|Default|SetTooltipFocused? false))
    (:else
      (Variables|Default|SetTooltipFocused? false))))

(event Custom|Event_InspectItem
  (if (Variables|Default|GetTooltipActive?)
    (if (Variables|Default|GetTooltipFocused?)
      (bind _fulliteminfo_focused (Variables|UI|GetFullItemInfo_Focused) ; Close old one
        (:then
          (Widget|RemovefromParent _fulliteminfo_focused)
          (Variables|UI|SetFullItemInfo_Focused 0)
          (Variables|Default|SetTooltipFocused? false))
        (:else
          (Variables|Default|SetTooltipFocused? false)))
      (else
        (bind _fulliteminforef (Variables|UI|GetFullItemInfoRef) ; Close not fixed full item info
          (:then
            (Widget|RemovefromParent _fulliteminforef)
            (Variables|UI|SetFullItemInfoRef 0))
          (:else
            _))
        (bind _returnvalue (Game|ConstructObjectfromClass "/Game/Inventory/UI/WB_FullItemInfo_Menu_Focused.WB_FullItemInfo_Menu_Focused_C" (Variables|Default|GetSlot_ItemID)))
        (bind _output_get (Variables|UI|SetFullItemInfo_Focused _returnvalue))
        (UserInterface|Viewport|AddtoViewport _output_get 0)
        (Variables|Default|SetTooltipFocused? true)))))

(event Custom|Event_InspectTalent
  (if (Variables|Default|GetTooltipActive?)
    (if (Variables|Default|GetTooltipFocused?)
      (bind _talentinfomenufocused (Variables|UI|GetTalentInfoMenuFocused) ; Close old one
        (:then
          (Widget|RemovefromParent _talentinfomenufocused)
          (Variables|UI|SetTalentInfoMenuFocused 0)
          (Variables|Default|SetTooltipFocused? false))
        (:else
          (Variables|Default|SetTooltipFocused? false)))
      (else
        (bind _talentinfomenu (Variables|UI|GetTalentInfoMenu) ; Close not fixed full item info
          (:then
            (Widget|RemovefromParent _talentinfomenu)
            (Variables|UI|SetTalentInfoMenu 0))
          (:else
            _))
        (bind _returnvalue (Game|ConstructObjectfromClass "/Game/Rogue/Blueprints/Core/TalentSystem/W_TalentInfoMenu_Focused.W_TalentInfoMenu_Focused_C" (Variables|Default|GetTalentID)))
        (bind _output_get (Variables|UI|SetTalentInfoMenuFocused _returnvalue))
        (UserInterface|Viewport|AddtoViewport _output_get 0)
        (Variables|Default|SetTooltipFocused? true)))))

(event Custom|CloseTalentTooltipFocused
  (bind _talentinfomenufocused (Variables|UI|GetTalentInfoMenuFocused) ; Close old one
    (:then
      (Widget|RemovefromParent _talentinfomenufocused)
      (Variables|UI|SetTalentInfoMenuFocused 0)
      (Variables|Default|SetTooltipFocused? false))
    (:else
      (Variables|Default|SetTooltipFocused? false))))

(event EventBeginPlay
  (bind _self self)
  (Utilities|FlowControl|Sequence
    (:then_0
      (bind _returnvalue (SaveGame|DoesSaveGameExist "save1"))
      (if _returnvalue
        (bind _returnvalue_2 (SaveGame|LoadGamefromSlot "save1"))
        (bind _asbp_save (Utilities|Casting|CastToBP_Save _returnvalue_2))
        (Variables|Default|SetBP%20Save _asbp_save)
        (else
          (bind _returnvalue_3 (SaveGame|CreateSaveGameObject "/Game/Rogue/Blueprints/SaveLoad/BP_Save.BP_Save_C"))
          (Variables|/Game/Rogue/Blueprints/SaveLoad/BP_Save.BP_Save_C|SetScore _returnvalue_3 (Utilities|Struct|MakeIntPoint 0 0))
          (Variables|/Game/Rogue/Blueprints/SaveLoad/BP_Save.BP_Save_C|SetPlayerExp _returnvalue_3 0)
          (SaveGame|SaveGametoSlot _returnvalue_3 "save1")
          (Variables|Default|SetBP%20Save _returnvalue_3))))
    (:then_1
      (bind _returnvalue_4 (Game|ConstructObjectfromClass "/Game/Rogue/Blueprints/Other/Menu/W_StartMenu.W_StartMenu_C" self))
      (bind _output_get (Variables|UI|SetW_StartMenu _returnvalue_4))
      (UserInterface|Viewport|AddtoViewport _output_get 0)
      (Game|LoadStreamLevel(byName) "L_Square" true :!label _label)
      (Default|EventShowBackground (Variables|UI|GetW_StartMenu))
      (Utilities|FlowControl|Delay 1e+01)
      (Default|EventHideBackground (Variables|UI|GetW_StartMenu))
      (Utilities|FlowControl|Delay 5.0)
      (Game|UnloadStreamLevel(byName) "L_Square" false)
      (goto _label))
    (:then_2
      (Utilities|FlowControl|Sequence
        (:then_0
          (bind _returnvalue_5 (Game|ConstructObjectfromClass "/Game/Rogue/Blueprints/Other/Menu/W_Meta.W_Meta_C" _self))
          (bind _output_get_2 (Variables|UI|SetW_Meta _returnvalue_5))
          (UserInterface|Viewport|AddtoViewport _output_get_2 0)
          (Widget|SetVisibility _output_get_2 "Hidden"))
        (:then_1
          (bind _returnvalue_6 (Game|ConstructObjectfromClass "/Game/Rogue/Blueprints/Other/Menu/W_BeforePlay.W_BeforePlay_C" _self))
          (bind _output_get_3 (Variables|UI|SetBeforePlayMenu _returnvalue_6))
          (UserInterface|Viewport|AddtoViewport _output_get_3 0)
          (Widget|SetVisibility _output_get_3 "Hidden"))
        (:then_2
          (bind _returnvalue_7 (Game|ConstructObjectfromClass "/Game/Rogue/Blueprints/Other/Menu/W_NotifyMenu.W_NotifyMenu_C"))
          (bind _output_get_4 (Variables|UI|SetNotifyMenu _returnvalue_7))
          (UserInterface|Viewport|AddtoViewport _output_get_4 0)
          (Variables|/Game/Rogue/Blueprints/Other/Menu/W_NotifyMenu.W_NotifyMenu_C|SetVisible? _output_get_4 true))
        (:then_3
          (Class|SimplyConfigSettings|LoadSimplySettings)
          (bind _returnvalue_8 (Game|ConstructObjectfromClass "/SimplySettings/UI_SettingsWidget.UI_SettingsWidget_C" self))
          (UserInterface|Viewport|AddtoViewport _returnvalue_8 0)
          (bind _output_get_5 (Variables|UI|SetW_Settings _returnvalue_8))
          (Widget|SetVisibility _output_get_5 "Hidden"))
        (:then_4
          (bind _returnvalue_9 (Game|ConstructObjectfromClass "/Game/Rogue/Blueprints/Other/Menu/W_Collection.W_Collection_C" _self))
          (bind _output_get_6 (Variables|UI|SetCollectionMenu _returnvalue_9))
          (UserInterface|Viewport|AddtoViewport _output_get_6 0)
          (Widget|SetVisibility _output_get_6 "Hidden"))
        (:then_5
          (bind _returnvalue_10 (Game|ConstructObjectfromClass "/Game/Rogue/Blueprints/Other/Menu/W_Background.W_Background_C" _self))
          (UserInterface|Viewport|AddtoViewport _returnvalue_10 0))
        (:then_6
          (bind _returnvalue_11 (Game|ConstructObjectfromClass "/Game/Rogue/Blueprints/Other/Menu/W_Collection_Items.W_Collection_Items_C" self))
          (bind _output_get_7 (Variables|UI|SetCollection_Items _returnvalue_11))
          (UserInterface|Viewport|AddtoViewport _output_get_7 0)
          (Widget|SetVisibility _output_get_7 "Hidden"))
        (:then_7
          (bind _returnvalue_12 (Game|ConstructObjectfromClass "/Game/Rogue/Blueprints/Core/TalentSystem/W_TalentMenu_OnlyWatch.W_TalentMenu_OnlyWatch_C" self))
          (bind _output_get_8 (Variables|UI|SetTalentMenu _returnvalue_12))
          (UserInterface|Viewport|AddtoViewport _output_get_8 0)
          (Widget|SetVisibility _output_get_8 "Hidden"))
        (:then_8
          (bind _returnvalue_13 (Game|ConstructObjectfromClass "/Game/Rogue/Blueprints/Other/Menu/W_Collection_Companions.W_Collection_Companions_C" self))
          (bind _output_get_9 (Variables|UI|SetCompanionsMenu _returnvalue_13))
          (UserInterface|Viewport|AddtoViewport _output_get_9 0)
          (Widget|SetVisibility _output_get_9 "Hidden"))))
    (:then_3
      (bind _returnvalue_14 (Actor|GetActorOfClass "/Game/Rogue/Blueprints/Core/Player/RoguePawn.RoguePawn_C"))
      (Variables|UI|SetPlayer _returnvalue_14))))

(event EventOnOtherMenuOpened
  (Widget|SetVisibility (Variables|UI|GetW_StartMenu) "Hidden")
  (Utilities|FlowControl|Sequence
    (:then_0
      (Utilities|IsValid (Variables|UI|GetFullItemInfo_Focused)
        (:Is%20Valid
          (Widget|RemovefromParent (Variables|UI|GetFullItemInfo_Focused))
          (Variables|UI|SetFullItemInfo_Focused 0))))
    (:then_1
      (Utilities|IsValid (Variables|UI|GetFullItemInfoRef)
        (:Is%20Valid
          (Widget|RemovefromParent (Variables|UI|GetFullItemInfoRef))
          (Variables|UI|SetFullItemInfoRef 0))))))

(fn ConstructionScript)

(fn AddXP
  (params (XP :type Integer))
  (bind _bp_save (Variables|Default|GetBP%20Save))
  (Variables|/Game/Rogue/Blueprints/SaveLoad/BP_Save.BP_Save_C|SetPlayerExp _bp_save (+ XP (Variables|/Game/Rogue/Blueprints/SaveLoad/BP_Save.BP_Save_C|GetPlayerExp _bp_save))))

(fn CheckandAddAchievment
  (params (New%20Achievment :type E_Achievment%20Enum :default "NewEnumerator10"))
  (bind _bp_save (Variables|Default|GetBP%20Save))
  (bind _achievments (Variables|/Game/Rogue/Blueprints/SaveLoad/BP_Save.BP_Save_C|GetAchievments _bp_save))
  (if (not (Utilities|Array|ContainsItem _achievments New%20Achievment))
    (Utilities|Array|Add _achievments New%20Achievment)
    (bind _returnvalue (Utilities|GetDataTableRow "/Game/Rogue/Blueprints/Core/AchievmentSystem/DT_Achievments.DT_Achievments" (Utilities|Name|EnumtoName New%20Achievment))
      (:then
        (CallFunction|AddXP (.XP_Value (Utilities|Struct|BreakS_Achievment _returnvalue)))
        (bind _returnvalue_2 (Game|ConstructObjectfromClass "/Game/Rogue/Blueprints/Core/AchievmentSystem/W_AchievmentCompleted.W_AchievmentCompleted_C" New%20Achievment))
        (Widget|Panel|AddChild (Variables|/Game/Rogue/Blueprints/Other/Menu/W_NotifyMenu.W_NotifyMenu_C|GetVB_Notifies (Variables|UI|GetNotifyMenu)) _returnvalue_2)
        (Default|PlayAnim _returnvalue_2)
        (Utilities|SaveGame)))))

(fn GetAvailableTalents
  (bind _outrownames (DataTable|GetDataTableRowNames "/Game/Rogue/Blueprints/Core/TalentSystem/DT_Talents.DT_Talents"))
  (for _array_element _outrownames
    (bind _returnvalue (Utilities|GetDataTableRow "/Game/Rogue/Blueprints/Core/TalentSystem/DT_Talents.DT_Talents" _array_element)
      (:then
        (if (<= (.TalentTier (Utilities|Struct|BreakS_TalentInfo _returnvalue)) (+ (Variables|/Game/Rogue/Blueprints/SaveLoad/BP_Save.BP_Save_C|GetTierUpgrades (Variables|Default|GetBP%20Save)) 2))
          (Utilities|Array|Add (LocalVariables|GetTalentsArray) (.Talent (Utilities|Struct|BreakS_TalentInfo _returnvalue)))))))
  (return (LocalVariables|GetTalentsArray)))

(fn GetAvailableItemsSorted
  (return (Variables|/Game/Rogue/Blueprints/SaveLoad/BP_Save.BP_Save_C|GetItemsUnlocked (Variables|Default|GetBP%20Save))))