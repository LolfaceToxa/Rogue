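; Level-placed combat scenario that quick-starts a grid battle and handles its outcome.
; Construction script previews the grid and maps units to tiles outside gameplay.
; BeginPlay builds teams from TeamIndex or actor names, gives non-zero teams to AI, scatters random lava, acid and trees (modifiers argument unused), then starts CombatSystem.
; Combat end updates or clears the rogue map, saves on some branches, and opens the adventure, combat or menu level.
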(event Custom|OnCombatEnded
  (bind _array (Utilities|Array|MakeArray))
  (bind _array_2 (Utilities|Array|MakeArray))
  (bind _array_3 (Utilities|Array|MakeArray))
  (bind _combatsystem (Variables|Default|GetCombatSystem))
  (bind _playeractions (Variables|Default|GetPlayerActions))
  (bind _playeractions_2 (Variables|Default|GetPlayerActions))
  (bind _s_roguemap (Utilities|Struct|MakeS_RogueMap _array_2 _array_3 _array))
  (bind _invholder (Variables|/Game/Rogue/Blueprints/Core/Player/BP_CombatPlayerActions.BP_CombatPlayerActions_C|GetInvHolder _playeractions))
  (bind _invholder_2 (Variables|/Game/Rogue/Blueprints/Core/Player/BP_CombatPlayerActions.BP_CombatPlayerActions_C|GetInvHolder _playeractions_2))
  (bind _bp_save (Variables|/Game/Rogue/Blueprints/Core/Player/BP_PlayerInventoryHolder.BP_PlayerInventoryHolder_C|GetBP%20Save _invholder_2))
  (if (== (Variables|/Game/Rogue/Blueprints/Core/Combat/BP_CombatSystem.BP_CombatSystem_C|GetObjectThatStartedCombat (Variables|Default|GetCombatSystem)) self)
    (if (Variables|/Game/Rogue/Blueprints/Core/Player/BP_CombatPlayerActions.BP_CombatPlayerActions_C|GetEncounterType? (Variables|Default|GetPlayerActions))
      (if (== (Variables|/Game/Rogue/Blueprints/Other/Menu/W_Menu_InCombat.W_Menu_InCombat_C|GetWinningTeamIndex (Variables|/Game/Rogue/Blueprints/Core/Player/BP_CombatPlayerActions.BP_CombatPlayerActions_C|GetMainMenu (Variables|Default|GetPlayerActions))) 0)
        (Variables|/Game/Rogue/Blueprints/Core/Player/RogueGameInstance.RogueGameInstance_C|SetRogueMap (Variables|/Game/Rogue/Blueprints/Core/Player/BP_CombatPlayerActions.BP_CombatPlayerActions_C|GetAs%20Rogue%20Game%20Instance _playeractions_2) (Variables|/Game/Rogue/Blueprints/Core/Player/BP_PlayerInventoryHolder.BP_PlayerInventoryHolder_C|GetRogueMap _invholder_2)) ; Win
        (Variables|/Game/Rogue/Blueprints/SaveLoad/BP_Save.BP_Save_C|SetRogueMap _bp_save (Variables|/Game/Rogue/Blueprints/Core/Player/BP_PlayerInventoryHolder.BP_PlayerInventoryHolder_C|GetRogueMap _invholder_2))
        (Game|OpenLevel(byName) "L_Adventure")
        (else
          (Variables|/Game/Rogue/Blueprints/Core/Player/RogueGameInstance.RogueGameInstance_C|SetRogueMap (Variables|/Game/Rogue/Blueprints/Core/Player/BP_CombatPlayerActions.BP_CombatPlayerActions_C|GetAs%20Rogue%20Game%20Instance (Variables|Default|GetPlayerActions)) _s_roguemap) ; Lose
          (Variables|/Game/Rogue/Blueprints/SaveLoad/BP_Save.BP_Save_C|SetRogueMap _bp_save _s_roguemap)
          (Utilities|SaveGame)
          (Game|OpenLevel(byName) "L_MainMenu")))
      (elif (Variables|/Game/Rogue/Blueprints/Core/Combat/BP_CombatSystem.BP_CombatSystem_C|GetContinueCombat? _combatsystem)
        (Variables|/Game/Rogue/Blueprints/Core/Combat/BP_CombatSystem.BP_CombatSystem_C|SetContinueCombat? _combatsystem false)
        (Game|OpenLevel(byName) "L_Combat_01_A")
        (else
          (Variables|/Game/Rogue/Blueprints/Core/Player/RogueGameInstance.RogueGameInstance_C|SetRogueMap (Variables|/Game/Rogue/Blueprints/Core/Player/BP_CombatPlayerActions.BP_CombatPlayerActions_C|GetAs%20Rogue%20Game%20Instance _playeractions) (Variables|/Game/Rogue/Blueprints/Core/Player/BP_PlayerInventoryHolder.BP_PlayerInventoryHolder_C|GetRogueMap _invholder))
          (Variables|/Game/Rogue/Blueprints/SaveLoad/BP_Save.BP_Save_C|SetRogueMap (Variables|/Game/Rogue/Blueprints/Core/Player/BP_PlayerInventoryHolder.BP_PlayerInventoryHolder_C|GetBP%20Save _invholder) (Variables|/Game/Rogue/Blueprints/Core/Player/BP_PlayerInventoryHolder.BP_PlayerInventoryHolder_C|GetRogueMap _invholder))
          (Utilities|SaveGame)
          (Game|OpenLevel(byName) "L_MainMenu"))))))

(event EventBeginPlay
  (Utilities|FlowControl|Delay 0.0001)
  (CallFunction|BuildTeamsBasedonUnitNames)
  (CallFunction|BuildAIListBasedonTeamIndexes)
  (Utilities|FlowControl|Delay 0.001)
  (EventDispatchers|BindEventtoOnCombatEnded (Variables|Default|GetCombatSystem) (delegate Custom|OnCombatEnded))
  (bind _returnvalue (Actor|GetActorOfClass "/Game/Rogue/Blueprints/Core/Grid/BP_Grid.BP_Grid_C"))
  (Variables|Default|SetGrid _returnvalue)
  (Utilities|FlowControl|Sequence
    (:then_0
      (bind _returnvalue_2 (Actor|GetActorOfClass "/Game/Rogue/Blueprints/Core/Player/BP_CombatPlayerActions.BP_CombatPlayerActions_C"))
      (Variables|Default|SetPlayerActions _returnvalue_2))
    (:then_1
      (CallFunction|SpawnModifierObstacles (.CombatModifiers (Utilities|Struct|BreakS_CombatScene (Variables|/Game/Rogue/Blueprints/Core/Player/RogueGameInstance.RogueGameInstance_C|GetNextEncounter (Variables|/Game/Rogue/Blueprints/Core/Player/BP_CombatPlayerActions.BP_CombatPlayerActions_C|GetAs%20Rogue%20Game%20Instance (Variables|Default|GetPlayerActions))))))
      (Default|QuickStartCombat (Variables|Default|GetCombatSystem) (Variables|Default|GetGridData) (Variables|Default|GetUnitsData) self))))

(fn ConstructionScript
  (if (not (CallFunction|IsinGame))
    (Utilities|Struct|SetmembersinS_QuickCombat_Grid (Variables|Default|GetGridData) (Transformation|GetActorLocation))
    (CallFunction|SpawnGrid)
    (CallFunction|BuildDesiredGridIndexesBasedonUnitLocations)))

(fn BuildTeamsBasedonUnitNames
  (bind _outactors (Actor|GetAllActorsOfClass "/Game/Rogue/Blueprints/Core/Units/BP_Unit.BP_Unit_C"))
  (for _array_element _outactors
    (bind _output_get (LocalVariables|SetCurUnit _array_element))
    (if (Variables|/Game/Rogue/Blueprints/Core/Units/BP_Unit.BP_Unit_C|GetSpawnedByLevel? _output_get)
      (LocalVariables|SetTeamIndex (Variables|/Game/Rogue/Blueprints/Core/Units/BP_Unit.BP_Unit_C|GetTeamIndex _output_get))
      (else
        (LocalVariables|SetTeamIndex (Math|Conversions|ToInteger(Byte) (.LeftS (Utilities|String|Split (.RightS (Utilities|String|Split (Utilities|GetDisplayName (LocalVariables|GetCurUnit)) "Team")) "_"))))))
    (if (< (Utilities|Array|Length (LocalVariables|GetUnitsTeams)) (+ (LocalVariables|GetTeamIndex) 1)) ; Is array too small
      (Utilities|Array|Resize (LocalVariables|GetUnitsTeams) (+ (LocalVariables|GetTeamIndex) 1)))
    (Utilities|Array|Add (Utilities|Struct|BreakS_UnitArray (Utilities|Array|Get(acopy) (LocalVariables|GetUnitsTeams) (LocalVariables|GetTeamIndex))) (LocalVariables|GetCurUnit)))
  (Utilities|Array|RemoveItem :TargetArray (LocalVariables|GetUnitsTeams)) ; Remove empty groups
  (Utilities|Struct|SetmembersinS_QuickCombat_UnitTeams (Variables|Default|GetUnitsData) (LocalVariables|GetUnitsTeams)))

(fn BuildAIListBasedonTeamIndexes
  (for (_array_element _array_index) (.UnitTeams (Utilities|Struct|BreakS_QuickCombat_UnitTeams (Variables|Default|GetUnitsData)))
    (if (!= _array_index 0) ; AI Only Enemies and Summons
      (Utilities|Array|AppendArray (LocalVariables|GetAIs) (Utilities|Struct|BreakS_UnitArray _array_element))))
  (Utilities|Struct|SetmembersinS_QuickCombat_UnitTeams (Variables|Default|GetUnitsData) (LocalVariables|GetAIs)))

(fn BuildDesiredGridIndexesBasedonUnitLocations
  (for _array_element (.UnitTeams (Utilities|Struct|BreakS_QuickCombat_UnitTeams (Variables|Default|GetUnitsData)))
    (for _array_element_2 (Utilities|Struct|BreakS_UnitArray _array_element)
      (bind _index (Default|GetTileIndexfromWorldLoc (Variables|/Game/Rogue/Blueprints/Core/Combat/BP_CombatSystem.BP_CombatSystem_C|GetGrid (Variables|Default|GetCombatSystem)) (Transformation|GetActorLocation _array_element_2)))
      (Utilities|Map|Add (LocalVariables|GetDesIndexes) _array_element_2 _index)))
  (Utilities|Struct|SetmembersinS_QuickCombat_UnitTeams (Variables|Default|GetUnitsData) (LocalVariables|GetDesIndexes)))

(fn SpawnGrid
  (bind _combatsystem (Variables|Default|GetCombatSystem))
  (bind _griddata (Variables|Default|GetGridData))
  (bind (_generategridbeforestartingcombat _centerlocation _tilesize _tilecount _shape _useenvironment) (Utilities|Struct|BreakS_QuickCombat_Grid _griddata))
  (bind _grid (Variables|/Game/Rogue/Blueprints/Core/Combat/BP_CombatSystem.BP_CombatSystem_C|GetGrid _combatsystem))
  (Utilities|IsValid _combatsystem
    (:Is%20Valid
      (Utilities|IsValid _grid
        (:Is%20Valid
          (Default|SpawnGrid _grid _centerlocation _tilesize (Math|Conversions|ToVector2D(IntPoint) _tilecount) _shape _useenvironment))))))

(fn SpawnModifierObstacles
  (params (Modifiers :type Array%20of%20E_CombatModifier%20Enums :default "NewEnumerator0"))
  (bind _returnvalue (Transformation|GetActorLocation))
  (bind _grid (Variables|Default|GetGrid))
  (bind _griddata (Variables|Default|GetGridData))
  (bind _tilesforspawning (LocalVariables|GetTilesForSpawning))
  (bind _grid_2 (Variables|Default|GetGrid))
  (bind (_generategridbeforestartingcombat _centerlocation _tilesize _tilecount) (Utilities|Struct|BreakS_QuickCombat_Grid _griddata))
  (bind (_x _y) (Math|Vector|BreakVector _returnvalue))
  (bind _gridbottomleftcornerlocation (Variables|/Game/Rogue/Blueprints/Core/Grid/BP_Grid.BP_Grid_C|GetGridBottomLeftCornerLocation _grid_2))
  (bind (_x_2 _y_2) (Utilities|Struct|BreakIntPoint _tilecount))
  (bind (_x_3 _y_3) (Math|Vector|BreakVector _tilesize))
  (bind (_x_4 _y_4 _z) (Math|Vector|BreakVector _gridbottomleftcornerlocation))
  (Utilities|FlowControl|Sequence
    (:then_0
      (bind _keys (Utilities|Map|Keys (Variables|/Game/Rogue/Blueprints/Core/Grid/BP_Grid.BP_Grid_C|GetGrid%20Tiles _grid)))
      (for _array_element _keys
        (if (Default|IsTileWalkable _grid _array_element)
          (Utilities|Array|Add (LocalVariables|GetTilesForSpawning) _array_element))))
    (:then_1
      (for _index (range 0 10)
        (bind _output_get (LocalVariables|SetCurrentActorToSpawn (.OutItem (Utilities|Array|Random (Utilities|Array|MakeArray "/Game/Rogue/LevelObjects/BP_Lava.BP_Lava_C" "/Game/Rogue/LevelObjects/BP_Acid.BP_Acid_C" "/Game/Rogue/LevelObjects/BP_Tree.BP_Tree_C")))))
        (if (== _output_get "/Game/Rogue/LevelObjects/BP_Tree.BP_Tree_C")
          (if (> (Utilities|Array|Length _tilesforspawning) 0)
            (bind _output_get_2 (LocalVariables|SetCurrentTile (.OutItem (Utilities|Array|Random _tilesforspawning))))
            (Utilities|Array|RemoveItem _tilesforspawning _output_get_2)
            (LocalVariables|SetCurrentTreeSize (Math|Random|RandomFloatinRange 0.6 0.9))
            (bind _returnvalue_2 (Game|SpawnActorfromClass "/Game/Rogue/LevelObjects/BP_Tree.BP_Tree_C" (Math|Transform|MakeTransform (Default|GetTileLocation (Variables|Default|GetGrid) _output_get_2) "0, 0, 0" (Math|Vector|MakeVector (LocalVariables|GetCurrentTreeSize) (LocalVariables|GetCurrentTreeSize) (LocalVariables|GetCurrentTreeSize))) "AdjustIfPossibleButDontSpawnIfColliding" "MultiplyWithRoot" 0 "NewEnumerator0" "NewEnumerator2" false 0))
            (Utilities|IsValid _returnvalue_2
              (:Is%20Valid
                (Transformation|SetActorLocation (Math|Vector|MakeVector _x _y (+ (.Z (Math|Vector|BreakVector (Variables|/Game/Rogue/Blueprints/Core/Grid/BP_Grid.BP_Grid_C|GetGridBottomLeftCornerLocation (Variables|Default|GetGrid)))) 1.0)) false false)
                (Transformation|SetRelativeRotation (Variables|/Game/Rogue/LevelObjects/BP_Tree.BP_Tree_C|GetStaticMesh _returnvalue_2) (Math|Rotator|MakeRotator 0.0 0.0 (Math|Random|RandomFloatinRange -45.0 135.0)) false false))))
          (else
            (bind _returnvalue_3 (Game|SpawnActorfromClass (LocalVariables|GetCurrentActorToSpawn) (Math|Transform|MakeTransform (Math|Vector|MakeVector (Math|Random|RandomFloatinRange (+ _x_4 3e+01) (+ (* (* _x_2 _x_3) 0.9) _x_4)) (Math|Random|RandomFloatinRange (+ _y_4 3e+01) (+ (* (* _y_2 _y_3) 0.9) _y_4)) (+ _z 5.0)) (Math|Rotator|SelectRotator (Math|Rotator|MakeRotator 0.0 0.0 0.0) (Math|Rotator|MakeRotator 0.0 0.0 9e+01) (Math|Random|RandomBool))) "AdjustIfPossibleButDontSpawnIfColliding" "MultiplyWithRoot" 0 0))
            (Utilities|IsValid _returnvalue_3
              (:Is%20Valid
                (Transformation|SetActorLocation _returnvalue_3 (Math|Vector|MakeVector (.X (Math|Vector|BreakVector (Transformation|GetActorLocation _returnvalue_3))) (.Y (Math|Vector|BreakVector (Transformation|GetActorLocation _returnvalue_3))) (+ (.Z (Math|Vector|BreakVector (Variables|/Game/Rogue/Blueprints/Core/Grid/BP_Grid.BP_Grid_C|GetGridBottomLeftCornerLocation (Variables|Default|GetGrid)))) 5.0)) false false)))))))))