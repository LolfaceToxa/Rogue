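; Deprecated overworld scenario actor that organizes placed BP_Unit actors into numbered groups and flags encounters; its BeginPlay does nothing.
; BuildGroupsBasedOnUnitNames rebuilds the UnitGroups map by parsing each unit's display name for the number after "Group" and an "_AI" encounter marker.
; Disconnected logic that never runs would add a back-to-menu widget, set unit contexts, and register groups and encounter flags with BP_OverworldUnitGroupsManager.
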(event EventBeginPlay)

(fn ConstructionScript)

(fn BuildGroupsBasedonUnitNames
  (Utilities|Map|Clear (Variables|Default|GetUnitGroups))
  (bind _outactors (Actor|GetAllActorsOfClass "/Game/Rogue/Blueprints/Core/Units/BP_Unit.BP_Unit_C"))
  (for _array_element _outactors
    (bind _output_get (LocalVariables|SetCurUnit _array_element))
    (LocalVariables|SetGroupID (Math|Conversions|ToInteger(Byte) (.LeftS (Utilities|String|Split (.RightS (Utilities|String|Split (Utilities|GetDisplayName _output_get) "Group")) "_"))))
    (LocalVariables|SetIsEncounter (Utilities|String|Contains (Utilities|GetDisplayName (LocalVariables|GetCurUnit)) "_AI"))
    (LocalVariables|SetGroup (.Value (Utilities|Map|Find (Variables|Default|GetUnitGroups) (LocalVariables|GetGroupID))))
    (Utilities|Struct|SetmembersinS_OverworldUnitGroup (LocalVariables|GetGroup) (LocalVariables|GetGroupID) (LocalVariables|GetIsEncounter))
    (Utilities|Array|AddUnique (.Units (Utilities|Struct|BreakS_OverworldUnitGroup (LocalVariables|GetGroup))) (LocalVariables|GetCurUnit))
    (Utilities|Map|Add (Variables|Default|GetUnitGroups) (LocalVariables|GetGroupID) (LocalVariables|GetGroup))))