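; BP_GridVisual renders the game grid as instanced tiles, with a flat view for walkable tiles and a toggleable tactical view colored by tile type.
; Two child BP_GridMeshInst actors take meshes from the grid's shape data and are updated per tile.
; Tactical tiles stretch in height from the lowest tracked Z and regenerate lazily when that view is enabled, which also hides actors tagged NotTactical.
; Helpers set or clear an attacked state on tiles.
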(event EventBeginPlay
  (Actor|Tick|SetActorTickEnabled false))

(fn ConstructionScript)

(fn InitGridVisual
  (params (Grid :type BP%20Grid%20Object%20Reference))
  (Variables|Default|SetGrid Grid)
  (Variables|Default|SetGridMeshInst (.AsBP%20Grid%20Mesh%20Inst (Utilities|Casting|CastToBP_GridMeshInst (Variables|/Script/Engine.ChildActorComponent|GetChildActor (Variables|Default|GetChildActor_GridMeshInst)))))
  (Variables|Default|SetGridMeshInst_Tactical (.AsBP%20Grid%20Mesh%20Inst (Utilities|Casting|CastToBP_GridMeshInst (Variables|/Script/Engine.ChildActorComponent|GetChildActor (Variables|Default|GetChildActor_GridMeshInst_Tactical)))))
  (Default|InitGridMeshInst (Variables|Default|GetGridMeshInst) (.FlatMesh (Utilities|Struct|BreakS_GridShapeData (Default|GetCurrentShapeData (Variables|Default|GetGrid)))) (.FlatMaterial (Utilities|Struct|BreakS_GridShapeData (Default|GetCurrentShapeData (Variables|Default|GetGrid)))) false "QueryOnly")
  (Default|InitGridMeshInst (Variables|Default|GetGridMeshInst_Tactical) (.Mesh (Utilities|Struct|BreakS_GridShapeData (Default|GetCurrentShapeData (Variables|Default|GetGrid)))) (.Material (Utilities|Struct|BreakS_GridShapeData (Default|GetCurrentShapeData (Variables|Default|GetGrid)))) true "QueryOnly")
  (Transformation|SetActorLocation "0, 0, 0" false false) ; Center grid in world
  (CallFunction|SetOffsetfromGround (Variables|Default|GetOffset%20from%20Ground))
  (CallFunction|SetGridLowestZ 999999.0)
  (CallFunction|SetIsTactical (Variables|Default|GetIsTactical)))

(fn SetOffsetfromGround
  (params (OffsetFromGround :type Float%20%28double-precision%29))
  (Variables|Default|SetOffset%20from%20Ground OffsetFromGround)
  (Transformation|SetRelativeLocation (Variables|Default|GetChildActor_GridMeshInst) (Math|Vector|MakeVector 0.0 0.0 (Variables|Default|GetOffset%20from%20Ground)) false false))

(fn DestroyGridVisual
  (bind _gridmeshinst (Variables|Default|GetGridMeshInst))
  (bind _gridmeshinst_tactical (Variables|Default|GetGridMeshInst_Tactical))
  (Utilities|FlowControl|Sequence
    (:then_0
      (Utilities|IsValid _gridmeshinst
        (:Is%20Valid
          (Default|ClearInstances _gridmeshinst))))
    (:then_1
      (Utilities|IsValid _gridmeshinst_tactical
        (:Is%20Valid
          (Default|ClearInstances _gridmeshinst_tactical))))
    (:then_2
      (CallFunction|SetGridLowestZ 999999.0))))

(fn UpdateTileVisual
  (params (Data :type S%20Tile%20Data%20F%20Structure))
  (Utilities|FlowControl|Sequence
    (:then_0
      (Default|RemoveInstance (Variables|Default|GetGridMeshInst) (.index Data))
      (if (CallFunction|IsTileTypeWalkable (.type Data))
        (Default|AddInstance (Variables|Default|GetGridMeshInst) (.transform Data) (.index Data) (.states Data) (.type Data))))
    (:then_1
      (CallFunction|UpdateTileVisualTactical Data))))

(fn UpdateTileVisualTactical
  (params (Data :type S%20Tile%20Data%20F%20Structure))
  (bind _grid (Variables|Default|GetGrid))
  (bind (_location _rotation _scale) (Math|Transform|BreakTransform (.transform Data)))
  (bind _location_2 (Math|Transform|BreakTransform (.transform Data)))
  (bind _returnvalue (Default|GetCurrentShapeData _grid))
  (bind _meshsize (Utilities|Struct|BreakS_GridShapeData _returnvalue))
  (bind _z (Math|Vector|BreakVector _meshsize))
  (Utilities|FlowControl|Sequence
    (:then_0
      (if (< (.z _location_2) (Variables|Default|GetGridLowestZ))
        (CallFunction|SetGridLowestZ (.z _location_2))))
    (:then_1
      (if (Variables|Default|GetIsTactical)
        (Default|RemoveInstance (Variables|Default|GetGridMeshInst_Tactical) (.index Data))
        (if (Utilities|Enum|NotEqual(Enum) (.type Data) "NewEnumerator0")
          (Default|AddInstance (Variables|Default|GetGridMeshInst_Tactical) (Math|Transform|MakeTransform _location _rotation (Math|Vector|MakeVector (.x _scale) (.y _scale) (/ (+ (- (.Z (Math|Vector|BreakVector (.Location (Math|Transform|BreakTransform (.transform Data))))) (Variables|Default|GetGridLowestZ)) _z) _z))) (.index Data) (.states Data) (.type Data)))
        (else
          (Variables|Default|SetNeedToRegenerateTacticalOnNextEnable true))))))

(fn SetGridLowestZ
  (params (Z :type Float%20%28double-precision%29))
  (Variables|Default|SetGridLowestZ Z)
  (Variables|Default|SetNeedToRegenerateTacticalOnNextEnable true))

(fn SetIsTactical
  (params (Tactical :type Boolean))
  (bind _gridmeshinst_tactical (Variables|Default|GetGridMeshInst_Tactical))
  (bind _grid (Variables|Default|GetGrid))
  (Variables|Default|SetIsTactical Tactical)
  (Development|SetHiddeninGame (Variables|Default|GetChildActor_GridMeshInst_Tactical) (not (Variables|Default|GetIsTactical)) false)
  (bind _outactors (Actor|GetAllActorswithTag "NotTactical"))
  (for _array_element _outactors
    (Rendering|SetActorHiddenInGame _array_element (Variables|Default|GetIsTactical)))
  (Utilities|FlowControl|Sequence
    (:then_0
      (if (and (Variables|Default|GetIsTactical) (Variables|Default|GetNeedToRegenerateTacticalOnNextEnable))
        (Variables|Default|SetNeedToRegenerateTacticalOnNextEnable false)
        (Utilities|IsValid _grid
          (:Is%20Valid
            (bind _values (Utilities|Map|Values (Variables|/Game/Rogue/Blueprints/Core/Grid/BP_Grid.BP_Grid_C|GetGrid%20Tiles _grid)))
            (for _array_element_2 _values
              (CallFunction|UpdateTileVisualTactical _array_element_2))))))
    (:then_1
      (Utilities|IsValid _gridmeshinst_tactical
        (:Is%20Valid
          (Collision|SetCollisionEnabled (Variables|/Game/Rogue/Blueprints/Core/Grid/Utilities/BP_GridMeshInst.BP_GridMeshInst_C|GetInstancedStaticMesh _gridmeshinst_tactical) (select (Variables|Default|GetIsTactical) "QueryOnly" "NoCollision")))))))

(fn SetTilesAttacked
  (params (Indexes :type Array%20of%20Int%20Point%20Structures))
  (for _array_element Indexes
    (Default|AddStatetoTile (Variables|Default|GetGrid) _array_element "NewEnumerator10")))

(fn RemoveTilesAttacked
  (params (Indexes :type Array%20of%20Int%20Point%20Structures))
  (for _array_element Indexes
    (Default|RemoveStatefromTile (Variables|Default|GetGrid) _array_element "NewEnumerator10")))

(fn UnionArray
  (params (Array1 :type Array%20of%20E_TileState%20Enums :default "NewEnumerator0") (Array2 :type Array%20of%20E_TileState%20Enums :default "NewEnumerator0"))
  (bind _combined (LocalVariables|GetCombined))
  (for _array_element Array1
    (Utilities|Array|AddUnique _combined _array_element))
  (for _array_element_2 Array2
    (Utilities|Array|AddUnique _combined _array_element_2))
  (return (LocalVariables|GetCombined)))

(fn RemovefromArray
  (params (ArrayFrom :type Array%20of%20E_TileState%20Enums :default "NewEnumerator0") (ArrayRemove :type Array%20of%20E_TileState%20Enums :default "NewEnumerator0"))
  (bind _removed (LocalVariables|GetRemoved))
  (for _array_element ArrayFrom
    (Utilities|Array|AddUnique _removed _array_element))
  (for _array_element_2 ArrayRemove
    (Utilities|Array|RemoveItem _removed _array_element_2))
  (return (LocalVariables|GetRemoved)))