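; Ranger unit AI Blueprint that adjusts movement logic based on whether the unit has cast a damaging spell this turn.
; It flags damage when a cast spell's minimum HP modifier is negative, clearing the flag as each AI turn starts.
; Movement uses a random pick between two logic options once flagged, otherwise a fixed default.
; A turn counter resets at combat start but feeds only unused logic.
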(event EventBeginPlay
  (|CallParentFunction) ; This node is disabled and will not be called.\nDrag off pins to build functionality.
)

(event EventCastSpell
  (bind _spelldata (CallFunction|GetSpellDatafromSpell (.Spell (Utilities|Struct|BreakS_UnitAISpellCastData (Variables|Default|GetAISpellCast))) (Variables|Default|GetUnit_AI)))
  (Variables|Default|SetDamagedUnitThisTurn (or (Variables|Default|GetDamagedUnitThisTurn) (< (.X (Utilities|Struct|BreakIntPoint (.MinMaxModifier_HP (Utilities|Struct|BreakS_SpellDataImpact (Utilities|Struct|BreakS_SpellData _spelldata))))) 0)))
  (|CallParentFunction))

(fn ConstructionScript
  (|CallParentFunction))

(fn AIPlayTurn
  (Math|Integer|IncrementInt (Variables|Default|GetTurnCount)
    (:%20%20
      (Variables|Default|SetDamagedUnitThisTurn false)
      (|CallParentFunction))))

(fn GetUnitMovementLogic
  (return (select (Variables|Default|GetDamagedUnitThisTurn) (Utilities|Array|Get(acopy) (Variables|Default|GetMovementLogic) (Math|Random|RandomInteger 2)) "NewEnumerator0")))

(fn AICombatStarted
  (Variables|Default|SetTurnCount 0)
  (|CallParentFunction))