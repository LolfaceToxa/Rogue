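; Overworld manager that tracks units in ID-keyed groups, syncing hover and movement across members.
; Unit events drive it, with temporary unbinding around propagated calls: encounters cluster near the mover's target, other groups follow in a chain.
; A non-encounter unit reaching an encounter disables bystanders and quick-starts combat on a random-sized grid.
; Afterwards it heals team 0 and winners (everyone on draws), destroys other combatants, restores positions and restarts encounter wandering.
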(event EventBeginPlay)

(event Collision|EventActorBeginOverlap
  (params (OtherActor :type Actor%20Object%20Reference)))

(event EventTick
  (params (DeltaSeconds :type Float%20%28single-precision%29)))

(fn ConstructionScript)

(fn AddUnittoGroup
  (params (UnitToAdd :type BP%20Unit%20Object%20Reference) (GroupID :type Integer))
  (if (!= GroupID (Variables|/Game/Rogue/Blueprints/Core/Units/BP_Unit.BP_Unit_C|GetOverworldGroupID UnitToAdd))
    (CallFunction|RemoveUnitfromCurGroup UnitToAdd)
    (if (!= GroupID -999)
      (bind _output_get (LocalVariables|SetGroup (.Value (Utilities|Map|Find (Variables|Default|GetUnitGroups) GroupID))))
      (Utilities|Array|Add (.Units (Utilities|Struct|BreakS_OverworldUnitGroup _output_get)) UnitToAdd)
      (Utilities|Struct|SetmembersinS_OverworldUnitGroup (LocalVariables|GetGroup) GroupID)
      (Utilities|Map|Add (Variables|Default|GetUnitGroups) GroupID (LocalVariables|GetGroup))
      (Variables|/Game/Rogue/Blueprints/Core/Units/BP_Unit.BP_Unit_C|SetOverworldGroupID UnitToAdd GroupID)
      (Game|BindEventtoOnDestroyed UnitToAdd (EventDispatchers|CreateEvent :!event OnUnitDestroyed))
      (EventDispatchers|BindEventtoOnUnitHoveredChanged UnitToAdd (EventDispatchers|CreateEvent :!event OnUnitHoveredChanged))
      (EventDispatchers|BindEventtoOnUnitStartedWalkingOverworld UnitToAdd (EventDispatchers|CreateEvent :!event OnUnitStartedWalkinginOverworld))
      (EventDispatchers|BindEventtoOnUnitReachedUnitinOverworld UnitToAdd (EventDispatchers|CreateEvent :!event OnUnitReachedUnitinOverworld)))))

(fn RemoveUnitfromCurGroup
  (params (UnitToRemove :type BP%20Unit%20Object%20Reference))
  (if (!= (Variables|/Game/Rogue/Blueprints/Core/Units/BP_Unit.BP_Unit_C|GetOverworldGroupID UnitToRemove) -999)
    (LocalVariables|SetGroup (.Value (Utilities|Map|Find (Variables|Default|GetUnitGroups) (Variables|/Game/Rogue/Blueprints/Core/Units/BP_Unit.BP_Unit_C|GetOverworldGroupID UnitToRemove))))
    (Utilities|Array|RemoveItem (Utilities|Struct|BreakS_OverworldUnitGroup (LocalVariables|GetGroup)) UnitToRemove)
    (if (> (Utilities|Array|Length (Utilities|Struct|BreakS_OverworldUnitGroup (LocalVariables|GetGroup))) 0)
      (Utilities|Map|Add (Variables|Default|GetUnitGroups) (Variables|/Game/Rogue/Blueprints/Core/Units/BP_Unit.BP_Unit_C|GetOverworldGroupID UnitToRemove) (LocalVariables|GetGroup))
      (else
        (Utilities|Map|Remove (Variables|Default|GetUnitGroups) (Variables|/Game/Rogue/Blueprints/Core/Units/BP_Unit.BP_Unit_C|GetOverworldGroupID UnitToRemove))))
    (Variables|/Game/Rogue/Blueprints/Core/Units/BP_Unit.BP_Unit_C|SetOverworldGroupID UnitToRemove -999)
    (EventDispatchers|UnbindEventfromOnUnitHoveredChanged UnitToRemove (EventDispatchers|CreateEvent :!event OnUnitHoveredChanged))
    (EventDispatchers|UnbindEventfromOnUnitStartedWalkingOverworld UnitToRemove (EventDispatchers|CreateEvent :!event OnUnitStartedWalkinginOverworld))
    (EventDispatchers|UnbindEventfromOnUnitReachedUnitinOverworld UnitToRemove (EventDispatchers|CreateEvent :!event OnUnitReachedUnitinOverworld))))

(fn OnUnitDestroyed
  (params (DestroyedActor :type Actor%20Object%20Reference))
  (bind _asbp_unit (Utilities|Casting|CastToBP_Unit DestroyedActor))
  (CallFunction|RemoveUnitfromCurGroup _asbp_unit))

(fn OnUnitHoveredChanged
  (params (Cur%20Unit :type BP%20Unit%20Object%20Reference))
  (bind _unitgroups (Variables|Default|GetUnitGroups))
  (bind _overworldgroupid (Variables|/Game/Rogue/Blueprints/Core/Units/BP_Unit.BP_Unit_C|GetOverworldGroupID Cur%20Unit))
  (bind (_value _returnvalue) (Utilities|Map|Find _unitgroups _overworldgroupid))
  (if (not (Variables|/Game/Rogue/Blueprints/Core/Combat/BP_CombatSystem.BP_CombatSystem_C|GetIsInCombat (Variables|Default|GetCombatSystem)))
    (if _returnvalue
      (bind _output_get (LocalVariables|SetGroup _value))
      (for _array_element (.Units (Utilities|Struct|BreakS_OverworldUnitGroup _output_get))
        (bind _output_get_2 (LocalVariables|SetU _array_element))
        (if (!= _output_get_2 Cur%20Unit)
          (EventDispatchers|UnbindEventfromOnUnitHoveredChanged (LocalVariables|GetU) (EventDispatchers|CreateEvent :!event OnUnitHoveredChanged))
          (Default|SetIsHovered (LocalVariables|GetU) (Variables|/Game/Rogue/Blueprints/Core/Units/BP_Unit.BP_Unit_C|GetIsHovered Cur%20Unit))
          (EventDispatchers|BindEventtoOnUnitHoveredChanged (LocalVariables|GetU) (EventDispatchers|CreateEvent :!event OnUnitHoveredChanged)))))))

(fn OnUnitStartedWalkinginOverworld
  (params (Unit :type BP%20Unit%20Object%20Reference))
  (if (Utilities|Struct|BreakS_OverworldUnitGroup (.Value (Utilities|Map|Find (Variables|Default|GetUnitGroups) (Variables|/Game/Rogue/Blueprints/Core/Units/BP_Unit.BP_Unit_C|GetOverworldGroupID Unit))))
    (for _array_element (Utilities|Struct|BreakS_OverworldUnitGroup (.Value (Utilities|Map|Find (Variables|Default|GetUnitGroups) (Variables|/Game/Rogue/Blueprints/Core/Units/BP_Unit.BP_Unit_C|GetOverworldGroupID Unit))))
      (LocalVariables|SetU _array_element)
      (if (!= (LocalVariables|GetU) Unit)
        (EventDispatchers|UnbindEventfromOnUnitStartedWalkingOverworld (LocalVariables|GetU) (EventDispatchers|CreateEvent :!event OnUnitStartedWalkinginOverworld))
        (bind _randomlocation (Default|GetRandomReachableLocinRadius (LocalVariables|GetU) (Variables|/Game/Rogue/Blueprints/Core/Units/BP_Unit.BP_Unit_C|GetTargetLocInOverworld Unit) "(X=100.000000,Y=400.000000)"))
        (Default|EventMoveUnitinOverworld (LocalVariables|GetU) _randomlocation 0 false)
        (EventDispatchers|BindEventtoOnUnitStartedWalkingOverworld (LocalVariables|GetU) (EventDispatchers|CreateEvent :!event OnUnitStartedWalkinginOverworld))))
    (else
      (LocalVariables|SetPrevious%20Unit Unit)
      (for _array_element_2 (Utilities|Struct|BreakS_OverworldUnitGroup (.Value (Utilities|Map|Find (Variables|Default|GetUnitGroups) (Variables|/Game/Rogue/Blueprints/Core/Units/BP_Unit.BP_Unit_C|GetOverworldGroupID Unit))))
        (bind _output_get (LocalVariables|SetU _array_element_2))
        (if (!= _output_get Unit)
          (EventDispatchers|UnbindEventfromOnUnitStartedWalkingOverworld (LocalVariables|GetU) (EventDispatchers|CreateEvent :!event OnUnitStartedWalkinginOverworld))
          (Default|EventMoveUnitinOverworld (LocalVariables|GetU) "0, 0, 0" (LocalVariables|GetPrevious%20Unit) false)
          (LocalVariables|SetPrevious%20Unit (LocalVariables|GetU))
          (EventDispatchers|BindEventtoOnUnitStartedWalkingOverworld (LocalVariables|GetU) (EventDispatchers|CreateEvent :!event OnUnitStartedWalkinginOverworld)))))))

(fn SetGroupIsEncounter
  (params (IsEncounter :type Boolean) (GroupID :type Integer))
  (bind _unitgroups (Variables|Default|GetUnitGroups))
  (bind (_value _returnvalue) (Utilities|Map|Find _unitgroups GroupID))
  (if _returnvalue
    (bind _output_get (LocalVariables|SetGroup _value))
    (if (!= (Utilities|Struct|BreakS_OverworldUnitGroup _output_get) IsEncounter)
      (Utilities|Struct|SetmembersinS_OverworldUnitGroup (LocalVariables|GetGroup) IsEncounter)
      (Utilities|Map|Add (Variables|Default|GetUnitGroups) GroupID (LocalVariables|GetGroup))
      (for _array_element (.Units (Utilities|Struct|BreakS_OverworldUnitGroup (LocalVariables|GetGroup)))
        (Default|EventStopMovingUnitinOverworld _array_element))
      (if (.IsEncounter (Utilities|Struct|BreakS_OverworldUnitGroup (LocalVariables|GetGroup)))
        (Default|EventMoveUnitinOverworld (Utilities|Array|Get(acopy) (.Units (Utilities|Struct|BreakS_OverworldUnitGroup (LocalVariables|GetGroup)))) "0, 0, 0" 0 true)))))

(fn SetCombatSystem
  (params (CombatSystem :type BP%20Combat%20System%20Object%20Reference))
  (Variables|Default|SetCombatSystem CombatSystem)
  (EventDispatchers|BindEventtoOnCombatEnded (Variables|Default|GetCombatSystem) (EventDispatchers|CreateEvent :!event OnCombatEnded)))

(fn OnUnitReachedUnitinOverworld
  (params (Unit :type BP%20Unit%20Object%20Reference))
  (LocalVariables|SetGroup1 (.Value (Utilities|Map|Find (Variables|Default|GetUnitGroups) (Variables|/Game/Rogue/Blueprints/Core/Units/BP_Unit.BP_Unit_C|GetOverworldGroupID Unit))))
  (LocalVariables|SetGroup2 (.Value (Utilities|Map|Find (Variables|Default|GetUnitGroups) (Variables|/Game/Rogue/Blueprints/Core/Units/BP_Unit.BP_Unit_C|GetOverworldGroupID (Variables|/Game/Rogue/Blueprints/Core/Units/BP_Unit.BP_Unit_C|GetUnit%20To%20Follow%20in%20Overworld Unit)))))
  (if (Math|Boolean|ANDBoolean (!= (.GroupID (Utilities|Struct|BreakS_OverworldUnitGroup (LocalVariables|GetGroup1))) (.GroupID (Utilities|Struct|BreakS_OverworldUnitGroup (LocalVariables|GetGroup2)))) (not (.IsEncounter (Utilities|Struct|BreakS_OverworldUnitGroup (LocalVariables|GetGroup1)))) (.IsEncounter (Utilities|Struct|BreakS_OverworldUnitGroup (LocalVariables|GetGroup2))))
    (CallFunction|TriggerEncounter (Utilities|Array|MakeArray (LocalVariables|GetGroup1) (LocalVariables|GetGroup2)))))

(fn TriggerEncounter
  (params (Groups :type Array%20of%20S%20Overworld%20Unit%20Group%20Structures))
  (if (not (Variables|/Game/Rogue/Blueprints/Core/Combat/BP_CombatSystem.BP_CombatSystem_C|GetIsInCombat (Variables|Default|GetCombatSystem)))
    (Utilities|FlowControl|Sequence
      (:then_0
        (Utilities|Map|Clear (Variables|Default|GetUnitPositionsWhenCombatStarted))
        (bind _values (Utilities|Map|Values (Variables|Default|GetUnitGroups)))
        (for _array_element _values
          (for _array_element_2 (.Units (Utilities|Struct|BreakS_OverworldUnitGroup _array_element))
            (Utilities|Map|Add (Variables|Default|GetUnitPositionsWhenCombatStarted) _array_element_2 (Transformation|GetActorLocation _array_element_2))
            (if (not (Utilities|Array|ContainsItem Groups _array_element))
              (Default|DisableUnit _array_element_2) ; Disable Units That Not In Combat
            ))))
      (:then_1
        (LocalVariables|SetGrid%20Data (Utilities|Struct|MakeS_QuickCombat_Grid true (Transformation|GetActorLocation (Utilities|Array|Get(acopy) (.Units (Utilities|Struct|BreakS_OverworldUnitGroup (Utilities|Array|Get(acopy) Groups))))) "200.000000,200.000000,100.000000" (Utilities|Struct|MakeIntPoint (Math|Random|RandomIntegerinRange 10 20) (Math|Random|RandomIntegerinRange 10 20))))
        (for _array_element_3 Groups
          (Utilities|Array|Add (LocalVariables|GetUnitTeams) (Utilities|Struct|MakeS_UnitArray (.Units (Utilities|Struct|BreakS_OverworldUnitGroup _array_element_3))))
          (if (.IsEncounter (Utilities|Struct|BreakS_OverworldUnitGroup _array_element_3))
            (Utilities|Array|AppendArray (LocalVariables|GetControlledByAI) (.Units (Utilities|Struct|BreakS_OverworldUnitGroup _array_element_3)))))
        (Default|QuickStartCombat (Variables|Default|GetCombatSystem) (LocalVariables|GetGrid%20Data) (Utilities|Struct|MakeS_QuickCombat_UnitTeams (LocalVariables|GetUnitTeams) (LocalVariables|GetControlledByAI) (Utilities|Map|MakeMap)) self)))))

(fn OnCombatEnded
  (bind _combatsystem (Variables|Default|GetCombatSystem))
  (bind _team_index_that_won_last (Variables|/Game/Rogue/Blueprints/Core/Combat/BP_CombatSystem.BP_CombatSystem_C|GetTeam%20Index%20That%20Won%20Last _combatsystem))
  (if (== (Variables|/Game/Rogue/Blueprints/Core/Combat/BP_CombatSystem.BP_CombatSystem_C|GetObjectThatStartedCombat (Variables|Default|GetCombatSystem)) self)
    (bind _keys (Utilities|Map|Keys (Variables|/Game/Rogue/Blueprints/Core/Combat/BP_CombatSystem.BP_CombatSystem_C|GetUnitTeams (Variables|Default|GetCombatSystem))))
    (for _array_element _keys
      (LocalVariables|SetTeam%20Index _array_element)
      (bind _output_get (LocalVariables|SetUnitsInTeams (Utilities|Struct|BreakS_UnitArray (.Value (Utilities|Map|Find (Variables|/Game/Rogue/Blueprints/Core/Combat/BP_CombatSystem.BP_CombatSystem_C|GetUnitTeams (Variables|Default|GetCombatSystem)) (LocalVariables|GetTeam%20Index))))))
      (for _array_element_2 _output_get
        (bind _output_get_2 (LocalVariables|SetU _array_element_2))
        (Default|RemoveUnitfromCombat (Variables|Default|GetCombatSystem) _output_get_2)
        (if (Math|Boolean|ORBoolean (== (LocalVariables|GetTeam%20Index) 0) (== (LocalVariables|GetTeam%20Index) _team_index_that_won_last) (== _team_index_that_won_last -1)) ; If unit in winning team - respawn it in overworld
          (Default|ResetHP (LocalVariables|GetU))
          (else
            (Actor|DestroyActor (LocalVariables|GetU))))))
    (bind _keys_2 (Utilities|Map|Keys (Variables|Default|GetUnitPositionsWhenCombatStarted)))
    (for _array_element_3 _keys_2 ; Put units where they were in overworld
      (bind _output_get_3 (LocalVariables|SetU _array_element_3))
      (Utilities|IsValid _output_get_3
        (:Is%20Valid
          (Transformation|SetActorLocation (LocalVariables|GetU) (.Value (Utilities|Map|Find (Variables|Default|GetUnitPositionsWhenCombatStarted) (LocalVariables|GetU))) false false)
          (Default|EnableUnit (LocalVariables|GetU) "NewEnumerator1"))))
    (Utilities|Map|Clear (Variables|Default|GetUnitPositionsWhenCombatStarted))
    (bind _values (Utilities|Map|Values (Variables|Default|GetUnitGroups)))
    (for _array_element_4 _values ; Ask encounters to move
      (if (.IsEncounter (Utilities|Struct|BreakS_OverworldUnitGroup _array_element_4))
        (Default|EventMoveUnitinOverworld (Utilities|Array|Get(acopy) (.Units (Utilities|Struct|BreakS_OverworldUnitGroup _array_element_4))) "0, 0, 0" 0 true)))
    (Default|DestroyGrid (Variables|/Game/Rogue/Blueprints/Core/Combat/BP_CombatSystem.BP_CombatSystem_C|GetGrid (Variables|Default|GetCombatSystem)))))