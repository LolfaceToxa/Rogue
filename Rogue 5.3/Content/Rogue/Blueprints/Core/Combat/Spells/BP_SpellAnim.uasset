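; Spell animation actor that visualizes a spell spreading from an origin tile to the attacked tiles on the grid.
; On BeginPlay it spawns one BP_AnimatedShape per target, using the grid's mesh with randomized red brightness and play rate.
; The shape completion handler broadcasts a tile hit and tracks remaining targets.
; When none remain, it clears attacked-tile visuals, broadcasts completion and destroys itself.
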(event Custom|EventPlaySpellAnim
  (bind _grid (Variables|Default|GetGrid))
  (bind _originindex (Variables|Default|GetOriginIndex))
  (bind _returnvalue (Default|GetCurrentShapeData _grid))
  (bind _transform (CallFunction|GetTileTransform _originindex))
  (bind (_meshsize _mesh _material) (Utilities|Struct|BreakS_GridShapeData _returnvalue))
  (Utilities|Array|Clear (Variables|Default|GetAttacked%20Indexes%20NO%20CHANGE))
  (for _array_element (Variables|Default|GetAttackedIndexes)
    (bind _returnvalue_2 (Game|SpawnActorfromClass "/Game/Rogue/Blueprints/Core/Combat/Spells/Anims/Components/BP_AnimatedShape.BP_AnimatedShape_C" (Math|Transform|MakeTransform "0, 0, 0" "0, 0, 0" "1.000000,1.000000,1.000000") "AlwaysSpawn" "MultiplyWithRoot" 0 _mesh _material (* "(R=1.000000,G=0.000000,B=0.000000,A=1.000000)" (Math|Random|RandomFloatinRange 0.5 1.5)) (Math|Transform|MakeTransform (.location _transform) (.rotation _transform) "0.010000,0.010000,0.010000") (CallFunction|GetTileTransform _array_element) (Math|Random|RandomFloatinRange 0.8 1.5) _array_element 0))
    (EventDispatchers|UnbindEventfromOnShapeAnimCompleted _returnvalue_2 (delegate Custom|OnShapeAnimCompleted))))

(event Custom|OnShapeAnimCompleted
  (params (AnimatedShape :type BP%20Animated%20Shape%20Object%20Reference))
  (bind _index (Variables|/Game/Rogue/Blueprints/Core/Combat/Spells/Anims/Components/BP_AnimatedShape.BP_AnimatedShape_C|GetIndex AnimatedShape))
  (bind _attackedindexes (Variables|Default|GetAttackedIndexes))
  (Default|CallOnSpellAnimHitTIle self _index)
  (Utilities|Array|Add (Variables|Default|GetAttacked%20Indexes%20NO%20CHANGE) _index)
  (Utilities|Array|RemoveItem _attackedindexes _index)
  (if (== (Utilities|Array|Length _attackedindexes) 0)
    (CallFunction|EventCompleteSpellAnim (Variables|Default|GetAttacked%20Indexes%20NO%20CHANGE))))

(event Custom|EventCompleteSpellAnim
  (params (AttackedIndexesNOCHANGE :type Array%20of%20Int%20Point%20Structures))
  (Default|RemoveTilesAttacked (Variables|/Game/Rogue/Blueprints/Core/Grid/BP_Grid.BP_Grid_C|GetGrid%20Visual (Variables|Default|GetGrid)) AttackedIndexesNOCHANGE)
  (Default|CallOnSpellAnimCompleted self)
  (Actor|DestroyActor))

(event EventBeginPlay
  (CallFunction|EventPlaySpellAnim))

(fn ConstructionScript)

(fn GetTileTransform
  (params (Index :type Int%20Point%20Structure%20%28by%20ref%29))
  (return (.Transform (Utilities|Struct|BreakS_TileDataF (.Value (Utilities|Map|Find (Variables|/Game/Rogue/Blueprints/Core/Grid/BP_Grid.BP_Grid_C|GetGrid%20Tiles (Variables|Default|GetGrid)) Index))))))