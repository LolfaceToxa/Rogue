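; Spell animation actor for Blade Dance, showing four spinning, blue-tinted blade meshes at the caster's origin tile, facing the target tile.
; A timeline drives material opacity and adds a fixed rotation to each mesh and the AnimRotationScale component every update, so spin speed follows frame rate.
; Once playback reaches 0.2 seconds, a DoOnce reports a hit for each attacked tile.
; The timeline's end completes the spell animation with those tiles.
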(event EventBeginPlay
  (|CallParentFunction) ; This node is disabled and will not be called.\nDrag off pins to build functionality.
)

(event EventEventPlaySpellAnim
  (Transformation|SetActorLocationAndRotation (.location (CallFunction|GetTileTransform (Variables|Default|GetOriginIndex))) (Math|Rotator|FindLookatRotation (Math|Conversions|ToVector(Vector2D) (Math|Conversions|ToVector2D(IntPoint) (Variables|Default|GetOriginIndex))) (Math|Conversions|ToVector(Vector2D) (Math|Conversions|ToVector2D(IntPoint) (Variables|Default|GetTargetIndex)))))
  (bind _opacity (Timeline|Timeline_BladeDance PlayFromStart)
    (:Update
      (for _array_element (Utilities|Array|MakeArray (Variables|Default|GetStaticMesh1) (Variables|Default|GetStaticMesh2) (Variables|Default|GetStaticMesh3) (Variables|Default|GetStaticMesh4))
        (CallFunction|AddRotationtoSceneComp _array_element "0.000000,5.000000,0.000000"))
      (CallFunction|AddRotationtoSceneComp (Variables|Default|GetAnim_RotationScale) "0.000000,5.000000,0.000000")
      (Rendering|Material|SetScalarParameterValueonMaterials (Variables|Default|GetStaticMesh1) "Opacity" _opacity)
      (if (>= (Components|Timeline|GetPlaybackPosition (Variables|Default|GetTimeline_BladeDance)) 0.2)
        (Utilities|FlowControl|DoOnce false
          (:Completed
            (for _array_element_2 (Variables|Default|GetAttackedIndexes)
              (Default|CallOnSpellAnimHitTIle self _array_element_2))))))
    (:Finished
      (CallFunction|EventCompleteSpellAnim (Variables|Default|GetAttackedIndexes)))))

(fn ConstructionScript
  (|CallParentFunction)
  (Rendering|Material|SetVectorParameterValueonMaterials (Variables|Default|GetStaticMesh1) "Color" (Math|Conversions|ToVector(LinearColor) "(R=0.100104,G=0.226754,B=0.775000,A=0.750000)"))
  (CallFunction|AddRotationtoSceneComp (Variables|Default|GetAnim_RotationScale) "0, 0, 0"))

(fn AddRotationtoSceneComp
  (params (SM :type Scene%20Component%20Object%20Reference) (AddRot :type Rotator))
  (Transformation|SetRelativeRotation SM (Math|Rotator|CombineRotators (Variables|/Script/Engine.SceneComponent|GetRelativeRotation SM) AddRot) false false))

(fn SetRotationtoSM
  (params (SM :type Static%20Mesh%20Component%20Object%20Reference) (AddRot :type Rotator))
  (Transformation|SetRelativeRotation SM (Math|Rotator|CombineRotators "0, 0, 0" AddRot) false false))