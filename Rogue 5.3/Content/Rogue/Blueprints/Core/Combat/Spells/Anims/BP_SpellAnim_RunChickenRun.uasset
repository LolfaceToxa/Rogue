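; BP_SpellAnim_RunChickenRun is the spell animation actor for the Run Chicken Run spell, shown as an icon on the target tile.
; On play, it moves to the tile and sets the widget component's image to the spell icon.
; A timeline animates the widget's height, draw size and opacity.
; It signals the tile hit once playback reaches 0.2 seconds, then completes the spell animation when the timeline finishes.
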(event EventBeginPlay
  (|CallParentFunction) ; This node is disabled and will not be called.\nDrag off pins to build functionality.
)

(event Collision|EventActorBeginOverlap
  (params (OtherActor :type Actor%20Object%20Reference)))

(event EventTick
  (params (DeltaSeconds :type Float%20%28single-precision%29)))

(event EventEventPlaySpellAnim
  (bind _widget (Variables|Default|GetWidget))
  (Transformation|SetActorLocation (.location (CallFunction|GetTileTransform (Variables|Default|GetTargetIndex))) false false)
  (bind _output_get (Variables|Default|SetAs%20W%20Image (.AsW%20Image (Utilities|Casting|CastToW_Image (UserInterface|GetUserWidgetObject (Variables|Default|GetWidget))))))
  (Appearance|SetBrushfromTexture (Variables|/Game/Rogue/Blueprints/Core/Combat/Spells/Anims/Components/W_Image.W_Image_C|GetImage_Comp _output_get) "/Game/Rogue/Blueprints/Core/Combat/Spells/Anims/Assets/Icon_RunChickenRun_NoBackground.Icon_RunChickenRun_NoBackground" false)
  (bind (_direction _locz _drawsize _opacity) (Timeline|Timeline_RunChickenRun PlayFromStart)
    (:Update
      (Transformation|SetRelativeLocation _widget (Math|Vector|MakeVector 0.0 0.0 _locz) false false)
      (Class|WidgetComponent|SetDrawSize _widget (Math|Vector2D|MakeVector2D _drawsize _drawsize))
      (Widget|SetRenderOpacity (Variables|Default|GetAs%20W%20Image) _opacity)
      (if (>= (Components|Timeline|GetPlaybackPosition (Variables|Default|GetTimeline_RunChickenRun)) 0.2)
        (Utilities|FlowControl|DoOnce false
          (:Completed
            (Default|CallOnSpellAnimHitTIle self (Variables|Default|GetTargetIndex))))))
    (:Finished
      (CallFunction|EventCompleteSpellAnim (Utilities|Array|MakeArray (Variables|Default|GetTargetIndex))))))

(fn ConstructionScript
  (|CallParentFunction))