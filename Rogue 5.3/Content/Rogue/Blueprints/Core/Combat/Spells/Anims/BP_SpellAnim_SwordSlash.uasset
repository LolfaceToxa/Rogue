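; Spell animation Blueprint for a sword slash from an origin tile toward a target tile in the tile-based combat.
; On play, it moves to the origin tile and yaws toward the target using the two grid indices.
; A timeline drives the pitch and scale of the slash component, reports the tile hit once partway through via DoOnce, then completes the animation with the target tile.
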(event EventBeginPlay
  (|CallParentFunction) ; This node is disabled and will not be called.\nDrag off pins to build functionality.
)

(event EventEventPlaySpellAnim
  (bind _anim_rotationscale (Variables|Default|GetAnim_RotationScale))
  (Transformation|SetActorLocationAndRotation (.location (CallFunction|GetTileTransform (Variables|Default|GetOriginIndex))) (Math|Rotator|FindLookatRotation (Math|Conversions|ToVector(Vector2D) (Math|Conversions|ToVector2D(IntPoint) (Variables|Default|GetOriginIndex))) (Math|Conversions|ToVector(Vector2D) (Math|Conversions|ToVector2D(IntPoint) (Variables|Default|GetTargetIndex)))))
  (bind (_direction _rotationy _scale) (Timeline|Timeline_SwordSlash PlayFromStart)
    (:Update
      (Transformation|SetRelativeRotation _anim_rotationscale (Math|Rotator|MakeRotator 0.0 _rotationy 0.0) false false)
      (Transformation|SetRelativeScale3D _anim_rotationscale (Math|Conversions|ToVector(Float) _scale))
      (if (>= (Components|Timeline|GetPlaybackPosition (Variables|Default|GetTimeline_SwordSlash)) 0.4)
        (Utilities|FlowControl|DoOnce false
          (:Completed
            (Default|CallOnSpellAnimHitTIle self (Variables|Default|GetTargetIndex))))))
    (:Finished
      (CallFunction|EventCompleteSpellAnim (Utilities|Array|MakeArray (Variables|Default|GetTargetIndex))))))

(fn ConstructionScript
  (|CallParentFunction))