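; Animated wind gust actor for spell animations: a short-lived translucent green shape that moves and changes opacity.
; The construction script gives both material slots dynamic translucent materials with randomized green brightness.
; On BeginPlay a rate-scaled timeline interpolates the actor from origin to target transform and drives the Opacity parameter.
; When the timeline finishes, it broadcasts shape-animation completion, then destroys itself after a brief delay.
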(event EventBeginPlay
  (Components|Timeline|SetPlayRate (Variables|Default|GetTimeline_PlayAnim) (Variables|Default|GetPlay%20Rate))
  (bind (_direction _alpha _opacity) (Timeline|Timeline_PlayAnim PlayFromStart)
    (:Update
      (Transformation|SetActorTransform (Math|Transform|Lerp(Transform) (Variables|Default|GetOriginTransform) (Variables|Default|GetTargetTransform) _alpha))
      (Rendering|Material|SetScalarParameterValueonMaterials (Variables|Default|GetAnimatedShape) "Opacity" _opacity)
      (Utilities|FlowControl|DoOnce (>= (Components|Timeline|GetPlaybackPosition (Variables|Default|GetTimeline_PlayAnim)) 0.0)))
    (:Finished
      (Default|CallOnShapeAnimCompleted self)
      (Utilities|FlowControl|Delay 0.5)
      (Actor|DestroyActor))))

(fn ConstructionScript
  (bind _returnvalue (Rendering|Material|CreateDynamicMaterialInstance (Variables|Default|GetAnimatedShape) 0 "/Game/Rogue/Art/Materials/M_Translucent.M_Translucent" "None" :!class /Script/Engine.PrimitiveComponent))
  (Rendering|Material|SetVectorParameterValue _returnvalue "Color" (* (Math|Random|RandomFloatinRange 0.8 1.5) "(R=0.000000,G=0.566667,B=0.040197,A=1.000000)") :!class /Script/Engine.MaterialInstanceDynamic)
  (bind _returnvalue_2 (Rendering|Material|CreateDynamicMaterialInstance (Variables|Default|GetAnimatedShape) 1 "/Game/Rogue/Art/Materials/M_Translucent.M_Translucent" "None" :!class /Script/Engine.PrimitiveComponent))
  (Rendering|Material|SetVectorParameterValue _returnvalue_2 "Color" (* (Math|Random|RandomFloatinRange 0.8 1.5) "(R=0.073472,G=0.766667,B=0.122645,A=1.000000)") :!class /Script/Engine.MaterialInstanceDynamic))