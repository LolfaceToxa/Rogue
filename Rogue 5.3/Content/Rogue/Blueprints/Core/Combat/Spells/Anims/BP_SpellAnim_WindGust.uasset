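; Spell animation for Wind Gust that sends animated gusts from the target tile out to every other attacked tile.
; After a short delay it reports a hit on the target tile, then spawns a BP_AnimatedWindGust per remaining tile, rotated outward with a random play rate.
; Each finished gust reports a hit on its tile.
; The spell animation completes once no attacked tiles remain.
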(event Custom|OnShapeAnimComplete
  (params (AnimatedShape :type BP%20Animated%20Wind%20Gust%20Object%20Reference))
  (bind _attackedindexes (Variables|Default|GetAttackedIndexes))
  (bind _index (Variables|/Game/Rogue/Blueprints/Core/Combat/Spells/Anims/Components/BP_AnimatedWindGust.BP_AnimatedWindGust_C|GetIndex AnimatedShape))
  (Default|CallOnSpellAnimHitTIle self _index)
  (Utilities|Array|Add (Variables|Default|GetAttacked%20Indexes%20NO%20CHANGE) _index)
  (Utilities|Array|RemoveItem _attackedindexes _index)
  (if (== (Utilities|Array|Length _attackedindexes) 0)
    (CallFunction|EventCompleteSpellAnim (Variables|Default|GetAttacked%20Indexes%20NO%20CHANGE))))

(event EventBeginPlay
  (|CallParentFunction) ; This node is disabled and will not be called.\nDrag off pins to build functionality.
)

(event Collision|EventActorBeginOverlap
  (params (OtherActor :type Actor%20Object%20Reference)))

(event EventTick
  (params (DeltaSeconds :type Float%20%28single-precision%29)))

(event EventEventPlaySpellAnim
  (bind _targetindex (Variables|Default|GetTargetIndex))
  (bind _transform (CallFunction|GetTileTransform _targetindex))
  (Utilities|Array|Clear (Variables|Default|GetAttacked%20Indexes%20NO%20CHANGE))
  (Utilities|FlowControl|Delay 0.1)
  (Default|CallOnSpellAnimHitTIle self (Variables|Default|GetTargetIndex))
  (Utilities|Array|Add (Variables|Default|GetAttacked%20Indexes%20NO%20CHANGE) (Variables|Default|GetTargetIndex))
  (Utilities|Array|RemoveItem (Variables|Default|GetAttackedIndexes) (Variables|Default|GetTargetIndex))
  (for _array_element (Variables|Default|GetAttackedIndexes)
    (bind _returnvalue (Game|SpawnActorfromClass "/Game/Rogue/Blueprints/Core/Combat/Spells/Anims/Components/BP_AnimatedWindGust.BP_AnimatedWindGust_C" (Math|Transform|MakeTransform "0, 0, 0" "0, 0, 0" "1.000000,1.000000,1.000000") "AlwaysSpawn" "MultiplyWithRoot" 0 (Math|Transform|MakeTransform (.location _transform) (Math|Rotator|FindLookatRotation (.location _transform) (.location (CallFunction|GetTileTransform _array_element))) "0.500000,0.500000,0.500000") (Math|Transform|MakeTransform (.location (CallFunction|GetTileTransform _array_element)) (Math|Rotator|FindLookatRotation (.location _transform) (.location (CallFunction|GetTileTransform _array_element)))) (Math|Random|RandomFloatinRange 0.8 1.5) _array_element 0))
    (EventDispatchers|BindEventtoOnShapeAnimCompleted _returnvalue (delegate Custom|OnShapeAnimComplete))))

(fn ConstructionScript
  (|CallParentFunction))