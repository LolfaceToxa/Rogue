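; Spell animation Blueprint for the Rage spell, showing a red spinning mesh effect on the target tile.
; On play, it moves to the target tile, facing away from the origin index, and a timeline named Timeline_Heal drives scale, rotation and opacity on three of six meshes.
; It signals the tile hit once, shortly into playback, and completes when the timeline finishes.
; The construction script tints the meshes in red shades.
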(event EventBeginPlay
  (|CallParentFunction) ; This node is disabled and will not be called.\nDrag off pins to build functionality.
)

(event EventEventPlaySpellAnim
  (Transformation|SetActorLocationAndRotation (.location (CallFunction|GetTileTransform (Variables|Default|GetTargetIndex))) (Math|Rotator|FindLookatRotation (Math|Conversions|ToVector(Vector2D) (Math|Conversions|ToVector2D(IntPoint) (Variables|Default|GetOriginIndex))) (Math|Conversions|ToVector(Vector2D) (Math|Conversions|ToVector2D(IntPoint) (Variables|Default|GetTargetIndex)))))
  (bind (_direction _opacity _scale _rot) (Timeline|Timeline_Heal PlayFromStart)
    (:Update
      (Transformation|SetRelativeScale3D (Variables|Default|GetAnim_RotationScale) _scale)
      (Rendering|Material|SetScalarParameterValueonMaterials (Variables|Default|GetStaticMesh) "Opacity" _opacity)
      (Transformation|SetRelativeRotation (Variables|Default|GetStaticMesh) (Math|Rotator|MakeRotator 0.0 0.0 _rot) false false)
      (if (>= (Components|Timeline|GetPlaybackPosition (Variables|Default|GetTimeline_Heal)) 0.2)
        (Utilities|FlowControl|DoOnce false
          (:Completed
            (Default|CallOnSpellAnimHitTIle self (Variables|Default|GetTargetIndex))))))
    (:Finished
      (CallFunction|EventCompleteSpellAnim))))

(fn ConstructionScript
  (|CallParentFunction)
  (Rendering|Material|SetVectorParameterValueonMaterials (Variables|Default|GetStaticMesh) "Color" (Math|Conversions|ToVector(LinearColor) "(R=0.858333,G=0.025035,B=0.025035,A=1.000000)"))
  (Rendering|Material|SetVectorParameterValueonMaterials (Variables|Default|GetStaticMesh1) "Color" (Math|Conversions|ToVector(LinearColor) "(R=0.550000,G=0.041250,B=0.046182,A=1.000000)"))
  (Rendering|Material|SetVectorParameterValueonMaterials (Variables|Default|GetStaticMesh2) "Color" (Math|Conversions|ToVector(LinearColor) "(R=1.000000,G=0.170833,B=0.170833,A=1.000000)"))
  (Rendering|Material|SetVectorParameterValueonMaterials (Variables|Default|GetStaticMesh3) "Color" (Math|Conversions|ToVector(LinearColor) "(R=0.629167,G=0.013108,B=0.074968,A=1.000000)"))
  (Rendering|Material|SetVectorParameterValueonMaterials (Variables|Default|GetStaticMesh4) "Color" (Math|Conversions|ToVector(LinearColor) "(R=1.000000,G=0.170833,B=0.170833,A=1.000000)"))
  (Rendering|Material|SetVectorParameterValueonMaterials (Variables|Default|GetStaticMesh5) "Color" (Math|Conversions|ToVector(LinearColor) "(R=0.629167,G=0.013108,B=0.074968,A=1.000000)")))