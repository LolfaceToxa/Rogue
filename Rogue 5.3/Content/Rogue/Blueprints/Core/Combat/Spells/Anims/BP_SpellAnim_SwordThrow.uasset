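; Spell animation actor that shows a sword being thrown from an origin tile to a target tile.
; On play, it faces the target and a timeline lerps the actor between the tiles while animating the AnimRotationScale component's sideways offset, yaw and scale.
; A DoOnce reports the target tile hit at a fixed point in the timeline, and the timeline's end completes the spell animation.
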(event EventBeginPlay
  (|CallParentFunction) ; This node is disabled and will not be called.\nDrag off pins to build functionality.
)

(event EventEventPlaySpellAnim
  (Transformation|SetActorLocationAndRotation (.location (CallFunction|GetTileTransform (Variables|Default|GetOriginIndex))) (Math|Rotator|FindLookatRotation (Math|Conversions|ToVector(Vector2D) (Math|Conversions|ToVector2D(IntPoint) (Variables|Default|GetOriginIndex))) (Math|Conversions|ToVector(Vector2D) (Math|Conversions|ToVector2D(IntPoint) (Variables|Default|GetTargetIndex)))))
  (bind (_direction _actorlocalpha _locy _rotz _scale) (Timeline|Timeline_SwordThrow PlayFromStart)
    (:Update
      (Transformation|SetActorLocation (Math|Vector|Lerp(Vector) (.location (CallFunction|GetTileTransform (Variables|Default|GetOriginIndex))) (.location (CallFunction|GetTileTransform (Variables|Default|GetTargetIndex))) _actorlocalpha) false false)
      (Transformation|SetRelativeTransform (Variables|Default|GetAnim_RotationScale) (Math|Transform|MakeTransform (Math|Vector|MakeVector 0.0 _locy 0.0) (Math|Rotator|MakeRotator 0.0 0.0 _rotz) (Math|Conversions|ToVector(Float) _scale)) false false)
      (if (>= (Components|Timeline|GetPlaybackPosition (Variables|Default|GetTimeline_SwordThrow)) 0.28)
        (Utilities|FlowControl|DoOnce false
          (:Completed
            (Default|CallOnSpellAnimHitTIle self (Variables|Default|GetTargetIndex))))))
    (:Finished
      (CallFunction|EventCompleteSpellAnim))))

(fn ConstructionScript
  (|CallParentFunction))