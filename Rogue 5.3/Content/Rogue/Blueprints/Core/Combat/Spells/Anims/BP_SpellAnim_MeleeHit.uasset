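; BP_SpellAnim_MeleeHit is the spell animation for a melee hit in the combat spell system.
; When played, it waits a short fixed delay, fires the tile-hit notification for its target index, then completes the animation with that single index.
; It spawns no visuals or sound in this graph, so it only supplies the timing of the hit.
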(event EventBeginPlay
  (|CallParentFunction) ; This node is disabled and will not be called.\nDrag off pins to build functionality.
)

(event Collision|EventActorBeginOverlap
  (params (OtherActor :type Actor%20Object%20Reference)))

(event EventTick
  (params (DeltaSeconds :type Float%20%28single-precision%29)))

(event EventEventPlaySpellAnim
  (Utilities|FlowControl|Delay 0.2)
  (Default|CallOnSpellAnimHitTIle self (Variables|Default|GetTargetIndex))
  (CallFunction|EventCompleteSpellAnim (Utilities|Array|MakeArray (Variables|Default|GetTargetIndex))))

(fn ConstructionScript
  (|CallParentFunction))