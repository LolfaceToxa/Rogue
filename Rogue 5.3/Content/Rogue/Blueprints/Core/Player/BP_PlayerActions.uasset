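; Player input hub for a grid tactics game, handling cursor hover, tile and unit selection, and click actions in the overworld and combat.
; Left and right clicks run swappable action actors, which also react to hover changes and repeat while the button is held.
; Combat events switch actions between move, spell cast and AI wait, and manage combat and end-screen widgets.
; BeginPlay also loads or creates a save and applies its time dilation.
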(event Custom|Event_SimulateLeftClickFromExternalSource
  (Utilities|FlowControl|Sequence
    (:then_0
      (CallFunction|UpdateHoveredUnitandTile)
      (Variables|Default|SetIsLeftMouseDown true)
      (Utilities|IsValid (Variables|Default|GetSelectedAction_LeftClick)
        (:Is%20Valid
          (Default|ExecuteAction (Variables|Default|GetSelectedAction_LeftClick) (Variables|Default|GetHoveredTile)))))
    (:then_1
      (Variables|Default|SetIsLeftMouseDown false))))

(event Custom|Event_ExectuteActionWhenHoveredTileChanged
  (bind _hoveredtile (Variables|Default|GetHoveredTile))
  (bind _selectedaction_leftclick (Variables|Default|GetSelectedAction_LeftClick))
  (bind _selectedaction_rightclick (Variables|Default|GetSelectedAction_RightClick))
  (Utilities|FlowControl|Sequence
    (:then_0
      (Utilities|IsValid _selectedaction_leftclick
        (:Is%20Valid
          (Default|ExecuteHoveredAction _selectedaction_leftclick _hoveredtile)
          (if (Variables|Default|GetIsLeftMouseDown)
            (Utilities|IsValid (Variables|Default|GetSelectedAction_LeftClick)
              (:Is%20Valid
                (Default|ExecuteAction (Variables|Default|GetSelectedAction_LeftClick) (Variables|Default|GetHoveredTile))))))))
    (:then_1
      (Utilities|IsValid _selectedaction_rightclick
        (:Is%20Valid
          (Default|ExecuteHoveredAction _selectedaction_rightclick _hoveredtile)
          (if (Variables|Default|GetIsRightMouseDown)
            (Utilities|IsValid (Variables|Default|GetSelectedAction_RightClick)
              (:Is%20Valid
                (Default|ExecuteAction (Variables|Default|GetSelectedAction_RightClick) (Variables|Default|GetHoveredTile))))))))))

(event Input|EnhancedActionEvents|EnhancedInputActionIA_RightClick
  (params (ActionValue :type Boolean) (ElapsedSeconds :type Float%20%28double-precision%29) (TriggeredSeconds :type Float%20%28double-precision%29) (InputAction :type Input%20Action%20Object%20Reference :default "/Game/Rogue/Blueprints/Core/Player/Inputs/IA_RightClick.IA_RightClick"))
  (if ActionValue
    (CallFunction|UpdateHoveredUnitandTile)
    (Variables|Default|SetIsRightMouseDown true)
    (Utilities|IsValid (Variables|Default|GetSelectedAction_RightClick)
      (:Is%20Valid
        (Default|ExecuteAction (Variables|Default|GetSelectedAction_RightClick) (Variables|Default|GetHoveredTile))))
    (else
      (Variables|Default|SetIsRightMouseDown false))))

(event Input|EnhancedActionEvents|EnhancedInputActionIA_SelectSpell
  (params (ActionValue :type Float%20%28double-precision%29) (ElapsedSeconds :type Float%20%28double-precision%29) (TriggeredSeconds :type Float%20%28double-precision%29) (InputAction :type Input%20Action%20Object%20Reference :default "/Game/Rogue/Blueprints/Core/Player/Inputs/IA_SelectSpell.IA_SelectSpell"))
  (bind _combatsystem (Variables|References|GetCombatSystem))
  (if (Math|Boolean|ANDBoolean (Variables|/Game/Rogue/Blueprints/Core/Combat/BP_CombatSystem.BP_CombatSystem_C|GetIsInCombat _combatsystem) (not (Variables|/Game/Rogue/Blueprints/Core/Combat/BP_CombatSystem.BP_CombatSystem_C|GetIsFinishingCombat _combatsystem)) (== (Variables|/Game/Rogue/Blueprints/Core/Combat/BP_CombatSystem.BP_CombatSystem_C|GetCurrentUnit _combatsystem) (Variables|Default|GetSelectedUnit)))
    (Default|SetSelectedSpellfromIndex (Variables|/Game/Rogue/Blueprints/Core/Combat/Widget/W_Combat.W_Combat_C|GetButtonList_Spells (Variables|Default|GetW_Combat)) (- (Math|Float|Round ActionValue) 1))))

(event Input|EnhancedActionEvents|EnhancedInputActionIA_EndTurn
  (params (ActionValue :type Boolean) (ElapsedSeconds :type Float%20%28double-precision%29) (TriggeredSeconds :type Float%20%28double-precision%29) (InputAction :type Input%20Action%20Object%20Reference :default "/Game/Rogue/Blueprints/Core/Player/Inputs/IA_EndTurn.IA_EndTurn"))
  (Default|NextUnit (Variables|References|GetCombatSystem)))

(event Input|EnhancedActionEvents|EnhancedInputActionIA_LeftClick
  (params (ActionValue :type Boolean) (ElapsedSeconds :type Float%20%28double-precision%29) (TriggeredSeconds :type Float%20%28double-precision%29) (InputAction :type Input%20Action%20Object%20Reference :default "/Game/Rogue/Blueprints/Core/Player/Inputs/IA_LeftClick.IA_LeftClick"))
  (if ActionValue
    (CallFunction|UpdateHoveredUnitandTile)
    (Variables|Default|SetIsLeftMouseDown true)
    (Utilities|IsValid (Variables|Default|GetSelectedAction_LeftClick)
      (:Is%20Valid
        (Default|ExecuteAction (Variables|Default|GetSelectedAction_LeftClick) (Variables|Default|GetHoveredTile))))
    (else
      (Variables|Default|SetIsLeftMouseDown false))))

(event EventBeginPlay
  (bind _combatsystem (Variables|References|GetCombatSystem))
  (bind _combatsystem_2 (Variables|References|GetCombatSystem))
  (bind _overworldunitgroupsmanager (Variables|References|GetOverworldUnitGroupsManager))
  (Utilities|FlowControl|Sequence
    (:then_0
      (bind _output_get (Variables|References|SetGrid (Variables|/Game/Rogue/Blueprints/Core/Combat/BP_CombatSystem.BP_CombatSystem_C|GetGrid (Variables|References|GetCombatSystem))))
      (EventDispatchers|BindEventtoOnGridGenerated _output_get (EventDispatchers|CreateEvent :!event OnGridGenerated))
      (EventDispatchers|BindEventtoOnTileDataUpdated _output_get (EventDispatchers|CreateEvent :!event OnTileDataUpdated))
      (EventDispatchers|BindEventtoOnUnitGridIndexChanged (Variables|References|GetCombatSystem) (EventDispatchers|CreateEvent :!event OnUnitGridIndexChanged))
      (EventDispatchers|BindEventtoOnCombatStarted _combatsystem (EventDispatchers|CreateEvent :!event OnCombatStarted))
      (EventDispatchers|BindEventtoOnCombatEnded _combatsystem (EventDispatchers|CreateEvent :!event OnCombatEnded))
      (EventDispatchers|BindEventtoOnUnitTurnStarted _combatsystem_2 (EventDispatchers|CreateEvent :!event OnUnitTurnStarted))
      (EventDispatchers|BindEventtoOnUnitTurnEnded _combatsystem_2 (EventDispatchers|CreateEvent :!event OnUnitTurnEnded))
      (EventDispatchers|BindEventtoOnCombatFinishing (Variables|References|GetCombatSystem) (EventDispatchers|CreateEvent :!event OnCombatFinishing)))
    (:then_1
      (Input|EnableInput (Game|GetPlayerController 0))
      (Utilities|IsValid _overworldunitgroupsmanager
        (:Is%20Valid
          (Default|SetCombatSystem _overworldunitgroupsmanager (Variables|References|GetCombatSystem))
          (if (Variables|Default|GetAutoSelectOverworldMovementActions)
            (CallFunction|SetSelectedActions "/Game/Rogue/Blueprints/Core/Player/Actions/Overworld/BP_Action_SelectUnitInOverworld.BP_Action_SelectUnitInOverworld_C" "/Game/Rogue/Blueprints/Core/Player/Actions/Overworld/BP_Action_MoveUnitInOverworld.BP_Action_MoveUnitInOverworld_C")))))
    (:then_2
      ;[1 0.7762 0] Save Load Game
      (bind _returnvalue (SaveGame|DoesSaveGameExist "save1"))
      (if _returnvalue
        (bind _returnvalue_2 (SaveGame|LoadGamefromSlot "save1"))
        (bind _asbp_save (Utilities|Casting|CastToBP_Save _returnvalue_2))
        (Variables|Default|SetBP%20Save _asbp_save)
        (else
          (bind _returnvalue_3 (SaveGame|CreateSaveGameObject "/Game/Rogue/Blueprints/SaveLoad/BP_Save.BP_Save_C"))
          (Variables|/Game/Rogue/Blueprints/SaveLoad/BP_Save.BP_Save_C|SetScore _returnvalue_3 (Utilities|Struct|MakeIntPoint 0 0))
          (bind _output_get_2 (Variables|/Game/Rogue/Blueprints/SaveLoad/BP_Save.BP_Save_C|SetGlobalTimeDilation _returnvalue_3 3.0))
          (Utilities|Time|SetGlobalTimeDilation _output_get_2)
          (SaveGame|SaveGametoSlot _returnvalue_3 "save1")
          (Variables|Default|SetBP%20Save _returnvalue_3))))
    (:then_3
      ;[1 0 0] For test
      (Utilities|FlowControl|Delay 1.0)
      (Utilities|Time|SetGlobalTimeDilation (Variables|/Game/Rogue/Blueprints/SaveLoad/BP_Save.BP_Save_C|GetGlobalTimeDilation (Variables|Default|GetBP%20Save))))))

(event EventTick
  (params (DeltaSeconds :type Float%20%28single-precision%29))
  (CallFunction|UpdateHoveredUnitandTile))

(fn ConstructionScript)

(fn UpdateHoveredUnitandTile
  (Utilities|FlowControl|Sequence
    (:then_0
      (Utilities|IsValid (Variables|Default|GetHoverdUnitOverride)
        (:Is%20Valid
          (LocalVariables|SetU (Variables|Default|GetHoverdUnitOverride)))
        (:Is%20Not%20Valid
          (bind _unit (CallFunction|GetUnitUnderCursor))
          (LocalVariables|SetU _unit)))
      (if (!= (LocalVariables|GetU) (Variables|Default|GetHoveredUnit))
        (Utilities|FlowControl|Sequence
          (:then_0
            (Utilities|IsValid (Variables|Default|GetHoveredUnit)
              (:Is%20Valid
                (Default|SetIsHovered (Variables|Default|GetHoveredUnit) false))))
          (:then_1
            (bind _output_get (Variables|Default|SetHoveredUnit (LocalVariables|GetU)))
            (Utilities|IsValid _output_get
              (:Is%20Valid
                (Default|SetIsHovered _output_get true)))))))
    (:then_1
      (Utilities|IsValid (Variables|Default|GetHoveredUnit)
        (:Is%20Valid
          (LocalVariables|SetNewIndex (Variables|/Game/Rogue/Blueprints/Core/Units/BP_Unit.BP_Unit_C|GetIndex (Variables|Default|GetHoveredUnit))))
        (:Is%20Not%20Valid
          (bind _index (Default|GetTileIndexUnderCursor (Variables|References|GetGrid) 0 (CallFunction|CanHoverGround) (CallFunction|CanHoverEmptySpace)))
          (LocalVariables|SetNewIndex _index)))
      (if (!= (LocalVariables|GetNewIndex) (Variables|Default|GetHoveredTile))
        (Default|RemoveStatefromTile (Variables|References|GetGrid) (Variables|Default|GetHoveredTile) "NewEnumerator1")
        (Variables|Default|SetHoveredTile (LocalVariables|GetNewIndex))
        (Default|AddStatetoTile (Variables|References|GetGrid) (Variables|Default|GetHoveredTile) "NewEnumerator1")
        (CallFunction|EventExectuteActionwhenHoveredTileChanged)
        (Default|CallOnHoveredTileChanged (Variables|Default|GetHoveredTile))))))

(fn SetSelectedActions
  (params (Left%20Action :type BP%20Action%20Class%20Reference) (Right%20Action :type BP%20Action%20Class%20Reference))
  (Utilities|FlowControl|Sequence
    (:then_0
      (Utilities|IsValid (Variables|Default|GetSelectedAction_LeftClick)
        (:Is%20Valid
          (Actor|DestroyActor (Variables|Default|GetSelectedAction_LeftClick))
          (Variables|Default|SetSelectedAction_LeftClick 0))
        (:Is%20Not%20Valid
          _))
      (if (Utilities|IsValidClass Left%20Action)
        (bind _returnvalue (Game|SpawnActorfromClass Left%20Action (Math|Transform|MakeTransform "0, 0, 0" "0, 0, 0" "1.000000,1.000000,1.000000") "Undefined" "SelectDefaultAtRuntime" 0 self 0))
        (Variables|Default|SetSelectedAction_LeftClick _returnvalue)))
    (:then_1
      (Utilities|IsValid (Variables|Default|GetSelectedAction_RightClick)
        (:Is%20Valid
          (Actor|DestroyActor (Variables|Default|GetSelectedAction_RightClick))
          (Variables|Default|SetSelectedAction_RightClick 0))
        (:Is%20Not%20Valid
          _))
      (if (Utilities|IsValidClass Right%20Action)
        (bind _returnvalue_2 (Game|SpawnActorfromClass Right%20Action (Math|Transform|MakeTransform "0, 0, 0" "0, 0, 0" "1.000000,1.000000,1.000000") "Undefined" "SelectDefaultAtRuntime" 0 self 0))
        (Variables|Default|SetSelectedAction_RightClick _returnvalue_2)))
    (:then_2
      (Default|CallOnSelectedActionsChanged (Variables|Default|GetSelectedAction_LeftClick) (Variables|Default|GetSelectedAction_RightClick)))))

(fn GetUnitUnderCursor
  (params (PlayerIndex :type Integer))
  (bind _returnvalue (Game|GetPlayerController PlayerIndex))
  (bind (_hitresult _returnvalue_2) (Game|Player|GetHitResultUnderCursorbyChannel _returnvalue "TraceTypeQuery5" true))
  (if _returnvalue_2
    (return (.AsBP%20Unit (Utilities|Casting|CastToBP_Unit (.HitActor (Collision|BreakHitResult _hitresult)))))
    (else
      (bind _index (Default|GetTileIndexUnderCursor (Variables|References|GetGrid) PlayerIndex (CallFunction|CanHoverGround) (CallFunction|CanHoverEmptySpace)))
      (return (.UnitOnTile (Utilities|Struct|BreakS_TileDataF (.Value (Utilities|Map|Find (Variables|/Game/Rogue/Blueprints/Core/Grid/BP_Grid.BP_Grid_C|GetGrid%20Tiles (Variables|References|GetGrid)) _index))))))))

(fn SetSelectedTileandUnit
  (params (Index :type Int%20Point%20Structure) (Unit :type BP%20Unit%20Object%20Reference) (Force :type Boolean))
  (LocalVariables|SetDesired%20Index Index)
  (Utilities|IsValid Unit
    (:Is%20Valid
      (LocalVariables|SetDesired%20Index (Variables|/Game/Rogue/Blueprints/Core/Units/BP_Unit.BP_Unit_C|GetIndex Unit)))
    (:Is%20Not%20Valid
      _))
  (Utilities|FlowControl|Sequence
    (:then_0
      (if (or (!= (Variables|Default|GetSelectedTile) (LocalVariables|GetDesired%20Index)) Force) ; Different Tile?
        (Default|RemoveStatefromTile (Variables|References|GetGrid) (Variables|Default|GetSelectedTile) "NewEnumerator2")
        (Variables|Default|SetSelectedTile (LocalVariables|GetDesired%20Index))
        (Default|AddStatetoTile (Variables|References|GetGrid) (Variables|Default|GetSelectedTile) "NewEnumerator2")
        (else
          (Default|RemoveStatefromTile (Variables|References|GetGrid) (Variables|Default|GetSelectedTile) "NewEnumerator2")
          (Variables|Default|SetSelectedTile (Utilities|Struct|MakeIntPoint -999 -999))))
      (Default|CallOnSelectedTileChanged (Variables|Default|GetSelectedTile)))
    (:then_1
      (LocalVariables|SetNewUnit (select (Utilities|IsValid Unit) Unit (.UnitOnTile (Utilities|Struct|BreakS_TileDataF (.Value (Utilities|Map|Find (Variables|/Game/Rogue/Blueprints/Core/Grid/BP_Grid.BP_Grid_C|GetGrid%20Tiles (Variables|References|GetGrid)) (Variables|Default|GetSelectedTile)))))))
      (if (or (!= (Variables|Default|GetSelectedUnit) (LocalVariables|GetNewUnit)) Force)
        (Utilities|FlowControl|Sequence
          (:then_0
            (Utilities|IsValid (Variables|Default|GetSelectedUnit)
              (:Is%20Valid
                (Default|SetIsSelected (Variables|Default|GetSelectedUnit) false))))
          (:then_1
            (bind _output_get (Variables|Default|SetSelectedUnit (LocalVariables|GetNewUnit)))
            (Utilities|IsValid _output_get
              (:Is%20Valid
                (Default|SetIsSelected _output_get true)))))))))

(fn OnGridGenerated
  (if (Default|IsIndexValid (Variables|References|GetGrid) (Variables|Default|GetSelectedTile))
    (CallFunction|SetSelectedTileandUnit (Variables|Default|GetSelectedTile) 0 true)
    (else
      (CallFunction|SetSelectedTileandUnit (Utilities|Struct|MakeIntPoint -999 -999) 0 true))))

(fn OnTileDataUpdated
  (params (Index :type Int%20Point%20Structure))
  (if (Class|KismetMathLibrary|EqualIntPointIntPoint Index (Variables|Default|GetSelectedTile))
    (CallFunction|OnGridGenerated)))

(fn OnUnitGridIndexChanged
  (params (Unit :type BP%20Unit%20Object%20Reference))
  (if (== Unit (Variables|Default|GetSelectedUnit))
    (CallFunction|SetSelectedTileandUnit (Variables|/Game/Rogue/Blueprints/Core/Units/BP_Unit.BP_Unit_C|GetIndex Unit) 0 false)))

(fn OnCombatStarted
  (CallFunction|SetSelectedActions)
  (CallFunction|SetSelectedTileandUnit (Utilities|Struct|MakeIntPoint -999 -999) 0 false)
  (bind _returnvalue (Game|ConstructObjectfromClass "/Game/Rogue/Blueprints/Core/Combat/Widget/W_Combat.W_Combat_C" self))
  (bind _output_get (Variables|Default|SetW_Combat _returnvalue))
  (UserInterface|Viewport|AddtoViewport _output_get 0)
  (EventDispatchers|BindEventtoOnSelectedSpellButtonChanged (Variables|/Game/Rogue/Blueprints/Core/Combat/Widget/W_Combat.W_Combat_C|GetButtonList_Spells (Variables|Default|GetW_Combat)) (EventDispatchers|CreateEvent :!event OnSelectedSpellChanged)))

(fn OnCombatEnded
  (Widget|RemovefromParent (Variables|Default|GetW_CombatEndScreen))
  (Variables|Default|SetW_CombatEndScreen 0)
  (if (Variables|Default|GetAutoSelectOverworldMovementActions)
    (CallFunction|SetSelectedActions "/Game/Rogue/Blueprints/Core/Player/Actions/Overworld/BP_Action_SelectUnitInOverworld.BP_Action_SelectUnitInOverworld_C" "/Game/Rogue/Blueprints/Core/Player/Actions/Overworld/BP_Action_MoveUnitInOverworld.BP_Action_MoveUnitInOverworld_C")
    (else
      (CallFunction|SetSelectedActions))))

(fn OnUnitTurnStarted
  (params (Unit :type BP%20Unit%20Object%20Reference))
  (Utilities|IsValid (Variables|/Game/Rogue/Blueprints/Core/Units/BP_Unit.BP_Unit_C|GetAI Unit)
    (:Is%20Valid
      (if (!= (Utilities|GetClass (Variables|Default|GetSelectedAction_LeftClick)) "/Game/Rogue/Blueprints/Core/Player/Actions/Combat/Action_Cbt_WaitForTurn.Action_Cbt_WaitForTurn_C")
        (CallFunction|SetSelectedActions "/Game/Rogue/Blueprints/Core/Player/Actions/Combat/Action_Cbt_WaitForTurn.Action_Cbt_WaitForTurn_C")))
    (:Is%20Not%20Valid
      (CallFunction|SetSelectedTileandUnit (Variables|/Game/Rogue/Blueprints/Core/Units/BP_Unit.BP_Unit_C|GetIndex Unit) 0 false)
      (CallFunction|SetSelectedActions "/Game/Rogue/Blueprints/Core/Player/Actions/Combat/Action_Cbt_Move.Action_Cbt_Move_C")
      (Default|LinkUnittoSpellList (Variables|/Game/Rogue/Blueprints/Core/Combat/Widget/W_Combat.W_Combat_C|GetButtonList_Spells (Variables|Default|GetW_Combat)) (Variables|Default|GetSelectedUnit)))))

(fn OnUnitTurnEnded
  (params (Unit :type BP%20Unit%20Object%20Reference))
  (CallFunction|SetSelectedTileandUnit (Utilities|Struct|MakeIntPoint -999 -999) 0 false)
  (Default|LinkUnittoSpellList (Variables|/Game/Rogue/Blueprints/Core/Combat/Widget/W_Combat.W_Combat_C|GetButtonList_Spells (Variables|Default|GetW_Combat))))

(fn OnSelectedSpellChanged
  (params (Button :type Button%20Spell%20Object%20Reference))
  (Utilities|IsValid Button
    (:Is%20Valid
      (CallFunction|SetSelectedActions "/Game/Rogue/Blueprints/Core/Player/Actions/Combat/Action_Cbt_CastSpell.Action_Cbt_CastSpell_C")
      (bind _asaction_cbt_cast_spell (Utilities|Casting|CastToAction_Cbt_CastSpell (Variables|Default|GetSelectedAction_LeftClick)))
      (Default|SetSpell _asaction_cbt_cast_spell (Variables|/Game/Rogue/Blueprints/Core/Combat/Spells/Widgets/Button_Spell.Button_Spell_C|GetSpell Button)))
    (:Is%20Not%20Valid
      (if (!= (Utilities|GetClass (Variables|Default|GetSelectedAction_LeftClick)) "/Game/Rogue/Blueprints/Core/Player/Actions/Combat/Action_Cbt_Move.Action_Cbt_Move_C")
        (CallFunction|SetSelectedActions "/Game/Rogue/Blueprints/Core/Player/Actions/Combat/Action_Cbt_Move.Action_Cbt_Move_C")))))

(fn OnCombatFinishing
  (CallFunction|SetSelectedActions)
  (CallFunction|SetSelectedTileandUnit (Utilities|Struct|MakeIntPoint -999 -999) 0 false)
  (Widget|RemovefromParent (Variables|Default|GetW_Combat))
  (Variables|Default|SetW_Combat 0)
  (bind _returnvalue (UserInterface|CreateWidget "/Game/Rogue/Blueprints/Core/Combat/Widget/W_CombatEndScreen.W_CombatEndScreen_C" 0 self (Variables|/Game/Rogue/Blueprints/Core/Combat/BP_CombatSystem.BP_CombatSystem_C|GetTeam%20Index%20That%20Won%20Last (Variables|References|GetCombatSystem))))
  (bind _output_get (Variables|Default|SetW_CombatEndScreen _returnvalue))
  (UserInterface|Viewport|AddtoViewport _output_get 0))

(fn SetHoveredUnitOverride
  (params (Unit :type BP%20Unit%20Object%20Reference))
  (Variables|Default|SetHoverdUnitOverride Unit)
  (CallFunction|UpdateHoveredUnitandTile))

(fn CanHoverGround
  (bind _selectedaction_leftclick (Variables|Default|GetSelectedAction_LeftClick))
  (bind _selectedaction_rightclick (Variables|Default|GetSelectedAction_RightClick))
  (bind _returnvalue (Utilities|GetClass _selectedaction_rightclick))
  (bind _returnvalue_2 (Utilities|GetClass _selectedaction_leftclick))
  (bind _array (Utilities|Array|MakeArray _returnvalue_2 _returnvalue))
  (return (or (Utilities|Array|ContainsItem _array "/Game/Rogue/Blueprints/Core/Player/Actions/Overworld/BP_Action_AddRemoveUnitFromOverworld.BP_Action_AddRemoveUnitFromOverworld_C") (Utilities|Array|ContainsItem _array "/Game/Rogue/Blueprints/Core/Player/Actions/Overworld/BP_Action_MoveUnitInOverworld.BP_Action_MoveUnitInOverworld_C"))))

(fn CanHoverEmptySpace
  (return (Utilities|Array|ContainsItem (Utilities|Array|MakeArray (Utilities|GetClass (Variables|Default|GetSelectedAction_LeftClick)) (Utilities|GetClass (Variables|Default|GetSelectedAction_RightClick))) "/Game/Rogue/Blueprints/Core/Player/Actions/Grid/Action_AddTile.Action_AddTile_C")))