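; Actor that holds the player's inventory and restores persistent run data from the Rogue game instance's save object.
; On BeginPlay it checks the "save1" slot and either loads non-empty saved inventory into its inventory component or saves, then initializes score, XP and global time dilation.
; It then copies player units and the rogue map from the save.
; A getter exposes the inventory component.
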(event EventBeginPlay
  (Utilities|FlowControl|Sequence
    (:then_0
      (bind _asrogue_game_instance (Utilities|Casting|CastToRogueGameInstance (Game|GetGameInstance)))
      (Variables|Default|SetAs%20Rogue%20Game%20Instance _asrogue_game_instance))
    (:then_1
      ;[1 0.7762 0] Save Load Game
      (bind _returnvalue (SaveGame|DoesSaveGameExist "save1"))
      (if _returnvalue
        (if (not (Utilities|Array|IsEmpty (Variables|/Game/Rogue/Blueprints/SaveLoad/BP_Save.BP_Save_C|GetInventoryContent (Variables|/Game/Rogue/Blueprints/Core/Player/RogueGameInstance.RogueGameInstance_C|GetBP%20Save (Variables|Default|GetAs%20Rogue%20Game%20Instance)))))
          (Variables|/Game/Inventory/BPC_Inventory.BPC_Inventory_C|SetContent (Variables|Default|GetBPC_Inventory) (Variables|/Game/Rogue/Blueprints/SaveLoad/BP_Save.BP_Save_C|GetInventoryContent (Variables|/Game/Rogue/Blueprints/Core/Player/RogueGameInstance.RogueGameInstance_C|GetBP%20Save (Variables|Default|GetAs%20Rogue%20Game%20Instance)))))
        (else
          (Default|SaveGame (Variables|Default|GetAs%20Rogue%20Game%20Instance))
          (Variables|/Game/Rogue/Blueprints/SaveLoad/BP_Save.BP_Save_C|SetScore (Variables|/Game/Rogue/Blueprints/Core/Player/RogueGameInstance.RogueGameInstance_C|GetBP%20Save (Variables|Default|GetAs%20Rogue%20Game%20Instance)) (Utilities|Struct|MakeIntPoint 0 0))
          (bind _output_get (Variables|/Game/Rogue/Blueprints/SaveLoad/BP_Save.BP_Save_C|SetGlobalTimeDilation (Variables|/Game/Rogue/Blueprints/Core/Player/RogueGameInstance.RogueGameInstance_C|GetBP%20Save (Variables|Default|GetAs%20Rogue%20Game%20Instance)) 3.0))
          (Utilities|Time|SetGlobalTimeDilation _output_get)
          (Variables|/Game/Rogue/Blueprints/SaveLoad/BP_Save.BP_Save_C|SetPlayerExp (Variables|/Game/Rogue/Blueprints/Core/Player/RogueGameInstance.RogueGameInstance_C|GetBP%20Save (Variables|Default|GetAs%20Rogue%20Game%20Instance)) 0))))
    (:then_2
      (Variables|Default|SetPlayer%20Units (Variables|/Game/Rogue/Blueprints/SaveLoad/BP_Save.BP_Save_C|GetPlayerUnits (Variables|/Game/Rogue/Blueprints/Core/Player/RogueGameInstance.RogueGameInstance_C|GetBP%20Save (Variables|Default|GetAs%20Rogue%20Game%20Instance))))
      (Variables|Default|SetRogueMap (Variables|/Game/Rogue/Blueprints/SaveLoad/BP_Save.BP_Save_C|GetRogueMap (Variables|/Game/Rogue/Blueprints/Core/Player/RogueGameInstance.RogueGameInstance_C|GetBP%20Save (Variables|Default|GetAs%20Rogue%20Game%20Instance)))))))

(fn ConstructionScript)

(fn GetPlayerInventoryRef
  (return (Variables|Default|GetBPC_Inventory)))