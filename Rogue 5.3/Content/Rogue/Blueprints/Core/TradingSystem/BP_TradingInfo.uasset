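; BP_TradingInfo runs the shop screen: it opens the player inventory, forwards its input, plays music and manages trade offers.
; BeginPlay loads or creates BP_Save, gathers for-sale and unlocked items, and spawns saved units far from itself.
; Trade functions fill WTrades with non-duplicate, capped buy/sell offers, with prices randomized from DT_Item base values.
; SaveAll writes inventory and units back to the save, sharing it with BP_PlayerInventoryHolder.
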(event Input|EnhancedActionEvents|EnhancedInputActionIA_TakeItem
  (params (ActionValue :type Boolean) (ElapsedSeconds :type Float%20%28double-precision%29) (TriggeredSeconds :type Float%20%28double-precision%29) (InputAction :type Input%20Action%20Object%20Reference :default "/Game/Inventory/Input/IA_TakeItem.IA_TakeItem"))
  ;[1 1 1] Input
  (Default|EventTakeItem (Variables|Default|GetPlayer%20Inventory)))

(event Input|EnhancedActionEvents|EnhancedInputActionIA_Drop1Item
  (params (ActionValue :type Boolean) (ElapsedSeconds :type Float%20%28double-precision%29) (TriggeredSeconds :type Float%20%28double-precision%29) (InputAction :type Input%20Action%20Object%20Reference :default "/Game/Inventory/Input/IA_Drop1Item.IA_Drop1Item"))
  (bind _player_inventory (Variables|Default|GetPlayer%20Inventory))
  ;[1 1 1] Input
  (if (Variables|/Game/Inventory/BPC_Inventory.BPC_Inventory_C|GetisInventoryVisible? _player_inventory)
    (Default|EventDrop1Item _player_inventory)))

(event Input|EnhancedActionEvents|EnhancedInputActionIA_LeftClick
  (params (ActionValue :type Boolean) (ElapsedSeconds :type Float%20%28double-precision%29) (TriggeredSeconds :type Float%20%28double-precision%29) (InputAction :type Input%20Action%20Object%20Reference :default "/Game/Rogue/Blueprints/Core/Player/Inputs/IA_LeftClick.IA_LeftClick"))
  ;[1 1 1] Input
)

(event Input|EnhancedActionEvents|EnhancedInputActionIA_MarkItem
  (params (ActionValue :type Boolean) (ElapsedSeconds :type Float%20%28double-precision%29) (TriggeredSeconds :type Float%20%28double-precision%29) (InputAction :type Input%20Action%20Object%20Reference :default "/Game/Inventory/Input/IA_MarkItem.IA_MarkItem"))
  (bind _player_inventory (Variables|Default|GetPlayer%20Inventory))
  ;[1 1 1] Input
  (if (Variables|/Game/Inventory/BPC_Inventory.BPC_Inventory_C|GetisInventoryVisible? _player_inventory)
    (Default|EventToggleSell _player_inventory)))

(event Input|EnhancedActionEvents|EnhancedInputActionIA_DropAllItem
  (params (ActionValue :type Boolean) (ElapsedSeconds :type Float%20%28double-precision%29) (TriggeredSeconds :type Float%20%28double-precision%29) (InputAction :type Input%20Action%20Object%20Reference :default "/Game/Inventory/Input/IA_DropAllItem.IA_DropAllItem"))
  (bind _player_inventory (Variables|Default|GetPlayer%20Inventory))
  ;[1 1 1] Input
  (if (Variables|/Game/Inventory/BPC_Inventory.BPC_Inventory_C|GetisInventoryVisible? _player_inventory)
    (Default|EventDropAllItem _player_inventory)))

(event Input|EnhancedActionEvents|EnhancedInputActionIA_UseItem
  (params (ActionValue :type Boolean) (ElapsedSeconds :type Float%20%28double-precision%29) (TriggeredSeconds :type Float%20%28double-precision%29) (InputAction :type Input%20Action%20Object%20Reference :default "/Game/Inventory/Input/IA_UseItem.IA_UseItem"))
  (bind _player_inventory (Variables|Default|GetPlayer%20Inventory))
  ;[1 1 1] Input
  (if (Variables|/Game/Inventory/BPC_Inventory.BPC_Inventory_C|GetisInventoryVisible? _player_inventory)
    (Default|EventUseItem _player_inventory)))

(event Input|EnhancedActionEvents|EnhancedInputActionIA_Share1Item
  (params (ActionValue :type Boolean) (ElapsedSeconds :type Float%20%28double-precision%29) (TriggeredSeconds :type Float%20%28double-precision%29) (InputAction :type Input%20Action%20Object%20Reference :default "/Game/Inventory/Input/IA_Share1Item.IA_Share1Item"))
  (bind _player_inventory (Variables|Default|GetPlayer%20Inventory))
  ;[1 1 1] Input
  (if (Variables|/Game/Inventory/BPC_Inventory.BPC_Inventory_C|GetisInventoryVisible? _player_inventory)
    (Default|EventShare1Item _player_inventory)))

(event Input|EnhancedActionEvents|EnhancedInputActionIA_ShareHalfItem
  (params (ActionValue :type Boolean) (ElapsedSeconds :type Float%20%28double-precision%29) (TriggeredSeconds :type Float%20%28double-precision%29) (InputAction :type Input%20Action%20Object%20Reference :default "/Game/Inventory/Input/IA_ShareHalfItem.IA_ShareHalfItem"))
  (bind _player_inventory (Variables|Default|GetPlayer%20Inventory))
  ;[1 1 1] Input
  (if (Variables|/Game/Inventory/BPC_Inventory.BPC_Inventory_C|GetisInventoryVisible? _player_inventory)
    (Default|EventShareHalfItem _player_inventory)))

(event Input|EnhancedActionEvents|EnhancedInputActionIA_OpenInventory
  (params (ActionValue :type Boolean) (ElapsedSeconds :type Float%20%28double-precision%29) (TriggeredSeconds :type Float%20%28double-precision%29) (InputAction :type Input%20Action%20Object%20Reference :default "/Game/Inventory/Input/IA_OpenInventory.IA_OpenInventory"))
  ;[1 1 1] Input
  (Default|EventOpenInventory (Variables|Default|GetPlayer%20Inventory)))

(event Input|EnhancedActionEvents|EnhancedInputActionIA_InspectItem
  (params (ActionValue :type Boolean) (ElapsedSeconds :type Float%20%28double-precision%29) (TriggeredSeconds :type Float%20%28double-precision%29) (InputAction :type Input%20Action%20Object%20Reference :default "/Game/Inventory/Input/IA_InspectItem.IA_InspectItem"))
  ;[1 1 1] Input
  (Default|EventInspectItem (Variables|Default|GetPlayer%20Inventory)))

(event EventBeginPlay
  (Utilities|FlowControl|Sequence
    (:then_0
      (bind _returnvalue (Actor|GetActorOfClass "/Game/Rogue/Blueprints/Core/Player/BP_PlayerInventoryHolder.BP_PlayerInventoryHolder_C"))
      (bind _playerinventory (Default|GetPlayerInventoryRef _returnvalue))
      (Variables|Default|SetPlayer%20Inventory _playerinventory)
      (Input|EnableInput (Game|GetPlayerController 0)))
    (:then_1
      (bind _returnvalue_2 (SaveGame|DoesSaveGameExist "save1"))
      (if _returnvalue_2
        (bind _returnvalue_3 (SaveGame|LoadGamefromSlot "save1"))
        (bind _asbp_save (Utilities|Casting|CastToBP_Save _returnvalue_3))
        (Variables|Default|SetBP%20Save _asbp_save)
        (else
          (bind _returnvalue_4 (SaveGame|CreateSaveGameObject "/Game/Rogue/Blueprints/SaveLoad/BP_Save.BP_Save_C"))
          (Variables|/Game/Rogue/Blueprints/SaveLoad/BP_Save.BP_Save_C|SetScore _returnvalue_4 (Utilities|Struct|MakeIntPoint 0 0))
          (Variables|/Game/Rogue/Blueprints/SaveLoad/BP_Save.BP_Save_C|SetPlayerExp _returnvalue_4 0)
          (SaveGame|SaveGametoSlot _returnvalue_4 "save1")
          (Variables|Default|SetBP%20Save _returnvalue_4))))
    (:then_2
      (Utilities|Array|Clear (Variables|Default|GetForSellItems))
      (for _array_element (Variables|/Game/Inventory/BPC_Inventory.BPC_Inventory_C|GetContent (Variables|Default|GetPlayer%20Inventory))
        (if (and (!= (.ItemID (Utilities|Struct|BreakS_Slot _array_element)) "") (.ForSell? (Utilities|Struct|BreakS_Slot _array_element)))
          (Utilities|Array|Add (Variables|Default|GetForSellItems) _array_element))))
    (:then_3
      (if (not (or (== (Utilities|Array|Length (Variables|/Game/Rogue/Blueprints/SaveLoad/BP_Save.BP_Save_C|GetPlayerUnits (Variables|Default|GetBP%20Save))) 0) (Variables|/Game/Rogue/Blueprints/SaveLoad/BP_Save.BP_Save_C|GetStartFromZero? (Variables|Default|GetBP%20Save))))
        (for (_array_element_2 _array_index) (Variables|/Game/Rogue/Blueprints/SaveLoad/BP_Save.BP_Save_C|GetPlayerUnits (Variables|Default|GetBP%20Save))
          (bind _returnvalue_5 (Game|SpawnActorfromClass "/Game/Rogue/Blueprints/Core/Units/BP_Unit.BP_Unit_C" (Math|Transform|MakeTransform (+ (Transformation|GetActorLocation) "10000.000000,10000.000000,0.000000") "0.000000,-90.000000,0.000000") "Undefined" "MultiplyWithRoot" 0 (.UnitType (Utilities|Struct|BreakS_UnitSaveLoad _array_element_2)) true 0 0))
          (Variables|/Game/Rogue/Blueprints/Core/Units/BP_Unit.BP_Unit_C|SetItems _returnvalue_5 (.InvContent (Utilities|Struct|BreakS_UnitSaveLoad _array_element_2)))
          (Variables|/Game/Rogue/Blueprints/Core/Units/BP_Unit.BP_Unit_C|SetAllyIndex _returnvalue_5 _array_index)
          (Default|SetTeamIndex _returnvalue_5)
          (Variables|/Game/Rogue/Blueprints/Core/Units/BP_Unit.BP_Unit_C|SetUpdTalents _returnvalue_5 (.TalentAmount (Utilities|Struct|BreakS_UnitSaveLoad _array_element_2)))
          (Utilities|Array|Add (Variables|Default|GetPlayerUnits) _returnvalue_5)
          (Variables|/Game/Rogue/Blueprints/Core/Units/BP_Unit.BP_Unit_C|SetTalents _returnvalue_5 (.SaveLoadTalents (Utilities|Struct|BreakS_UnitSaveLoad _array_element_2)))
          (Default|RefreshAllStats _returnvalue_5 false false))))
    (:then_4
      (Utilities|Array|Clear (Variables|Default|GetAllBuyItems))
      (bind _items (Additional|GetAvailableItemsSorted))
      (for _array_element_3 _items
        (Utilities|Array|Add (Variables|Default|GetAllBuyItems) (Utilities|Struct|MakeS_Slot (Additional|ItemNametoNameFunc _array_element_3) 1 false))))
    (:then_5
      (bind _returnvalue_6 (Actor|GetActorOfClass "/Game/Rogue/Blueprints/Core/Player/RoguePawn.RoguePawn_C"))
      (Variables|Components|SetPlayer _returnvalue_6)
      (Class|GameplayStatics|SetBaseSoundMix "/Game/Rogue/Sounds/Master_SoundMixClass.Master_SoundMixClass")
      (Music|PlayMusic "/Game/Sound/Music_audio/Elven_Harmonies_Cue.Elven_Harmonies_Cue" 0.2))
    (:then_6
      (Utilities|FlowControl|Delay 0.01)
      (Default|EventOpenInventory (Variables|Default|GetPlayer%20Inventory))
      (bind _aswb_player_menu (Utilities|Casting|CastToWB_PlayerMenu (Variables|/Game/Inventory/UI/WB_PlayerHUD.WB_PlayerHUD_C|GetPlayerMenu (Variables|/Game/Inventory/BPC_Inventory.BPC_Inventory_C|GetHUD (Variables|Default|GetPlayer%20Inventory)))))
      (Variables|Default|SetAs%20WB%20Player%20Menu _aswb_player_menu))))

(event EventOnPopUpAppear
  (Music|PlaySound "/Game/Sound/Interface_And_Item_Sounds/WAV/Click_07_Cue.Click_07_Cue" 0.15))

(event EventOnButtonClicked
  (Music|PlaySound "/Game/Sound/Interface_And_Item_Sounds/WAV/Musical_Click_08_Cue.Musical_Click_08_Cue" 0.4))

(fn ConstructionScript)

(fn GenerateSellPrice
  (params (Item :type S%20Slot%20Structure))
  (bind (_item _found_) (Additional|GetDatafromSlot Item))
  (if _found_
    (return (Math|Float|Round (* (.Price (Utilities|Struct|BreakS_Item _item)) (Math|Random|RandomFloatinRange (Variables|Default|GetSellMinCoef) (Variables|Default|GetSellMaxCoef)))) true)
    (else
      (return 0 false))))

(fn GetDatafromSlot
  (params (Slot :type S%20Slot%20Structure))
  (bind _returnvalue (Utilities|GetDataTableRow "/Game/Inventory/DT_Item.DT_Item" (.ItemID (Utilities|Struct|BreakS_Slot Slot)))
    (:then
      (return _returnvalue true))
    (:RowNotFound
      (return "" false))))

(fn GenerateBuyPrice
  (params (Item :type S%20Slot%20Structure))
  (bind (_item _found_) (Additional|GetDatafromSlot Item))
  (if _found_
    (return (Math|Float|Round (* (.Price (Utilities|Struct|BreakS_Item _item)) (Math|Random|RandomFloatinRange (Variables|Default|GetBuyMinCoef) (Variables|Default|GetBuyMaxCoef)))) true)
    (else
      (return 0 false))))

(fn GetAvailableItemsSorted
  (return (Variables|/Game/Rogue/Blueprints/SaveLoad/BP_Save.BP_Save_C|GetItemsUnlocked (Variables|Default|GetBP%20Save))))

(fn GetAvailableTalents
  (bind _outrownames (DataTable|GetDataTableRowNames "/Game/Rogue/Blueprints/Core/TalentSystem/DT_Talents.DT_Talents"))
  (for _array_element _outrownames
    (bind _returnvalue (Utilities|GetDataTableRow "/Game/Rogue/Blueprints/Core/TalentSystem/DT_Talents.DT_Talents" _array_element)
      (:then
        (if (<= (.TalentTier (Utilities|Struct|BreakS_TalentInfo _returnvalue)) (+ (Variables|/Game/Rogue/Blueprints/SaveLoad/BP_Save.BP_Save_C|GetTierUpgrades (Variables|Default|GetBP%20Save)) 2))
          (Utilities|Array|Add (LocalVariables|GetTalentsArray) (.Talent (Utilities|Struct|BreakS_TalentInfo _returnvalue)))))))
  (return (LocalVariables|GetTalentsArray)))

(fn GetAvailableCompanionsSorted
  (return (Variables|/Game/Rogue/Blueprints/SaveLoad/BP_Save.BP_Save_C|GetCompanions (Variables|Default|GetBP%20Save))))

(fn ItemNametoNameFunc
  (params (ItemName :type E_ItemName%20Enum :default "NewEnumerator14"))
  (return (Utilities|String|StringToName (Utilities|String|Replace (Utilities|String|EnumtoString ItemName) " "))))

(fn GenerateSellBuy
  (params (ForMoney? :type Boolean))
  (bind _w_trades (Variables|UI|GetW_Trades))
  (bind _w_trades_2 (Variables|UI|GetW_Trades))
  (if (< (+ (Variables|/Game/Rogue/Blueprints/Core/TradingSystem/W_Trades.W_Trades_C|GetNumOfBuy _w_trades) (Variables|/Game/Rogue/Blueprints/Core/TradingSystem/W_Trades.W_Trades_C|GetNumOfSell _w_trades)) (* (Variables|Default|GetMaxNumOfCertaintTrades) 2))
    (if (Utilities|Array|IsEmpty (Variables|Default|GetForSellItems))
      _
      (else
        (bind _notsold (Shop|ArrayIntersectionSell (Variables|/Game/Rogue/Blueprints/Core/TradingSystem/W_Trades.W_Trades_C|GetSellingTrades (Variables|UI|GetW_Trades)) (Variables|Default|GetForSellItems)))
        (if (and (!= (Utilities|Array|Length _notsold) 0) (< (Variables|/Game/Rogue/Blueprints/Core/TradingSystem/W_Trades.W_Trades_C|GetNumOfSell (Variables|UI|GetW_Trades)) (Variables|Default|GetMaxNumOfCertaintTrades)))
          (if (Math|Random|RandomBool)
            _
            (else
              (Default|AddNewSell _w_trades_2 ForMoney? _notsold)
              (return true))))))
    (bind _notsold_2 (Shop|ArrayIntersectionSell (Variables|/Game/Rogue/Blueprints/Core/TradingSystem/W_Trades.W_Trades_C|GetBuyingTrades (Variables|UI|GetW_Trades)) (Variables|Default|GetAllBuyItems)))
    (if (and (< (Variables|/Game/Rogue/Blueprints/Core/TradingSystem/W_Trades.W_Trades_C|GetNumOfBuy (Variables|UI|GetW_Trades)) (Variables|Default|GetMaxNumOfCertaintTrades)) (!= (Utilities|Array|Length _notsold_2) 0))
      (Default|AddNewBuy _w_trades_2 ForMoney? _notsold_2)
      (return true)
      (else
        (return false)))
    (else
      (return false))))

(fn PlaySound
  (params (Sound :type Sound%20Base%20Object%20Reference) (VolumeMultiplier :type Float%20%28single-precision%29))
  (bind _returnvalue (Audio|SpawnSound2D Sound 1.0 1.0 0.0 0))
  (Audio|Components|Audio|FadeOut _returnvalue VolumeMultiplier 0.0 "Linear" :!class /Script/Engine.AudioComponent))

(fn RefreshSellBuy
  (params (ForMoney? :type Boolean))
  (bind _w_trades (Variables|UI|GetW_Trades))
  (LocalVariables|SetBuyNum (Variables|/Game/Rogue/Blueprints/Core/TradingSystem/W_Trades.W_Trades_C|GetNumOfBuy _w_trades))
  (LocalVariables|SetSellNum (Variables|/Game/Rogue/Blueprints/Core/TradingSystem/W_Trades.W_Trades_C|GetNumOfSell _w_trades))
  (Default|RefreshAll (Variables|UI|GetW_Trades))
  (if (!= (LocalVariables|GetBuyNum) 0)
    (Utilities|FlowControl|ForLoopwithBreak 0 (- (LocalVariables|GetBuyNum) 1)
      (:LoopBody
        (bind (_added_ _items) (Shop|GenerateBuy false))
        (if _added_
          (Default|AddNewBuy (Variables|UI|GetW_Trades) false _items)))
      (:Completed
        (if (!= (LocalVariables|GetSellNum) 0) :!label _label
          (Utilities|FlowControl|ForLoopwithBreak 0 (- (LocalVariables|GetSellNum) 1)
            (:LoopBody
              (if (Utilities|Array|IsEmpty (Variables|Default|GetForSellItems))
                (bind (_added__2 _items_2) (Shop|GenerateSell false))
                (if _added__2
                  (Default|AddNewSell (Variables|UI|GetW_Trades) ForMoney? _items_2))))))))
    (else
      (goto _label))))

(fn SpawnAllyUnitsfromZero)

(fn SaveAll
  (Variables|/Game/Rogue/Blueprints/SaveLoad/BP_Save.BP_Save_C|SetInventoryContent (Variables|Default|GetBP%20Save) (Variables|/Game/Inventory/BPC_Inventory.BPC_Inventory_C|GetContent (Variables|Default|GetPlayer%20Inventory)))
  (for _array_element (Variables|Default|GetPlayerUnits)
    (Utilities|Array|Add (LocalVariables|GetPlayerUnitsData) (Utilities|Struct|MakeS_UnitSaveLoad (.UnitName (Utilities|Struct|BreakS_UnitDataF (Variables|/Game/Rogue/Blueprints/Core/Units/BP_Unit.BP_Unit_C|GetUnitData _array_element))) (Variables|/Game/Rogue/Blueprints/Core/Units/BP_Unit.BP_Unit_C|GetTalents _array_element) (Variables|/Game/Rogue/Blueprints/Core/Units/BP_Unit.BP_Unit_C|GetUpdTalents _array_element) (Variables|/Game/Rogue/Blueprints/Core/Units/BP_Unit.BP_Unit_C|GetItems _array_element) (.Stats (Utilities|Struct|BreakS_UnitDataF (Variables|/Game/Rogue/Blueprints/Core/Units/BP_Unit.BP_Unit_C|GetUnitData _array_element))))))
  (Variables|/Game/Rogue/Blueprints/SaveLoad/BP_Save.BP_Save_C|SetPlayerUnits (Variables|Default|GetBP%20Save) (LocalVariables|GetPlayerUnitsData))
  (CallFunction|ShareSaveGame)
  (Utilities|SaveGame))

(fn UpdateResourceValues
  (params (PlayerMenu :type WB%20Player%20Menu%20Object%20Reference))
  (Default|UpdateResourceValues (Variables|/Game/Inventory/UI/WB_PlayerMenu.WB_PlayerMenu_C|GetWB_PlayerResources PlayerMenu) PlayerMenu)
  (Default|UpdateResourceValues (Variables|/Game/Inventory/UI/WB_PlayerMenu.WB_PlayerMenu_C|GetWB_PlayerResources_1 PlayerMenu) PlayerMenu))

(fn ArrayIntersectionSell
  (params (MapAlready :type Array%20of%20S%20Slot%20Structures) (MapAll :type Array%20of%20S%20Slot%20Structures))
  (LocalVariables|SetAllItems MapAll)
  (for _array_element MapAlready
    (LocalVariables|SetItem1 _array_element)
    (for _array_element_2 MapAll
      (LocalVariables|SetItem2 _array_element_2)
      (if (Math|Boolean|ANDBoolean (== (.ItemID (Utilities|Struct|BreakS_Slot (LocalVariables|GetItem1))) (.ItemID (Utilities|Struct|BreakS_Slot (LocalVariables|GetItem2)))) (== (.Quantity (Utilities|Struct|BreakS_Slot (LocalVariables|GetItem1))) (.Quantity (Utilities|Struct|BreakS_Slot (LocalVariables|GetItem2)))) (== (.ForSell? (Utilities|Struct|BreakS_Slot (LocalVariables|GetItem1))) (.ForSell? (Utilities|Struct|BreakS_Slot (LocalVariables|GetItem2)))))
        (Utilities|Array|RemoveItem (LocalVariables|GetAllItems) (LocalVariables|GetItem2)))))
  (return (LocalVariables|GetAllItems)))

(fn SaveGameFunc
  (bind _returnvalue (SaveGame|DoesSaveGameExist "save1"))
  (if _returnvalue
    (SaveGame|SaveGametoSlot (Variables|Default|GetBP%20Save) "save1")))

(fn ShareSaveGame
  (bind _returnvalue (Actor|GetActorOfClass "/Game/Rogue/Blueprints/Core/Player/BP_PlayerInventoryHolder.BP_PlayerInventoryHolder_C"))
  (Variables|/Game/Rogue/Blueprints/Core/Player/BP_PlayerInventoryHolder.BP_PlayerInventoryHolder_C|SetBP%20Save _returnvalue (Variables|Default|GetBP%20Save)))

(fn GenerateSell
  (params (ForMoney? :type Boolean))
  (bind _w_trades (Variables|UI|GetW_Trades))
  (if (< (+ (Variables|/Game/Rogue/Blueprints/Core/TradingSystem/W_Trades.W_Trades_C|GetNumOfBuy _w_trades) (Variables|/Game/Rogue/Blueprints/Core/TradingSystem/W_Trades.W_Trades_C|GetNumOfSell _w_trades)) (* (Variables|Default|GetMaxNumOfCertaintTrades) 2))
    (if (Utilities|Array|IsEmpty (Variables|Default|GetForSellItems))
      (return false 0)
      (else
        (bind _notsold (Shop|ArrayIntersectionSell (Variables|/Game/Rogue/Blueprints/Core/TradingSystem/W_Trades.W_Trades_C|GetSellingTrades (Variables|UI|GetW_Trades)) (Variables|Default|GetForSellItems)))
        (if (and (!= (Utilities|Array|Length _notsold) 0) (< (Variables|/Game/Rogue/Blueprints/Core/TradingSystem/W_Trades.W_Trades_C|GetNumOfSell (Variables|UI|GetW_Trades)) (Variables|Default|GetMaxNumOfCertaintTrades)))
          (return true _notsold)
          (else
            (return false 0)))))
    (else
      (return false 0))))

(fn GenerateBuy
  (params (ForMoney? :type Boolean))
  (bind _w_trades (Variables|UI|GetW_Trades))
  (if (< (+ (Variables|/Game/Rogue/Blueprints/Core/TradingSystem/W_Trades.W_Trades_C|GetNumOfBuy _w_trades) (Variables|/Game/Rogue/Blueprints/Core/TradingSystem/W_Trades.W_Trades_C|GetNumOfSell _w_trades)) (* (Variables|Default|GetMaxNumOfCertaintTrades) 2))
    (bind _notsold (Shop|ArrayIntersectionSell (Variables|/Game/Rogue/Blueprints/Core/TradingSystem/W_Trades.W_Trades_C|GetBuyingTrades (Variables|UI|GetW_Trades)) (Variables|Default|GetAllBuyItems)))
    (if (and (< (Variables|/Game/Rogue/Blueprints/Core/TradingSystem/W_Trades.W_Trades_C|GetNumOfBuy (Variables|UI|GetW_Trades)) (Variables|Default|GetMaxNumOfCertaintTrades)) (!= (Utilities|Array|Length _notsold) 0))
      (return true _notsold)
      (else
        (return false 0)))
    (else
      (return false 0))))

(fn PlayMusic
  (params (Music :type Sound%20Base%20Object%20Reference) (VolumeMultiplier :type Float%20%28single-precision%29))
  (bind _returnvalue (Audio|SpawnSound2D Music VolumeMultiplier 1.0 0.0 0))
  (Variables|Default|SetShopMusic _returnvalue))

(fn StopMusic
  (Audio|Components|Audio|FadeOut (Variables|Default|GetShopMusic) 2.0 0.0 "Linear" :!class /Script/Engine.AudioComponent))

(fn GetPlayerInventoryRef
  (return (Variables|Default|GetPlayer%20Inventory)))