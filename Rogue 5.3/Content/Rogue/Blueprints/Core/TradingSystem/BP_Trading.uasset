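; BP_Trading is the trading logic for the game, handling sell lists, item pricing and the content available from the player's save.
; On BeginPlay it caches the player inventory and loads the save slot, creating a fresh save if none exists.
; Buy and sell prices scale DT_Item base prices by random coefficient ranges.
; Getters return saved unlocked items and companions, plus DT_Talents entries within the saved upgrade tier plus two.
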(event EventBeginPlay
  (Utilities|FlowControl|Sequence
    (:then_0
      (bind _returnvalue (Actor|GetActorOfClass "/Game/Rogue/Blueprints/Core/Player/BP_PlayerInventoryHolder.BP_PlayerInventoryHolder_C"))
      (bind _playerinventory (Default|GetPlayerInventoryRef _returnvalue))
      (Variables|Default|SetPlayer%20Inventory _playerinventory))
    (:then_1
      (bind _returnvalue_2 (SaveGame|DoesSaveGameExist "save1"))
      (if _returnvalue_2
        (bind _returnvalue_3 (SaveGame|LoadGamefromSlot "save1"))
        (bind _asbp_save (Utilities|Casting|CastToBP_Save _returnvalue_3))
        (Variables|Default|SetBP%20Save _asbp_save)
        (else
          (bind _returnvalue_4 (SaveGame|CreateSaveGameObject "/Game/Rogue/Blueprints/SaveLoad/BP_Save.BP_Save_C"))
          (Variables|/Game/Rogue/Blueprints/SaveLoad/BP_Save.BP_Save_C|SetScore _returnvalue_4 (Utilities|Struct|MakeIntPoint 0 0))
          (Variables|/Game/Rogue/Blueprints/SaveLoad/BP_Save.BP_Save_C|SetPlayerExp _returnvalue_4 0)
          (SaveGame|SaveGametoSlot _returnvalue_4 "save1")
          (Variables|Default|SetBP%20Save _returnvalue_4))))))

(fn ConstructionScript)

(fn ClearSell
  (Utilities|Array|Clear (Variables|Default|GetForSellItems)))

(fn AddSellItem
  (params (NewItem :type S%20Slot%20Structure%20%28by%20ref%29))
  (Utilities|Array|Add (Variables|Default|GetForSellItems) NewItem))

(fn RemoveSellItem
  (params (RemoveItem :type S%20Slot%20Structure%20%28by%20ref%29))
  (bind _forsellitems (Variables|Default|GetForSellItems))
  (bind _returnvalue (Utilities|Array|FindItem _forsellitems RemoveItem))
  (if (== _returnvalue -1)
    (return false)
    (else
      (Utilities|Array|RemoveIndex (Variables|Default|GetForSellItems) _returnvalue)
      (return true))))

(fn GenerateSellPrice
  (params (Item :type S%20Slot%20Structure))
  (bind (_item _found_) (Additional|GetDatafromSlot Item))
  (if _found_
    (return (Math|Float|Round (* (.Price (Utilities|Struct|BreakS_Item _item)) (Math|Random|RandomFloatinRange (Variables|Default|GetSellMinCoef) (Variables|Default|GetSellMaxCoef)))) true)
    (else
      (return 0 false))))

(fn GetDatafromSlot
  (params (Slot :type S%20Slot%20Structure))
  (bind _returnvalue (Utilities|GetDataTableRow "/Game/Inventory/DT_Item.DT_Item" (.ItemID (Utilities|Struct|BreakS_Slot Slot)))
    (:then
      (return _returnvalue true))
    (:RowNotFound
      (return "" false))))

(fn GenerateBuyPrice
  (params (Item :type S%20Slot%20Structure))
  (bind (_item _found_) (Additional|GetDatafromSlot Item))
  (if _found_
    (return (Math|Float|Round (* (.Price (Utilities|Struct|BreakS_Item _item)) (Math|Random|RandomFloatinRange (Variables|Default|GetBuyMinCoef) (Variables|Default|GetBuyMaxCoef)))) true)
    (else
      (return 0 false))))

(fn GetAvailableItemsSorted
  (return (Variables|/Game/Rogue/Blueprints/SaveLoad/BP_Save.BP_Save_C|GetItemsUnlocked (Variables|Default|GetBP%20Save))))

(fn GetAvailableTalents
  (bind _outrownames (DataTable|GetDataTableRowNames "/Game/Rogue/Blueprints/Core/TalentSystem/DT_Talents.DT_Talents"))
  (for _array_element _outrownames
    (bind _returnvalue (Utilities|GetDataTableRow "/Game/Rogue/Blueprints/Core/TalentSystem/DT_Talents.DT_Talents" _array_element)
      (:then
        (if (<= (.TalentTier (Utilities|Struct|BreakS_TalentInfo _returnvalue)) (+ (Variables|/Game/Rogue/Blueprints/SaveLoad/BP_Save.BP_Save_C|GetTierUpgrades (Variables|Default|GetBP%20Save)) 2))
          (Utilities|Array|Add (LocalVariables|GetTalentsArray) (.Talent (Utilities|Struct|BreakS_TalentInfo _returnvalue)))))))
  (return (LocalVariables|GetTalentsArray)))

(fn GetAvailableCompanionsSorted
  (return (Variables|/Game/Rogue/Blueprints/SaveLoad/BP_Save.BP_Save_C|GetCompanions (Variables|Default|GetBP%20Save))))

(fn ItemNametoNameFunc
  (params (ItemName :type E_ItemName%20Enum :default "NewEnumerator14"))
  (return (Utilities|String|StringToName (Utilities|String|Replace (Utilities|String|EnumtoString ItemName) " "))))