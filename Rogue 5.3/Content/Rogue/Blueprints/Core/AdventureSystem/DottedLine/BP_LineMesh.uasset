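; Adventure system actor that draws a dotted line of spline meshes between two actors, Point1 and Point2.
; ConstructNow clears old segments, then spawns a distance-based count of straight spline mesh dashes spaced by SizeCoef.
; The parent spline moves to Point1 and rotates toward Point2, so segments lay out along local X.
; Early dashes get slight random yaw, and short lines randomize the last dash's length.
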(event Custom|ConstructNow
  (bind _components (Variables|Default|GetComponents))
  (bind _point1 (Variables|Default|GetPoint1))
  (bind _yzscale (Variables|Default|GetYZScale))
  (bind _point2 (Variables|Default|GetPoint2))
  (bind _spline (Variables|Default|GetSpline))
  (bind _returnvalue (Transformation|GetActorLocation _point1))
  (bind _returnvalue_2 (Transformation|GetActorLocation _point2))
  (bind _returnvalue_3 (- _returnvalue_2 _returnvalue))
  (Utilities|FlowControl|Sequence
    (:then_0
      (for _array_element _components
        (Components|DestroyComponent _array_element))
      (Utilities|Array|Clear _components))
    (:then_1
      (Variables|Default|SetP1 (Transformation|GetActorLocation (Variables|Default|GetPoint1)))
      (Variables|Default|SetP2 (Transformation|GetActorLocation (Variables|Default|GetPoint2)))
      (Variables|Default|SetBetweetPointLen (Math|Vector|VectorLength _returnvalue_3))
      (Variables|Default|SetBetweenPointRot (Math|Conversions|RotationFromXVector _returnvalue_3))
      (Utilities|FlowControl|Sequence
        (:then_0
          (if (Variables|Default|GetAllow%20Scaling)
            (Variables|Default|SetSectionLength (* (.x (Transformation|GetActorScale3D)) 1e+02)))
          (if (Variables|Default|GetMustBeFullLenMeshes)
            (bind _output_get (Variables|Default|SetMaxIndex (- (Math|Float|Truncate (/ (Variables|Default|GetBetweetPointLen) (* (Variables|Default|GetSectionLength) (+ (Variables|Default|GetSizeCoef) (Math|Float|Lerp 0.22 0.12 (/ (Variables|Default|GetBetweetPointLen) 2e+03)))))) 1)))
            (for _index (range 0 _output_get)
              (Variables|Default|SetLoopIndex _index)
              (bind _returnvalue_4 (AddComponent|AddSplineMeshComponent false))
              (Utilities|Array|Add (Variables|Default|GetComponents) _returnvalue_4)
              (Transformation|AttachComponentToComponent _returnvalue_4 (Variables|Default|GetSpline) "None" "KeepRelative" "KeepRelative" "KeepRelative" true)
              (Components|StaticMesh|SetStaticMesh _returnvalue_4 (Variables|Default|GetSpline%20Mesh))
              (SplineMesh|SetForwardAxis _returnvalue_4 "X" true)
              (Variables|Default|SetOneCut (Math|Vector|MakeVector (Variables|Default|GetSectionLength) 0.0 0.0))
              (bind _tang (CallFunction|GetStartPosTang (Variables|Default|GetLoopIndex)))
              (bind _tang_2 (CallFunction|GetEndPosTang (Variables|Default|GetLoopIndex)))
              (SplineMesh|SetStartandEnd _returnvalue_4 (* (Variables|Default|GetOneCut) (Math|Float|Max(Float) (* (Variables|Default|GetLoopIndex) (Variables|Default|GetSizeCoef)) 0.5)) _tang (* (Variables|Default|GetOneCut) (Math|Float|SelectFloat (+ (* (Variables|Default|GetLoopIndex) (Variables|Default|GetSizeCoef)) (Math|Random|RandomFloatinRange 0.5 0.8)) (+ (* (Variables|Default|GetLoopIndex) (Variables|Default|GetSizeCoef)) 1.0) (and (== (Variables|Default|GetLoopIndex) (Variables|Default|GetMaxIndex)) (< (Variables|Default|GetMaxIndex) 2)))) _tang_2 true :!class /Script/Engine.SplineMeshComponent)
              (Collision|SetCollisionEnabled _returnvalue_4 (Variables|Default|GetCollisionType))
              (if (< (Variables|Default|GetLoopIndex) 6)
                (bind _output_get_2 (Variables|Default|SetLastRot (Math|Rotator|MakeRotator 0.0 0.0 (Math|Float|Clamp(Float) (+ (.Roll (Math|Rotator|BreakRotator (Variables|Default|GetLastRot))) (Math|Random|RandomFloatinRange -2.0 2.0)) -5.0 5.0))))
                (Transformation|SetRelativeRotation _returnvalue_4 _output_get_2 false false)))
            (else
              (bind _output_get_3 (Variables|Default|SetMaxIndex (Math|Float|Truncate (/ (Variables|Default|GetBetweetPointLen) (* (Variables|Default|GetSectionLength) (+ (Variables|Default|GetSizeCoef) (Math|Float|Lerp 0.22 0.12 (/ (Variables|Default|GetBetweetPointLen) 2e+03))))))))
              (for _index_2 (range 0 _output_get_3)
                (Variables|Default|SetLoopIndex _index_2)
                (bind _returnvalue_5 (AddComponent|AddSplineMeshComponent false))
                (Utilities|Array|Add (Variables|Default|GetComponents) _returnvalue_5)
                (Transformation|AttachComponentToComponent _returnvalue_5 (Variables|Default|GetSpline) "None" "KeepRelative" "KeepRelative" "KeepRelative" true)
                (Components|StaticMesh|SetStaticMesh _returnvalue_5 (Variables|Default|GetSpline%20Mesh))
                (SplineMesh|SetForwardAxis _returnvalue_5 "X" true)
                (Variables|Default|SetOneCut (Math|Vector|MakeVector (Variables|Default|GetSectionLength) 0.0 0.0))
                (bind _tang_3 (CallFunction|GetStartPosTang (Variables|Default|GetLoopIndex)))
                (bind _tang_4 (CallFunction|GetEndPosTang (Variables|Default|GetLoopIndex)))
                (SplineMesh|SetStartandEnd _returnvalue_5 (* (Variables|Default|GetOneCut) (Math|Float|Max(Float) (* (Variables|Default|GetLoopIndex) (Variables|Default|GetSizeCoef)) 0.5)) _tang_3 (* (Variables|Default|GetOneCut) (Math|Float|SelectFloat (+ (* (Variables|Default|GetLoopIndex) (Variables|Default|GetSizeCoef)) (Math|Random|RandomFloatinRange 0.5 0.8)) (+ (* (Variables|Default|GetLoopIndex) (Variables|Default|GetSizeCoef)) 1.0) (and (== (Variables|Default|GetLoopIndex) (Variables|Default|GetMaxIndex)) (< (Variables|Default|GetMaxIndex) 2)))) _tang_4 true :!class /Script/Engine.SplineMeshComponent)
                (Collision|SetCollisionEnabled _returnvalue_5 (Variables|Default|GetCollisionType))
                (if (< (Variables|Default|GetLoopIndex) 6)
                  (bind _output_get_4 (Variables|Default|SetLastRot (Math|Rotator|MakeRotator 0.0 0.0 (Math|Float|Clamp(Float) (+ (.Roll (Math|Rotator|BreakRotator (Variables|Default|GetLastRot))) (Math|Random|RandomFloatinRange -2.0 2.0)) -5.0 5.0))))
                  (Transformation|SetRelativeRotation _returnvalue_5 _output_get_4 false false))))))
        (:then_1
          (Transformation|SetWorldLocation _spline _returnvalue false false)
          (Transformation|SetWorldRotation _spline (Variables|Default|GetBetweenPointRot) false false)
          (Transformation|SetRelativeScale3D _spline (Math|Vector|MakeVector 1.0 _yzscale _yzscale)))))))

(fn ConstructionScript)

(fn GetStartPosTang
  (params (Index :type Integer))
  (bind _spline (Variables|Default|GetSpline))
  (bind _sectionlength (Variables|Default|GetSectionLength))
  (return (Spline|GetLocationatDistanceAlongSpline _spline (* (Math|Float|SelectFloat (/ (- (* Index 2) 1) 2) (Math|Conversions|ToFloat(Integer) Index) (== (Math|Integer|%(Integer) Index 2) 1)) _sectionlength) "Local") (Math|Vector|ClampVectorSize (Spline|GetTangentatDistanceAlongSpline _spline (* Index _sectionlength) "Local") 0.0 2.0)))

(fn GetEndPosTang
  (params (Index :type Integer))
  (bind _returnvalue (+ Index 1))
  (bind _spline (Variables|Default|GetSpline))
  (bind _sectionlength (Variables|Default|GetSectionLength))
  (return (Spline|GetLocationatDistanceAlongSpline _spline (* _returnvalue _sectionlength) "Local") (Math|Vector|ClampVectorSize (Spline|GetTangentatDistanceAlongSpline _spline (* _returnvalue _sectionlength) "Local") 0.0 2.0)))