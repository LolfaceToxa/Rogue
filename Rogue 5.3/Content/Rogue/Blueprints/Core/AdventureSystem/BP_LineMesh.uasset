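; BP_LineMesh is an adventure-system actor that draws a straight line between two referenced actors, Point1 and Point2, using a stretched mesh.
; It places LineMesh at their midpoint, aims its X axis along the connecting vector and scales its length to the distance with a fixed thin cross-section.
; The same logic is duplicated in the construction script and a Construct event, with no per-tick update.
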(event Custom|Construct
  (bind _point1 (Variables|Default|GetPoint1))
  (bind _point2 (Variables|Default|GetPoint2))
  (bind _linemesh (Variables|Default|GetLineMesh))
  (bind _returnvalue (Transformation|GetActorLocation _point2))
  (bind _returnvalue_2 (Transformation|GetActorLocation _point1))
  (bind _returnvalue_3 (- _returnvalue _returnvalue_2))
  (Transformation|SetWorldLocation _linemesh (/ (+ _returnvalue_2 _returnvalue) 2.0) false false)
  (Transformation|SetWorldRotation _linemesh (Math|Conversions|RotationFromXVector _returnvalue_3) false false)
  (Transformation|SetRelativeScale3D _linemesh (Math|Vector|MakeVector (/ (Math|Vector|VectorLength _returnvalue_3) 1e+02) 0.1 0.1)))

(event EventBeginPlay)

(fn ConstructionScript
  (bind _point1 (Variables|Default|GetPoint1))
  (bind _point2 (Variables|Default|GetPoint2))
  (bind _linemesh (Variables|Default|GetLineMesh))
  (bind _returnvalue (Transformation|GetActorLocation _point2))
  (bind _returnvalue_2 (Transformation|GetActorLocation _point1))
  (bind _returnvalue_3 (- _returnvalue _returnvalue_2))
  (Transformation|SetWorldLocation _linemesh (/ (+ _returnvalue_2 _returnvalue) 2.0) false false)
  (Transformation|SetWorldRotation _linemesh (Math|Conversions|RotationFromXVector _returnvalue_3) false false)
  (Transformation|SetRelativeScale3D _linemesh (Math|Vector|MakeVector (/ (Math|Vector|VectorLength _returnvalue_3) 1e+02) 0.1 0.1)))