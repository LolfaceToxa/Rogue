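; Combat level start logic that sets up a roguelike fight behind a loading screen.
; It spawns player units from the save or as a fresh pair, then derives a difficulty budget from score, bonus and unit hardness.
; Random enemies consume part of that budget, and random talents and items fill the rest, though the slot check always blocks item placement.
; It also adds the key-helper HUD and a navmesh-placed acid obstacle.
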(event Custom|StartLogic
  (bind _returnvalue (UserInterface|CreateWidget "/Game/Rogue/Blueprints/Other/Menu/W_LoadingScreen.W_LoadingScreen_C"))
  (bind _output_get (Variables|Default|SetLoadingScreen _returnvalue))
  (UserInterface|Viewport|AddtoViewport _output_get 0)
  (Input|DisableInput (Game|GetPlayerController 0))
  (Utilities|FlowControl|Sequence
    (:then_0
      (bind _outactors (Actor|GetAllActorsOfClass "/Game/Rogue/Blueprints/Core/Player/BP_CombatPlayerActions.BP_CombatPlayerActions_C"))
      (Variables|Default|SetPlayerActions (Utilities|Array|Get(acopy) _outactors))
      (bind _outrownames (DataTable|GetDataTableRowNames "/Game/Rogue/Blueprints/Core/TalentSystem/DT_Talents.DT_Talents"))
      (Variables|Default|SetTalents _outrownames)
      (bind _outrownames_2 (DataTable|GetDataTableRowNames "/Game/Inventory/DT_Item.DT_Item"))
      (Variables|Default|SetItems _outrownames_2)
      (Variables|Default|SetDifficulty (* (Math|Integer|SelectInt (- (+ (Utilities|Struct|BreakIntPoint (Variables|/Game/Rogue/Blueprints/SaveLoad/BP_Save.BP_Save_C|GetScore (Variables|/Game/Rogue/Blueprints/Core/Player/BP_CombatPlayerActions.BP_CombatPlayerActions_C|GetBP%20Save (Variables|Default|GetPlayerActions)))) 6 (Math|Integer|%(Integer) (Utilities|Struct|BreakIntPoint (Variables|/Game/Rogue/Blueprints/SaveLoad/BP_Save.BP_Save_C|GetScore (Variables|/Game/Rogue/Blueprints/Core/Player/BP_CombatPlayerActions.BP_CombatPlayerActions_C|GetBP%20Save (Variables|Default|GetPlayerActions)))) 2)) 1) (+ (Utilities|Struct|BreakIntPoint (Variables|/Game/Rogue/Blueprints/SaveLoad/BP_Save.BP_Save_C|GetScore (Variables|/Game/Rogue/Blueprints/Core/Player/BP_CombatPlayerActions.BP_CombatPlayerActions_C|GetBP%20Save (Variables|Default|GetPlayerActions)))) 6 (Math|Integer|%(Integer) (Utilities|Struct|BreakIntPoint (Variables|/Game/Rogue/Blueprints/SaveLoad/BP_Save.BP_Save_C|GetScore (Variables|/Game/Rogue/Blueprints/Core/Player/BP_CombatPlayerActions.BP_CombatPlayerActions_C|GetBP%20Save (Variables|Default|GetPlayerActions)))) 2)) (Utilities|Enum|Equal(Enum) (Variables|/Game/Rogue/Blueprints/SaveLoad/BP_Save.BP_Save_C|GetSelectedBonus (Variables|/Game/Rogue/Blueprints/Core/Player/BP_CombatPlayerActions.BP_CombatPlayerActions_C|GetBP%20Save (Variables|Default|GetPlayerActions))) "NewEnumerator4")) 2))
      (Variables|Default|SetRandomEnemyTalentsArray (Utilities|Array|MakeArray))
      (Variables|Default|SetEnemyUnits (Utilities|Array|MakeArray)))
    (:then_1
      (if (or (== (Utilities|Array|Length (Variables|/Game/Rogue/Blueprints/SaveLoad/BP_Save.BP_Save_C|GetPlayerUnits (Variables|/Game/Rogue/Blueprints/Core/Player/BP_CombatPlayerActions.BP_CombatPlayerActions_C|GetBP%20Save (Variables|Default|GetPlayerActions)))) 0) (Variables|/Game/Rogue/Blueprints/SaveLoad/BP_Save.BP_Save_C|GetStartFromZero? (Variables|/Game/Rogue/Blueprints/Core/Player/BP_CombatPlayerActions.BP_CombatPlayerActions_C|GetBP%20Save (Variables|Default|GetPlayerActions))))
        (Variables|/Game/Rogue/Blueprints/SaveLoad/BP_Save.BP_Save_C|SetStartFromZero? (Variables|/Game/Rogue/Blueprints/Core/Player/BP_CombatPlayerActions.BP_CombatPlayerActions_C|GetBP%20Save (Variables|Default|GetPlayerActions)) false)
        (Utilities|SaveGame)
        (Default|SaveValuesAfterLose (Variables|Default|GetPlayerActions))
        (CallFunction|SpawnAllyUnitsfromZero)
        (else
          (for (_array_element _array_index) (Variables|/Game/Rogue/Blueprints/SaveLoad/BP_Save.BP_Save_C|GetPlayerUnits (Variables|/Game/Rogue/Blueprints/Core/Player/BP_CombatPlayerActions.BP_CombatPlayerActions_C|GetBP%20Save (Variables|Default|GetPlayerActions)))
            (bind _returnvalue_2 (Game|SpawnActorfromClass "/Game/Rogue/Blueprints/Core/Units/BP_Unit.BP_Unit_C" (Math|Transform|MakeTransform (+ (Transformation|GetActorLocation (Variables|Default|GetPlayerActions)) "0.000000,600.000000,0.000000") "0.000000,-90.000000,0.000000") "Undefined" "MultiplyWithRoot" 0 (.UnitType (Utilities|Struct|BreakS_UnitSaveLoad _array_element)) true 0 0))
            (Variables|/Game/Rogue/Blueprints/Core/Units/BP_Unit.BP_Unit_C|SetCurrentEquipmentItems _returnvalue_2 (.InvContent (Utilities|Struct|BreakS_UnitSaveLoad _array_element)))
            (Variables|/Game/Rogue/Blueprints/Core/Units/BP_Unit.BP_Unit_C|SetAllyIndex _returnvalue_2 _array_index)
            (Default|SetTeamIndex _returnvalue_2)
            (Variables|/Game/Rogue/Blueprints/Core/Units/BP_Unit.BP_Unit_C|SetUpdTalents _returnvalue_2 (.TalentAmount (Utilities|Struct|BreakS_UnitSaveLoad _array_element)))
            (Utilities|Array|Add (Variables|/Game/Rogue/Blueprints/Core/Player/BP_CombatPlayerActions.BP_CombatPlayerActions_C|GetPlayerUnits (Variables|Default|GetPlayerActions)) _returnvalue_2)
            (Variables|/Game/Rogue/Blueprints/Core/Units/BP_Unit.BP_Unit_C|SetTalents _returnvalue_2 (.SaveLoadTalents (Utilities|Struct|BreakS_UnitSaveLoad _array_element)))
            (Default|RefreshAllStats _returnvalue_2 false)))))
    (:then_2
      (CallFunction|GenerateFightOfNeededDifficulty))
    (:then_3
      (bind _returnvalue_3 (Game|ConstructObjectfromClass "/Game/Inventory/UI/WB_KeyHelpersPlayerHUD.WB_KeyHelpersPlayerHUD_C"))
      (bind _output_get_2 (Variables|Default|SetKeyHelpers _returnvalue_3))
      (bind _output_get_3 (Variables|/Game/Rogue/Blueprints/Core/Player/BP_CombatPlayerActions.BP_CombatPlayerActions_C|SetPlayerKeyHelpers (Variables|Default|GetPlayerActions) _output_get_2))
      (UserInterface|Viewport|AddtoViewport _output_get_3 0))
    (:then_4
      (CallFunction|SpawnObstacles))
    (:then_5
      (Widget|RemovefromParent (Variables|Default|GetLoadingScreen))
      (Input|EnableInput (Game|GetPlayerController 0)))))

(event Custom|Spawn%20Ally%20Units%20From%20Zero
  (bind _array (Utilities|Array|MakeArray "NewEnumerator2"))
  (bind _array_2 (Utilities|Array|MakeArray "NewEnumerator1"))
  (bind _playeractions (Variables|Default|GetPlayerActions))
  (bind _playeractions_2 (Variables|Default|GetPlayerActions))
  (bind _playeractions_3 (Variables|Default|GetPlayerActions))
  (bind _returnvalue (Transformation|GetActorLocation _playeractions))
  (bind _bp_save (Variables|/Game/Rogue/Blueprints/Core/Player/BP_CombatPlayerActions.BP_CombatPlayerActions_C|GetBP%20Save _playeractions_2))
  (bind _bp_save_2 (Variables|/Game/Rogue/Blueprints/Core/Player/BP_CombatPlayerActions.BP_CombatPlayerActions_C|GetBP%20Save _playeractions_3))
  (bind _returnvalue_2 (- _returnvalue "0.000000,600.000000,0.000000"))
  (bind _secondunittype (Variables|/Game/Rogue/Blueprints/SaveLoad/BP_Save.BP_Save_C|GetSecondUnitType _bp_save))
  (bind _selectedbonus (Variables|/Game/Rogue/Blueprints/SaveLoad/BP_Save.BP_Save_C|GetSelectedBonus _bp_save_2))
  (bind _returnvalue_3 (Math|Transform|MakeTransform _returnvalue_2 "0.000000,-90.000000,0.000000"))
  (bind _returnvalue_4 (Utilities|Select :Index _selectedbonus :NewEnumerator0 "NewEnumerator0" :NewEnumerator1 _array_2 :NewEnumerator2 _array :NewEnumerator3 "NewEnumerator0" :NewEnumerator4 "NewEnumerator0"))
  (bind _returnvalue_5 (Game|SpawnActorfromClass "/Game/Rogue/Blueprints/Core/Units/BP_Unit.BP_Unit_C" _returnvalue_3 "Undefined" "MultiplyWithRoot" 0 "NewEnumerator13" true 0 0))
  (Variables|Default|SetPlayerUnit _returnvalue_5)
  (bind _returnvalue_6 (Game|SpawnActorfromClass "/Game/Rogue/Blueprints/Core/Units/BP_Unit.BP_Unit_C" _returnvalue_3 "Undefined" "MultiplyWithRoot" 0 _secondunittype true 0 0))
  (Default|SetTeamIndex (Variables|Default|GetPlayerUnit))
  (Variables|/Game/Rogue/Blueprints/Core/Player/BP_CombatPlayerActions.BP_CombatPlayerActions_C|SetPlayerUnits (Variables|Default|GetPlayerActions) (Utilities|Array|MakeArray (Variables|Default|GetPlayerUnit) _returnvalue_6))
  (Variables|/Game/Rogue/Blueprints/Core/Units/BP_Unit.BP_Unit_C|SetAllyIndex (Variables|Default|GetPlayerUnit) 0)
  (Variables|/Game/Rogue/Blueprints/Core/Units/BP_Unit.BP_Unit_C|SetAllyIndex _returnvalue_6 1)
  (Variables|/Game/Rogue/Blueprints/Core/Player/BP_CombatPlayerActions.BP_CombatPlayerActions_C|SetPlayerUnitsData (Variables|Default|GetPlayerActions) (Utilities|Array|MakeArray (Utilities|Struct|MakeS_UnitSaveLoad "NewEnumerator13" _returnvalue_4 0 0 "(ValidTileTypes_6_BB0A15FF4D4F153DEDA3F6AB8F56389A=(NewEnumerator1,NewEnumerator3,NewEnumerator4),MP_Current_19_C77B1359466788C328B8BCA9009F06D6=3,MP_Max_22_9EFF56BE46C441C6BFE4719AAD37C023=3,AvailableSpellsList_14_4A30C352451254E1F66A91ADD5944A43=(NewEnumerator2),HP_Current_16_9FE28CD043CC35C593D3DD84099FA4CC=50,HP_Max_18_362D735046FB450EC32405BBDED3F5DC=50,AP_Current_25_C71C52324B5E6916CE43F98C86D77C49=6,AP_Max_27_15170DA145CB5B8F21145786F9FD3798=6,MissChance_30_DE64097445776FF35AFB058DC497B0CD=0.000000,HitVampiric_33_00B1CDFF49592382C128DBAD12DB88A7=0,KillVampiric_35_D2973179483632FC32D13BB501B64739=0,BaseDMG_42_10F143664A69C9CA9BB6AFA62B772857=0,MinDMG_43_627F3B18434F6F747DC41DB7BA0E65BF=0,MaxDMG_45_DAC57158472B841741F5FB8322FBEED9=0,BaseDMGBlock_90_CFE1C9FA4CC7B7F07F3B10AC752FBADE=0,MaxDMGBlock_91_FC1E03374A1B261B3B3FFA910EC481ED=0,MinDMGBlock_92_FE94357F45AD4E32BBC34D9349C2C40E=0,Evasion_95_4C01ED7E4E7389F064ED9DBF890AE6B2=0.000000,CanMoveDiagonally_5_4DEFA6294B6F1AC54C042EA89121B452=False,IgnoreObstacles_48_7706332D46ABC9010EA04A87F27FED77=False,IgnoreLoweredSpeed_50_A6908A444C497B8FFB6C198AD3790E3B=False,HitMP_DMG_59_E82D283A4C987667EAEC12904865B5FA=0,HitAP_DMG_60_B2B688F74FCE5AFEB183F3805E1051DD=0,SpellRange_61_D86CBEAA40F76002C2F5F38CABF57549=0,SpellRangeAOE_65_1494B18C409C1C148306CFB010824920=0,HitHP_SelfDMG_68_5DEB32C1445F7027856A609F11527F7C=0,Accuracy_75_B3774CDC4461D5D86E4F498437AAF88B=0.000000,CD_Reduction_101_E37B6240426DBEF34A19EFB8606B4462=0,ActiveSetBonuses_72_9ECE72C14EEE1CBCA232BEBBC9B5D78B=,CritChance_105_786635594517164712AF15A3868C5CA9=0.000000,CritMod_107_69343E284BFB9ACAD7DAC3814A255A93=0.000000,Hardness_78_AD8AEEA947100AFAF34279BDB64E7918=0,Intelligence_110_D5D4E7A448E14FE7F26F7B9064913A79=0)") (Utilities|Struct|MakeS_UnitSaveLoad _secondunittype "NewEnumerator0" 0 0 "(ValidTileTypes_6_BB0A15FF4D4F153DEDA3F6AB8F56389A=(NewEnumerator1,NewEnumerator3,NewEnumerator4),MP_Current_19_C77B1359466788C328B8BCA9009F06D6=3,MP_Max_22_9EFF56BE46C441C6BFE4719AAD37C023=3,AvailableSpellsList_14_4A30C352451254E1F66A91ADD5944A43=(NewEnumerator2),HP_Current_16_9FE28CD043CC35C593D3DD84099FA4CC=50,HP_Max_18_362D735046FB450EC32405BBDED3F5DC=50,AP_Current_25_C71C52324B5E6916CE43F98C86D77C49=6,AP_Max_27_15170DA145CB5B8F21145786F9FD3798=6,MissChance_30_DE64097445776FF35AFB058DC497B0CD=0.000000,HitVampiric_33_00B1CDFF49592382C128DBAD12DB88A7=0,KillVampiric_35_D2973179483632FC32D13BB501B64739=0,BaseDMG_42_10F143664A69C9CA9BB6AFA62B772857=0,MinDMG_43_627F3B18434F6F747DC41DB7BA0E65BF=0,MaxDMG_45_DAC57158472B841741F5FB8322FBEED9=0,BaseDMGBlock_90_CFE1C9FA4CC7B7F07F3B10AC752FBADE=0,MaxDMGBlock_91_FC1E03374A1B261B3B3FFA910EC481ED=0,MinDMGBlock_92_FE94357F45AD4E32BBC34D9349C2C40E=0,Evasion_95_4C01ED7E4E7389F064ED9DBF890AE6B2=0.000000,CanMoveDiagonally_5_4DEFA6294B6F1AC54C042EA89121B452=False,IgnoreObstacles_48_7706332D46ABC9010EA04A87F27FED77=False,IgnoreLoweredSpeed_50_A6908A444C497B8FFB6C198AD3790E3B=False,HitMP_DMG_59_E82D283A4C987667EAEC12904865B5FA=0,HitAP_DMG_60_B2B688F74FCE5AFEB183F3805E1051DD=0,SpellRange_61_D86CBEAA40F76002C2F5F38CABF57549=0,SpellRangeAOE_65_1494B18C409C1C148306CFB010824920=0,HitHP_SelfDMG_68_5DEB32C1445F7027856A609F11527F7C=0,Accuracy_75_B3774CDC4461D5D86E4F498437AAF88B=0.000000,CD_Reduction_101_E37B6240426DBEF34A19EFB8606B4462=0,ActiveSetBonuses_72_9ECE72C14EEE1CBCA232BEBBC9B5D78B=,CritChance_105_786635594517164712AF15A3868C5CA9=0.000000,CritMod_107_69343E284BFB9ACAD7DAC3814A255A93=0.000000,Hardness_78_AD8AEEA947100AFAF34279BDB64E7918=0,Intelligence_110_D5D4E7A448E14FE7F26F7B9064913A79=0)")))
  (Variables|/Game/Rogue/Blueprints/Core/Units/BP_Unit.BP_Unit_C|SetTalents (Variables|Default|GetPlayerUnit) _returnvalue_4)
  (Default|RefreshAllStats (Variables|Default|GetPlayerUnit) false)
  (bind _playerinventory (Default|GetPlayerInventoryRef (Variables|Default|GetPlayerActions)))
  (Variables|Default|SetPlayer%20Inventory _playerinventory))

(fn ConstructionScript)

(fn MapAdd
  (params (TargetMap :type Map%20of%20E_Units%20Enums%20to%20Integers :default "NewEnumerator13") (Key :type E_Units%20Enum%20%28by%20ref%29 :default "NewEnumerator13"))
  (bind (_value _returnvalue) (Utilities|Map|Find TargetMap Key))
  (if _returnvalue
    (Utilities|Map|Add TargetMap Key (+ _value 1))
    (else
      (Utilities|Map|Add TargetMap Key 1))))

(fn RandomizeEnemies
  (LocalVariables|SetNeededDiffuculty (Math|Integer|Clamp(Integer) (Math|Float|Round (/ (Variables|Default|GetDifficulty) (Math|Float|Clamp(Float) (+ 1.5 (/ (/ (Utilities|Struct|BreakIntPoint (Variables|/Game/Rogue/Blueprints/SaveLoad/BP_Save.BP_Save_C|GetScore (Variables|/Game/Rogue/Blueprints/Core/Player/BP_CombatPlayerActions.BP_CombatPlayerActions_C|GetBP%20Save (Variables|Default|GetPlayerActions)))) 10) -1e+01)) 0.7 1.5))) 10 999))
  (bind _outrownames (DataTable|GetDataTableRowNames "/Game/Rogue/Blueprints/Core/Units/Utilities/DT_Default_UnitDataPerType.DT_Default_UnitDataPerType"))
  (LocalVariables|SetLength (Utilities|Array|Length _outrownames))
  (for _array_element _outrownames
    (bind _returnvalue (Utilities|GetDataTableRow "/Game/Rogue/Blueprints/Core/Units/Utilities/DT_Default_UnitDataPerType.DT_Default_UnitDataPerType" _array_element)
      (:then
        (Utilities|Array|Add (LocalVariables|GetUnitTypes) (.UnitName (Utilities|Struct|BreakS_UnitDataF _returnvalue)))
        (Utilities|Array|Add (LocalVariables|GetUnitDiffuculties) (.Difficulty (Utilities|Struct|BreakS_UnitDataF _returnvalue))))))
  (while (not (and (> (Utilities|Map|Length (LocalVariables|GetRet)) 0) (< (- (LocalVariables|GetNeededDiffuculty) (LocalVariables|GetSumDifficulty)) 5)))
    (LocalVariables|SetRandomNumber (Math|Random|RandomInteger (- (LocalVariables|GetLength) 1)))
    (LocalVariables|SetNextUnitType (Utilities|Array|Get(acopy) (LocalVariables|GetUnitTypes) (LocalVariables|GetRandomNumber)))
    (LocalVariables|SetNextUnitDiff (Utilities|Array|Get(acopy) (LocalVariables|GetUnitDiffuculties) (LocalVariables|GetRandomNumber)))
    (if (<= (LocalVariables|GetNextUnitDiff) (LocalVariables|GetNeededDiffuculty))
      (if (<= (+ (LocalVariables|GetSumDifficulty) (LocalVariables|GetNextUnitDiff)) (LocalVariables|GetNeededDiffuculty))
        (LocalVariables|SetSumDifficulty (+ (LocalVariables|GetSumDifficulty) (LocalVariables|GetNextUnitDiff)))
        (CallFunction|MapAdd (LocalVariables|GetRet) (LocalVariables|GetNextUnitType)))))
  (Variables|Default|SetCurrentDifficulty (LocalVariables|GetSumDifficulty))
  (return (LocalVariables|GetRet)))

(fn RandomizeTalentsandItems
  (params (DiffLeft :type Integer))
  (bind _itemsarrayequip (Variables|Default|GetItemsArrayEquip))
  (if (!= DiffLeft 0)
    (if (Math|Random|RandomBool)
      (LocalVariables|SetLen (Utilities|Array|Length (Variables|Default|GetTalents)))
      (while (< (LocalVariables|GetIteration) 10)
        (bind _output_get (LocalVariables|SetRandomNumber (Math|Random|RandomInteger (- (LocalVariables|GetLen) 1))))
        (Math|Integer|IncrementInt (LocalVariables|GetIteration)
          (:%20%20
            (bind _returnvalue (Utilities|GetDataTableRow "/Game/Rogue/Blueprints/Core/TalentSystem/DT_Talents.DT_Talents" (Utilities|String|StringToName (Utilities|String|Replace (Utilities|String|ToString(Name) (Utilities|Array|Get(acopy) (Variables|Default|GetTalents) _output_get)) " ")))
              (:then
                (if (and (<= (.TalentBotDifficulty (Utilities|Struct|BreakS_TalentInfo _returnvalue)) DiffLeft) (not (Utilities|Array|ContainsItem (Variables|Default|GetRandomEnemyTalentsArray) (.Talent (Utilities|Struct|BreakS_TalentInfo _returnvalue)))))
                  (return (.Talent (Utilities|Struct|BreakS_TalentInfo _returnvalue)) "NewEnumerator14" (.TalentBotDifficulty (Utilities|Struct|BreakS_TalentInfo _returnvalue)) true)))))))
      (return "NewEnumerator0" "NewEnumerator14" 0 false)
      (else
        (LocalVariables|SetLen (Utilities|Array|Length (Variables|Default|GetItems)))
        (while (< (LocalVariables|GetIteration) 10)
          (bind _output_get_2 (LocalVariables|SetRandomNumber (Math|Random|RandomInteger (- (LocalVariables|GetLen) 1))))
          (Math|Integer|IncrementInt (LocalVariables|GetIteration)
            (:%20%20
              (bind _returnvalue_2 (Utilities|GetDataTableRow "/Game/Inventory/DT_Item.DT_Item" (Utilities|String|StringToName (Utilities|String|Replace (Utilities|String|ToString(Name) (Utilities|Array|Get(acopy) (Variables|Default|GetItems) _output_get_2)) " ")))
                (:then
                  (LocalVariables|SetItemName (.Name (Utilities|Struct|BreakS_Item _returnvalue_2)))
                  (LocalVariables|SetItemEquipType (Utilities|Select :Index (.EquipmentType (Utilities|Struct|BreakS_Item _returnvalue_2)) :NewEnumerator0 "NewEnumerator0" :NewEnumerator1 "NewEnumerator1" :NewEnumerator2 "NewEnumerator2" :NewEnumerator3 "NewEnumerator3" :NewEnumerator4 "NewEnumerator6" :NewEnumerator5 "NewEnumerator6" :NewEnumerator6 "NewEnumerator6" :NewEnumerator8 "NewEnumerator0" :NewEnumerator7 "NewEnumerator0" :NewEnumerator10 "NewEnumerator0" :NewEnumerator11 "NewEnumerator0"))
                  (Utilities|FlowControl|Sequence
                    (:then_0
                      (if (.ReturnValue (Utilities|Map|Find (Variables|Default|GetItemsArrayEquip) (LocalVariables|GetItemEquipType)))
                        (if (<= (.Value (Utilities|Map|Find (Variables|Default|GetItemsArrayEquip) (LocalVariables|GetItemEquipType))) (Utilities|Array|Length (Variables|Default|GetEnemyUnits)))
                          (LocalVariables|SetCanItemOfType? true)
                          (else
                            (LocalVariables|SetCanItemOfType? false)))
                        (else
                          (LocalVariables|SetCanItemOfType? true))))
                    (:then_1
                      (if (Math|Boolean|ANDBoolean (not (Utilities|Array|ContainsItem (Variables|Default|GetRandomEnemyItemsArray) (LocalVariables|GetItemName))) (LocalVariables|GetCanItemOfType?) (<= (Utilities|Struct|BreakS_ItemStats (.ItemStats (Utilities|Struct|BreakS_Item _returnvalue_2))) DiffLeft))
                        (if (.ReturnValue (Utilities|Map|Find (Variables|Default|GetItemsArrayEquip) (LocalVariables|GetItemEquipType)))
                          (bind _keys (Utilities|Map|Keys _itemsarrayequip))
                          (bind _values (Utilities|Map|Values _itemsarrayequip))
                          (Math|Integer|IncrementInt (Utilities|Array|Get(acopy) _values (Utilities|Array|FindItem _keys (LocalVariables|GetItemEquipType)))
                            (:%20%20
                              _))
                          (else
                            (Utilities|Map|Add (Variables|Default|GetItemsArrayEquip) (LocalVariables|GetItemEquipType) 1)))
                        (return "NewEnumerator0" (LocalVariables|GetItemName) (Utilities|Struct|BreakS_ItemStats (.ItemStats (Utilities|Struct|BreakS_Item _returnvalue_2))) true)))))))))
        (return "NewEnumerator0" "NewEnumerator14" 0 false)))
    (else
      (return "NewEnumerator0" "NewEnumerator14" 0 false))))

(fn CheckEquipmentSlotsandSetRandom
  (params (ItemSlots :type Array%20of%20S%20Slot%20Structures) (WhichToCheck :type Array%20of%20Integers))
  (bind _emptyslots (LocalVariables|GetEmptySlots))
  (for _array_element WhichToCheck
    (if (== (.ItemID (Utilities|Struct|BreakS_Slot (Utilities|Array|Get(acopy) ItemSlots _array_element))) "Empty")
      (Utilities|Array|Add (LocalVariables|GetEmptySlots) _array_element)))
  (if (Utilities|Array|IsEmpty _emptyslots)
    (return false 0)
    (else
      (return false (Math|Random|RandomInteger (- (Utilities|Array|Length _emptyslots) 1))))))

(fn AdditivePlayerItemsDiffuculty
  (for _array_element (Variables|/Game/Rogue/Blueprints/Core/Player/BP_CombatPlayerActions.BP_CombatPlayerActions_C|GetPlayerUnits (Variables|Default|GetPlayerActions))
    (Variables|Default|SetDifficulty (+ (.Hardness (Utilities|Struct|BreakS_UnitDataStats (.Stats (Utilities|Struct|BreakS_UnitDataF (Variables|/Game/Rogue/Blueprints/Core/Units/BP_Unit.BP_Unit_C|GetUnitData _array_element))))) (Variables|Default|GetDifficulty)))))

(fn AddTalentsandItemstoRandomUnits
  (bind _randomenemytalentsarray (Variables|Default|GetRandomEnemyTalentsArray))
  (bind _randomenemyitemsarray (Variables|Default|GetRandomEnemyItemsArray))
  (bind _randomenemyitemsarray_2 (Variables|Default|GetRandomEnemyItemsArray))
  (bind _randomenemytalentsarray_2 (Variables|Default|GetRandomEnemyTalentsArray))
  (bind _returnvalue (Utilities|Array|Length _randomenemytalentsarray_2))
  (bind _returnvalue_2 (- _returnvalue 1))
  (bind _returnvalue_3 (Math|Random|RandomInteger _returnvalue_2))
  (bind _output (Utilities|Array|Get(acopy) _randomenemytalentsarray_2 _returnvalue_3))
  (LocalVariables|SetUnitsNum (- (Utilities|Array|Length (Variables|Default|GetEnemyUnits)) 1))
  (Utilities|FlowControl|Sequence
    (:then_0
      (LocalVariables|SetInitNum (Utilities|Array|Length (Variables|Default|GetRandomEnemyTalentsArray)))
      (while (and (Utilities|Array|IsNotEmpty (Variables|Default|GetRandomEnemyTalentsArray)) (< (LocalVariables|GetIter) (* (LocalVariables|GetInitNum) 5)))
        (LocalVariables|SetUnitIndex (Math|Random|RandomInteger (LocalVariables|GetUnitsNum)))
        (Math|Integer|IncrementInt (LocalVariables|GetIter)
          (:%20%20
            (if (not (Utilities|Array|ContainsItem (Variables|/Game/Rogue/Blueprints/Core/Units/BP_Unit.BP_Unit_C|GetTalents (Utilities|Array|Get(acopy) (Variables|Default|GetEnemyUnits) (LocalVariables|GetUnitIndex))) _output))
              (Default|ModifyUnitDatawithTalents (Utilities|Array|Get(acopy) (Variables|Default|GetEnemyUnits) (LocalVariables|GetUnitIndex)) (Utilities|Array|MakeArray _output) (Variables|/Game/Rogue/Blueprints/Core/Units/BP_Unit.BP_Unit_C|GetUnitData (Utilities|Array|Get(acopy) (Variables|Default|GetEnemyUnits) (LocalVariables|GetUnitIndex))) false)
              (Utilities|Array|RemoveIndex _randomenemytalentsarray (Utilities|Array|FindItem _randomenemytalentsarray _output)))))))
    (:then_1
      (LocalVariables|SetInitNum (Utilities|Array|Length (Variables|Default|GetRandomEnemyItemsArray)))
      (while (and (Utilities|Array|IsNotEmpty (Variables|Default|GetRandomEnemyItemsArray)) (< (LocalVariables|GetIter) (* (LocalVariables|GetInitNum) 5)))
        (LocalVariables|SetUnitIndex (Math|Random|RandomInteger (LocalVariables|GetUnitsNum)))
        (Math|Integer|IncrementInt (LocalVariables|GetIter)
          (:%20%20
            (bind _output_get (LocalVariables|SetItem (Utilities|Array|Get(acopy) _randomenemyitemsarray_2 (Math|Random|RandomInteger (- (Utilities|Array|Length _randomenemyitemsarray_2) 1)))))
            (if (not (Utilities|Array|ContainsItem (.ItemNamesArray (Default|GetEquipmentItems (Utilities|Array|Get(acopy) (Variables|Default|GetEnemyUnits) (LocalVariables|GetUnitIndex)))) _output_get))
              (bind _returnvalue_4 (Utilities|GetDataTableRow "/Game/Inventory/DT_Item.DT_Item" (Utilities|Name|EnumtoName (LocalVariables|GetItem)))
                (:then
                  (switch Utilities|FlowControl|Switch|SwitchonE_EquipmentType (.EquipmentType (Utilities|Struct|BreakS_Item _returnvalue_4))
                    (:NewEnumerator1
                      (bind (_cansetsomeitem _whichtoset) (CallFunction|CheckEquipmentSlotsandSetRandom (.ItemSlotsArray (Default|GetEquipmentItems (Utilities|Array|Get(acopy) (Variables|Default|GetEnemyUnits) (LocalVariables|GetUnitIndex)))) (Utilities|Array|MakeArray 0)))
                      (LocalVariables|SetCanSetSomeItem _cansetsomeitem)
                      (LocalVariables|SetWhictItemToSet _whichtoset))
                    (:NewEnumerator2
                      (bind (_cansetsomeitem_2 _whichtoset_2) (CallFunction|CheckEquipmentSlotsandSetRandom (.ItemSlotsArray (Default|GetEquipmentItems (Utilities|Array|Get(acopy) (Variables|Default|GetEnemyUnits) (LocalVariables|GetUnitIndex)))) (Utilities|Array|MakeArray 1)))
                      (LocalVariables|SetCanSetSomeItem _cansetsomeitem_2)
                      (LocalVariables|SetWhictItemToSet _whichtoset_2))
                    (:NewEnumerator3
                      (bind (_cansetsomeitem_3 _whichtoset_3) (CallFunction|CheckEquipmentSlotsandSetRandom (.ItemSlotsArray (Default|GetEquipmentItems (Utilities|Array|Get(acopy) (Variables|Default|GetEnemyUnits) (LocalVariables|GetUnitIndex)))) (Utilities|Array|MakeArray 2)))
                      (LocalVariables|SetCanSetSomeItem _cansetsomeitem_3)
                      (LocalVariables|SetWhictItemToSet _whichtoset_3))
                    (:NewEnumerator4
                      (bind (_cansetsomeitem_4 _whichtoset_4) (CallFunction|CheckEquipmentSlotsandSetRandom (.ItemSlotsArray (Default|GetEquipmentItems (Utilities|Array|Get(acopy) (Variables|Default|GetEnemyUnits) (LocalVariables|GetUnitIndex)))) (Utilities|Array|MakeArray 3 4) :!label _label))
                      (LocalVariables|SetCanSetSomeItem _cansetsomeitem_4)
                      (LocalVariables|SetWhictItemToSet _whichtoset_4))
                    (:NewEnumerator5
                      (goto _label))
                    (:NewEnumerator6
                      (goto _label))
                    (:NewEnumerator8
                      (bind (_cansetsomeitem_5 _whichtoset_5) (CallFunction|CheckEquipmentSlotsandSetRandom (.ItemSlotsArray (Default|GetEquipmentItems (Utilities|Array|Get(acopy) (Variables|Default|GetEnemyUnits) (LocalVariables|GetUnitIndex)))) (Utilities|Array|MakeArray 0 1 2)))
                      (LocalVariables|SetCanSetSomeItem _cansetsomeitem_5)
                      (LocalVariables|SetWhictItemToSet _whichtoset_5))
                    (:NewEnumerator7
                      (bind (_cansetsomeitem_6 _whichtoset_6) (CallFunction|CheckEquipmentSlotsandSetRandom (.ItemSlotsArray (Default|GetEquipmentItems (Utilities|Array|Get(acopy) (Variables|Default|GetEnemyUnits) (LocalVariables|GetUnitIndex)))) (Utilities|Array|MakeArray 0 1 2 3 4)))
                      (LocalVariables|SetCanSetSomeItem _cansetsomeitem_6)
                      (LocalVariables|SetWhictItemToSet _whichtoset_6)))
                  (if (LocalVariables|GetCanSetSomeItem)
                    (Utilities|Array|SetArrayElem (Variables|/Game/Rogue/Blueprints/Core/Units/BP_Unit.BP_Unit_C|GetCurrentEquipmentItems (Utilities|Array|Get(acopy) (Variables|Default|GetEnemyUnits) (LocalVariables|GetUnitIndex))) (+ (LocalVariables|GetWhictItemToSet) (- (Utilities|Array|Length (Variables|/Game/Rogue/Blueprints/Core/Units/BP_Unit.BP_Unit_C|GetCurrentEquipmentItems (Utilities|Array|Get(acopy) (Variables|Default|GetEnemyUnits) (LocalVariables|GetUnitIndex)))) 5)) (Utilities|Struct|MakeS_Slot (Utilities|Name|EnumtoName (LocalVariables|GetItem)) 1 false))
                    (Utilities|Array|RemoveIndex _randomenemyitemsarray (Utilities|Array|FindItem _randomenemyitemsarray (LocalVariables|GetItem))))))))))
      (for _array_element (Variables|Default|GetEnemyUnits)
        (Default|ModifyUnitDatawithItems _array_element (Variables|/Game/Rogue/Blueprints/Core/Units/BP_Unit.BP_Unit_C|GetUnitData _array_element) false)))))

(fn GenerateFightOfNeededDifficulty
  (CallFunction|AdditivePlayerItemsDiffuculty)
  (bind _units (CallFunction|RandomizeEnemies))
  (bind _keys (Utilities|Map|Keys _units))
  (for _array_element _keys
    (if (== (.Value (Utilities|Map|Find _units _array_element)) 1)
      (bind _returnvalue (Game|SpawnActorfromClass "/Game/Rogue/Blueprints/Core/Units/BP_Unit.BP_Unit_C" (Math|Transform|MakeTransform "3.591587,-405.000000,72.636747" "0.000000,-90.000000,0.000000") "Undefined" "MultiplyWithRoot" 0 _array_element true 0 0 :!label _label))
      (Default|SetTeamIndex _returnvalue 1)
      (Utilities|Array|Add (Variables|Default|GetEnemyUnits) _returnvalue)
      (else
        (for _index (range 0 (- (.Value (Utilities|Map|Find _units _array_element)) 1))
          (goto _label)))))
  (while (< (Variables|Default|GetCurrentDifficulty) (Variables|Default|GetDifficulty))
    (bind (_talent _item _diffchange _smthfound_) (CallFunction|RandomizeTalentsandItems (- (+ (Variables|Default|GetDifficulty) 8) (Variables|Default|GetCurrentDifficulty))))
    (if _smthfound_
      (if (Utilities|Enum|NotEqual(Enum) _talent "NewEnumerator0")
        (Utilities|Array|AddUnique (Variables|Default|GetRandomEnemyTalentsArray) _talent)
        (else
          (Utilities|Array|AddUnique (Variables|Default|GetRandomEnemyItemsArray) _item)))
      (Variables|Default|SetCurrentDifficulty (+ (Variables|Default|GetCurrentDifficulty) _diffchange))))
  (CallFunction|AddTalentsandItemstoRandomUnits))

(fn SpawnObstacles
  (bind _returnvalue (Actor|GetActorOfClass "/Script/NavigationSystem.RecastNavMesh"))
  (bind _output_get (Variables|Default|SetNav%20Data _returnvalue))
  (Game|SpawnActorfromClass "/Game/Rogue/LevelObjects/BP_Acid.BP_Acid_C" (Math|Transform|MakeTransform (Math|Vector|MakeVectorNetQuantize (.X (Math|Vector|BreakVector (.RandomLocation (AI|Navigation|GetRandomReachablePointinRadius (Transformation|GetActorLocation (Variables|Default|GetPlayerActions)) 5e+02 _output_get 0)))) (.Y (Math|Vector|BreakVector (.RandomLocation (AI|Navigation|GetRandomReachablePointinRadius (Transformation|GetActorLocation (Variables|Default|GetPlayerActions)) 5e+02 _output_get 0)))) 2.0) (Math|Rotator|SelectRotator (Math|Rotator|MakeRotator 0.0 0.0 0.0) (Math|Rotator|MakeRotator 0.0 0.0 9e+01) (Math|Random|RandomBool)) "4.000000,4.000000,1.000000") "AlwaysSpawn" "MultiplyWithRoot" 0 "NewEnumerator0" "NewEnumerator8" false 0))