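; Combat scenario actor that quick-starts a fight on BeginPlay through BP_CombatSystem, passing its grid and unit data.
; The construction script finds that system and spawns a grid centred on this actor as a preview.
; Separate helper functions, not called here, fill unit data from level BP_Units: teams parsed from display names, non-zero teams as AI, and desired tiles from unit positions.
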(event EventBeginPlay
  (Default|QuickStartCombat (Variables|Default|GetCombatSystem) (Variables|Default|GetGridData) (Variables|Default|GetUnitsData) self))

(event Collision|EventActorBeginOverlap
  (params (OtherActor :type Actor%20Object%20Reference)))

(event EventTick
  (params (DeltaSeconds :type Float%20%28single-precision%29)))

(fn ConstructionScript
  (bind _returnvalue (Actor|GetActorOfClass "/Game/Rogue/Blueprints/Core/Combat/BP_CombatSystem.BP_CombatSystem_C"))
  (Variables|Default|SetCombatSystem _returnvalue)
  (Utilities|Struct|SetmembersinS_QuickCombat_Grid (Variables|Default|GetGridData) (Transformation|GetActorLocation))
  (CallFunction|SpawnGrid))

(fn BuildTeamsBasedonUnitNames
  (bind _outactors (Actor|GetAllActorsOfClass "/Game/Rogue/Blueprints/Core/Units/BP_Unit.BP_Unit_C"))
  (for _array_element _outactors
    (LocalVariables|SetCurUnit _array_element)
    (LocalVariables|SetTeamIndex (Math|Conversions|ToInteger(Byte) (.LeftS (Utilities|String|Split (.RightS (Utilities|String|Split (Utilities|GetDisplayName (LocalVariables|GetCurUnit)) "Team")) "_"))))
    (if (< (Utilities|Array|Length (LocalVariables|GetUnitsTeams)) (+ (LocalVariables|GetTeamIndex) 1)) ; Is array too small
      (Utilities|Array|Resize (LocalVariables|GetUnitsTeams) (+ (LocalVariables|GetTeamIndex) 1)))
    (Utilities|Array|Add (Utilities|Struct|BreakS_UnitArray (Utilities|Array|Get(acopy) (LocalVariables|GetUnitsTeams) (LocalVariables|GetTeamIndex))) (LocalVariables|GetCurUnit)))
  (Utilities|Array|RemoveItem :TargetArray (LocalVariables|GetUnitsTeams)) ; Remove empty groups
  (Utilities|Struct|SetmembersinS_QuickCombat_UnitTeams (Variables|Default|GetUnitsData) (LocalVariables|GetUnitsTeams)))

(fn BuildAIListBasedonTeamIndexes
  (for (_array_element _array_index) (.UnitTeams (Utilities|Struct|BreakS_QuickCombat_UnitTeams (Variables|Default|GetUnitsData)))
    (if (!= _array_index 0)
      (Utilities|Array|AppendArray (LocalVariables|GetAIs) (Utilities|Struct|BreakS_UnitArray _array_element))))
  (Utilities|Struct|SetmembersinS_QuickCombat_UnitTeams (Variables|Default|GetUnitsData) (LocalVariables|GetAIs)))

(fn BuildDesiredGridIndexesBasedonUnitLocations
  (for _array_element (.UnitTeams (Utilities|Struct|BreakS_QuickCombat_UnitTeams (Variables|Default|GetUnitsData)))
    (for _array_element_2 (Utilities|Struct|BreakS_UnitArray _array_element)
      (bind _index (Default|GetTileIndexfromWorldLoc (Variables|/Game/Rogue/Blueprints/Core/Combat/BP_CombatSystem.BP_CombatSystem_C|GetGrid (Variables|Default|GetCombatSystem)) (Transformation|GetActorLocation _array_element_2)))
      (Utilities|Map|Add (LocalVariables|GetDesIndexes) _array_element_2 _index)))
  (Utilities|Struct|SetmembersinS_QuickCombat_UnitTeams (Variables|Default|GetUnitsData) (LocalVariables|GetDesIndexes)))

(fn SpawnGrid
  (bind _combatsystem (Variables|Default|GetCombatSystem))
  (bind _griddata (Variables|Default|GetGridData))
  (bind (_generategridbeforestartingcombat _centerlocation _tilesize _tilecount _shape _useenvironment) (Utilities|Struct|BreakS_QuickCombat_Grid _griddata))
  (bind _grid (Variables|/Game/Rogue/Blueprints/Core/Combat/BP_CombatSystem.BP_CombatSystem_C|GetGrid _combatsystem))
  (Utilities|IsValid _combatsystem
    (:Is%20Valid
      (Utilities|IsValid _grid
        (:Is%20Valid
          (Default|SpawnGrid _grid _centerlocation _tilesize (Math|Conversions|ToVector2D(IntPoint) _tilecount) _shape _useenvironment))))))