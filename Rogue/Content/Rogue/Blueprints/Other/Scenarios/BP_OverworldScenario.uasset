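; Overworld scenario actor that registers groups of units with the overworld unit groups manager at play start.
; On BeginPlay, after a brief delay, it walks the UnitGroups map, sets each unit's context, adds units to their group and flags encounter groups.
; BuildGroupsBasedOnUnitNames rebuilds that map from all BP_Unit display names, parsing the ID after "Group" and treating "_AI" as an encounter.
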(event EventBeginPlay
  (Utilities|FlowControl|Delay 0.001)
  (bind _returnvalue (Actor|GetActorOfClass "/Game/Rogue/Blueprints/Core/Units/OverworldUnitGroups/BP_OverworldUnitGroupsManager.BP_OverworldUnitGroupsManager_C"))
  (Variables|Default|SetOverworldUnitGroupManager _returnvalue)
  (bind _values (Utilities|Map|Values (Variables|Default|GetUnitGroups)))
  (for _array_element _values
    (for _array_element_2 (.Units (Utilities|Struct|BreakS_OverworldUnitGroup _array_element))
      (Default|SetUnitContext _array_element_2 "NewEnumerator1")
      (Default|AddUnittoGroup (Variables|Default|GetOverworldUnitGroupManager) _array_element_2 (.GroupID (Utilities|Struct|BreakS_OverworldUnitGroup _array_element))))
    (Default|SetGroupIsEncounter (Variables|Default|GetOverworldUnitGroupManager) (.IsEncounter (Utilities|Struct|BreakS_OverworldUnitGroup _array_element)) (.GroupID (Utilities|Struct|BreakS_OverworldUnitGroup _array_element)))))

(fn ConstructionScript)

(fn BuildGroupsBasedonUnitNames
  (Utilities|Map|Clear (Variables|Default|GetUnitGroups))
  (bind _outactors (Actor|GetAllActorsOfClass "/Game/Rogue/Blueprints/Core/Units/BP_Unit.BP_Unit_C"))
  (for _array_element _outactors
    (bind _output_get (LocalVariables|SetCurUnit _array_element))
    (LocalVariables|SetGroupID (Math|Conversions|ToInteger(Byte) (.LeftS (Utilities|String|Split (.RightS (Utilities|String|Split (Utilities|GetDisplayName _output_get) "Group")) "_"))))
    (LocalVariables|SetIsEncounter (Utilities|String|Contains (Utilities|GetDisplayName (LocalVariables|GetCurUnit)) "_AI"))
    (LocalVariables|SetGroup (.Value (Utilities|Map|Find (Variables|Default|GetUnitGroups) (LocalVariables|GetGroupID))))
    (Utilities|Struct|SetmembersinS_OverworldUnitGroup (LocalVariables|GetGroup) (LocalVariables|GetGroupID) (LocalVariables|GetIsEncounter))
    (Utilities|Array|AddUnique (.Units (Utilities|Struct|BreakS_OverworldUnitGroup (LocalVariables|GetGroup))) (LocalVariables|GetCurUnit))
    (Utilities|Map|Add (Variables|Default|GetUnitGroups) (LocalVariables|GetGroupID) (LocalVariables|GetGroup))))