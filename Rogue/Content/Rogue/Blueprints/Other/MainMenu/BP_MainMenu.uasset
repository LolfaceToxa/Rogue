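; BP_MainMenu runs the main menu, creating the W_MainMenu widget on BeginPlay and adding it to the viewport.
; It then loops endlessly: it streams in L_Square, tells the widget to show its background, waits, hides the background, waits again and unloads the level.
; The cycle is a chain of latent stream and delay nodes wired back to the load, with only that one level cycled.
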(event EventBeginPlay
  (bind _returnvalue (Game|ConstructObjectfromClass "/Game/Rogue/Blueprints/Other/MainMenu/W_MainMenu.W_MainMenu_C"))
  (bind _output_get (Variables|Default|SetMainMenu _returnvalue))
  (UserInterface|Viewport|AddtoViewport _output_get 0)
  (Game|LoadStreamLevel(byName) "L_Square" true :!label _label)
  (Default|EventShowBackground (Variables|Default|GetMainMenu))
  (Utilities|FlowControl|Delay 1e+01)
  (Default|EventHideBackground (Variables|Default|GetMainMenu))
  (Utilities|FlowControl|Delay 5.0)
  (Game|UnloadStreamLevel(byName) "L_Square" false)
  (goto _label))

(fn ConstructionScript)