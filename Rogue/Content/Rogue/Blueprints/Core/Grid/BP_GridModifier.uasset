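; BP_GridModifier is an editor-placed marker for a grid tile type, such as normal, obstacle, costlier movement or flying-only, and is hidden in game.
; Its construction script takes mesh and flat material from the Shape data, then colors and fills the material by Type.
; It overlaps one custom trace channel and blocks another, presumably for grid detection, and has no active runtime logic.
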(event EventBeginPlay)

(event Collision|EventActorBeginOverlap
  (params (OtherActor :type Actor%20Object%20Reference)))

(event EventTick
  (params (DeltaSeconds :type Float%20%28single-precision%29)))

(fn ConstructionScript
  (bind _staticmesh (Variables|Default|GetStaticMesh))
  (bind _shape (Variables|Default|GetShape))
  (bind _data (CallFunction|GetShapeData _shape))
  (Components|StaticMesh|SetStaticMesh _staticmesh (.mesh _data))
  (Rendering|Material|SetMaterial _staticmesh 0 (.flatmaterial _data))
  (Rendering|Material|SetVectorParameterValueonMaterials _staticmesh "Color" (Math|Conversions|ToVector(LinearColor) (Utilities|Select :Index (Variables|Default|GetType) :NewEnumerator0 "" :NewEnumerator1 "(R=1.000000,G=1.000000,B=1.000000,A=1.000000)" :NewEnumerator2 "(R=1.000000,G=0.000000,B=0.000000,A=1.000000)" :NewEnumerator3 "(R=0.720833,G=0.590884,B=0.168586,A=1.000000)" :NewEnumerator4 "(R=0.216667,G=0.068795,B=0.000000,A=1.000000)" :NewEnumerator5 "(R=0.184801,G=0.012678,B=0.416667,A=1.000000)")))
  (Rendering|Material|SetScalarParameterValueonMaterials _staticmesh "isFilled" 1.0)
  (Collision|SetCollisionResponsetoChannel (Variables|Default|GetStaticMesh) "ECC_GameTraceChannel1" "ECR_Overlap")
  (Collision|SetCollisionResponsetoChannel (Variables|Default|GetStaticMesh) "ECC_GameTraceChannel4" "ECR_Block")
  (Rendering|SetActorHiddenInGame true))