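; BP_Grid is a tile grid actor that builds a shaped, snapped grid in the world and maps cursor positions to tile indices.
; SpawnGrid runs at construction, storing each tile in GridTiles and forwarding it to a child BP_GridVisual actor.
; Sphere traces set tile height from the ground and tile type from any BP_GridModifier hit.
; Cursor lookup uses a hit trace with a grid-plane intersection fallback; only square shapes resolve to indices.
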(event EventBeginPlay)

(event Collision|EventActorBeginOverlap
  (params (OtherActor :type Actor%20Object%20Reference)))

(event EventTick
  (params (DeltaSeconds :type Float%20%28single-precision%29)))

(fn ConstructionScript
  (Variables|Default|SetGrid%20Visual (.AsBP%20Grid%20Visual (Utilities|Casting|CastToBP_GridVisual (Variables|/Script/Engine.ChildActorComponent|GetChildActor (Variables|Default|GetChildActor_GridVisual)))))
  (CallFunction|SpawnGrid (Transformation|GetActorLocation) (Variables|Default|GetGrid%20Tile%20Size) (Variables|Default|GetGrid%20Tile%20Count) (Variables|Default|GetGrid%20Shape) true))

(fn SpawnGrid
  (params (CenterLocation :type Vector) (TileSize :type Vector) (TileCount :type Vector%202D%20Structure) (Shape :type E_GridShape%20Enum :default "NewEnumerator1") (UseEnvironment :type Boolean))
  (Variables|Default|SetGrid%20Center%20Location CenterLocation)
  (Variables|Default|SetGrid%20Tile%20Size TileSize)
  (Variables|Default|SetGrid%20Shape Shape)
  (Variables|Default|SetGrid%20Tile%20Count (Math|Vector2D|MakeVector2D (Math|Conversions|ToFloat(Integer) (Math|Float|Round (.x TileCount))) (Math|Conversions|ToFloat(Integer) (Math|Float|Round (.y TileCount)))))
  (CallFunction|DestroyGrid)
  (Default|InitGridVisual (Variables|Default|GetGrid%20Visual) self)
  (bind (_center _bottomleft) (CallFunction|CalculateCenterandBottomLeft))
  (Variables|Default|SetGrid%20Center%20Location _center)
  (Variables|Default|SetGridBottomLeftCornerLocation _bottomleft)
  (for _index (range 0 (- (Math|Float|Round (.x (Variables|Default|GetGrid%20Tile%20Count))) 1))
    (LocalVariables|SetX _index)
    (for _index_2 (range 0 (- (Math|Float|Round (.y (Variables|Default|GetGrid%20Tile%20Count))) 1))
      (LocalVariables|SetY _index_2)
      (LocalVariables|SetIndex (Utilities|Struct|MakeIntPoint (LocalVariables|GetX) (LocalVariables|GetY)))
      (bind _output_get (LocalVariables|SetTileTransform (Math|Transform|MakeTransform (+ (Variables|Default|GetGridBottomLeftCornerLocation) (* (Variables|Default|GetGrid%20Tile%20Size) (Math|Vector|MakeVector (Math|Conversions|ToFloat(Integer) (LocalVariables|GetX)) (Math|Conversions|ToFloat(Integer) (LocalVariables|GetY)) 0.0)) "0.000000,0.000000,2.000000") (CallFunction|GetTileRotationfromGrid (LocalVariables|GetIndex)) (/ (Variables|Default|GetGrid%20Tile%20Size) (.MeshSize (Utilities|Struct|BreakS_GridShapeData (CallFunction|GetCurrentShapeData)))))))
      (Variables|Default|SetTileTransfom_ _output_get)
      (if UseEnvironment
        (bind (_tile_type _outlocation) (CallFunction|TraceforGround (.location (Variables|Default|GetTileTransfom_))))
        (CallFunction|AddGridTile (Utilities|Struct|MakeS_TileData (LocalVariables|GetIndex) _tile_type (Math|Transform|MakeTransform _outlocation (.rotation (Variables|Default|GetTileTransfom_)) (.scale (Variables|Default|GetTileTransfom_)))))
        (else
          (CallFunction|AddGridTile (Utilities|Struct|MakeS_TileData (LocalVariables|GetIndex) "NewEnumerator1" (Variables|Default|GetTileTransfom_))))))))

(fn GetCurrentShapeData
  (return (CallFunction|GetShapeData (Variables|Default|GetGrid%20Shape))))

(fn DestroyGrid
  (Utilities|Map|Clear (Variables|Default|GetGrid%20Tiles))
  (Default|DestroyGridVisual (Variables|Default|GetGrid%20Visual)))

(fn CalculateCenterandBottomLeft
  (bind _grid_tile_count (Variables|Default|GetGrid%20Tile%20Count))
  (LocalVariables|SetC (CallFunction|SnapVectortoVector (Variables|Default|GetGrid%20Center%20Location) (Variables|Default|GetGrid%20Tile%20Size)))
  (return (LocalVariables|GetC) (- (LocalVariables|GetC) (Math|Conversions|ToVector(Vector2D) (* (/ (- (Variables|Default|GetGrid%20Tile%20Count) (Math|Vector2D|MakeVector2D (Math|Float|SelectFloat 0.0 1.0 (CallFunction|IsFloatEven (.x _grid_tile_count))) (Math|Float|SelectFloat 0.0 1.0 (CallFunction|IsFloatEven (.y _grid_tile_count))))) "(X=2.000000,Y=2.000000)") (Math|Conversions|ToVector2D(Vector) (Variables|Default|GetGrid%20Tile%20Size)))))))

(fn TraceforGround
  (params (Location :type Vector))
  (Variables|Default|SetRadius (/ (.x (Variables|Default|GetGrid%20Tile%20Size)) 3.0))
  (bind _outhits (Collision|MultiSphereTraceByChannel (+ Location "0.000000,0.000000,1000.000000") (+ Location "0.000000,0.000000,-1000.000000") (Variables|Default|GetRadius) "TraceTypeQuery3" false 0 "None"))
  (if (> (Utilities|Array|Length _outhits) 0)
    (LocalVariables|SetRetType "NewEnumerator1")
    (for _array_element _outhits
      (bind _asbp_grid_modifier (Utilities|Casting|CastToBP_GridModifier (.HitActor (Collision|BreakHitResult _array_element)))
        (:then
          (LocalVariables|SetRetType (Variables|/Game/Rogue/Blueprints/Core/Grid/BP_GridModifier.BP_GridModifier_C|GetType _asbp_grid_modifier)))
        (:CastFailed
          (LocalVariables|SetRetZ (+ (Math|Float|SnapToGrid(Float) (- (.Z (Class|KismetMathLibrary|BreakVector3f (.Location (Collision|BreakHitResult _array_element)))) (/ (Variables|Default|GetRadius) 1.01)) (.z (Variables|Default|GetGrid%20Tile%20Size))) 1e+01)))))
    (return (LocalVariables|GetRetType) (Math|Vector|MakeVector (.x Location) (.y Location) (LocalVariables|GetRetZ)))
    (else
      (return "NewEnumerator0" Location))))

(fn AddGridTile
  (params (Data :type S%20Tile%20Data%20Structure))
  (Utilities|Map|Add (Variables|Default|GetGrid%20Tiles) (.index Data) Data)
  (Default|UpdateTileVisual (Variables|Default|GetGrid%20Visual) Data))

(fn GetTileRotationfromGrid
  (params (GridIndex :type Int%20Point%20Structure))
  (return "0, 0, 0"))

(fn GetCursorLoconGrid
  (params (PlayerIndex :type Integer))
  (bind _returnvalue (Game|GetPlayerController PlayerIndex))
  (bind _grid_center_location (Variables|Default|GetGrid%20Center%20Location))
  (bind (_hitresult _returnvalue_2) (Game|Player|GetHitResultUnderCursorbyChannel _returnvalue "TraceTypeQuery4" false))
  (bind (_worldlocation _worlddirection) (Game|Player|ConvertMouseLocationToWorldSpace _returnvalue))
  (bind _returnvalue_3 (Class|KismetMathLibrary|MakePlanefromPointandNormal _grid_center_location "0.000000,0.000000,1.000000"))
  (bind _returnvalue_4 (* _worlddirection 999999.0))
  (bind _returnvalue_5 (+ _worldlocation _returnvalue_4))
  (bind (_t _intersection _returnvalue_6) (Class|KismetMathLibrary|LinePlaneIntersection _worldlocation _returnvalue_5 _returnvalue_3))
  (if _returnvalue_2
    (return (.Location (Collision|BreakHitResult _hitresult)))
    (elif _returnvalue_6
      (return _intersection)
      (else
        (return "-999.000000,-999.000000,-999.000000")))))

(fn GetTileIndexfromWorldLoc
  (params (Location :type Vector))
  (LocalVariables|SetLoc%20On%20Grid (- Location (Variables|Default|GetGridBottomLeftCornerLocation)))
  (switch Utilities|FlowControl|Switch|SwitchonE_GridShape (Variables|Default|GetGrid%20Shape)
    (:NewEnumerator1
      (return (Utilities|Struct|MakeIntPoint -999 -999)))
    (:NewEnumerator0
      (LocalVariables|SetSnap%20Loc%20On%20Grid (Math|Conversions|ToVector2D(Vector) (CallFunction|SnapVectortoVector (LocalVariables|GetLoc%20On%20Grid) (Variables|Default|GetGrid%20Tile%20Size))))
      (return (Class|KismetMathLibrary|ToIntPoint(Vector2D) (/ (LocalVariables|GetSnap%20Loc%20On%20Grid) (Math|Conversions|ToVector2D(Vector) (Variables|Default|GetGrid%20Tile%20Size))))))))

(fn GetTileIndexUnderCursor
  (params (PlayerIndex :type Integer))
  (bind _location (CallFunction|GetCursorLoconGrid PlayerIndex))
  (bind _index (CallFunction|GetTileIndexfromWorldLoc _location))
  (return _index))