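; Heal spell animation actor that plays a spinning, green-tinted mesh effect on the target tile.
; On play, it moves to the target tile and takes its facing from the origin-to-target direction.
; A timeline drives scale, yaw on six meshes and opacity on three, firing the tile-hit callback once shortly after starting and completing the animation when finished.
; The construction script tints each mesh its own shade of green.
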(event EventBeginPlay
  (|CallParentFunction) ; This node is disabled and will not be called.\nDrag off pins to build functionality.
)

(event EventEventPlaySpellAnim
  (Transformation|SetActorLocationAndRotation (.location (CallFunction|GetTileTransform (Variables|Default|GetTargetIndex))) (Math|Rotator|FindLookatRotation (Math|Conversions|ToVector(Vector2D) (Math|Conversions|ToVector2D(IntPoint) (Variables|Default|GetOriginIndex))) (Math|Conversions|ToVector(Vector2D) (Math|Conversions|ToVector2D(IntPoint) (Variables|Default|GetTargetIndex)))))
  (bind (_direction _opacity _scale _rot) (Timeline|Timeline_Heal PlayFromStart)
    (:Update
      (Transformation|SetRelativeScale3D (Variables|Default|GetAnim_RotationScale) _scale)
      (Rendering|Material|SetScalarParameterValueonMaterials (Variables|Default|GetStaticMesh) "Opacity" _opacity)
      (Transformation|SetRelativeRotation (Variables|Default|GetStaticMesh) (Math|Rotator|MakeRotator 0.0 0.0 _rot) false false)
      (if (>= (Components|Timeline|GetPlaybackPosition (Variables|Default|GetTimeline_Heal)) 0.2)
        (Utilities|FlowControl|DoOnce false
          (:Completed
            (Default|CallOnSpellAnimHitTIle self (Variables|Default|GetTargetIndex))))))
    (:Finished
      (CallFunction|EventCompleteSpellAnim))))

(fn ConstructionScript
  (|CallParentFunction)
  (Rendering|Material|SetVectorParameterValueonMaterials (Variables|Default|GetStaticMesh) "Color" (Math|Conversions|ToVector(LinearColor) "(R=0.334918,G=0.645833,B=0.312153,A=1.000000)"))
  (Rendering|Material|SetVectorParameterValueonMaterials (Variables|Default|GetStaticMesh1) "Color" (Math|Conversions|ToVector(LinearColor) "(R=0.244777,G=0.550000,B=0.201667,A=1.000000)"))
  (Rendering|Material|SetVectorParameterValueonMaterials (Variables|Default|GetStaticMesh2) "Color" (Math|Conversions|ToVector(LinearColor) "(R=0.149427,G=0.683333,B=0.093958,A=1.000000)"))
  (Rendering|Material|SetVectorParameterValueonMaterials (Variables|Default|GetStaticMesh3) "Color" (Math|Conversions|ToVector(LinearColor) "(R=0.150168,G=0.645833,B=0.244994,A=1.000000)"))
  (Rendering|Material|SetVectorParameterValueonMaterials (Variables|Default|GetStaticMesh4) "Color" (Math|Conversions|ToVector(LinearColor) "(R=0.186982,G=0.645833,B=0.153385,A=1.000000)"))
  (Rendering|Material|SetVectorParameterValueonMaterials (Variables|Default|GetStaticMesh5) "Color" (Math|Conversions|ToVector(LinearColor) "(R=0.194387,G=0.445833,B=0.078603,A=1.000000)")))