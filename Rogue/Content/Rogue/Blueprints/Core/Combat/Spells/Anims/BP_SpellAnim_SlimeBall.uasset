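; Spell animation actor that shows a slime ball flying from the origin tile to the target tile.
; When played, a single timeline moves it between tile locations with an added height curve while driving its scale and the opacity of three meshes.
; The construction script tints each mesh a different green, and the timeline's end signals spell animation completion.
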(event EventBeginPlay
  (|CallParentFunction) ; This node is disabled and will not be called.\nDrag off pins to build functionality.
)

(event EventEventPlaySpellAnim
  (Transformation|SetActorLocation (.location (CallFunction|GetTileTransform (Variables|Default|GetTargetIndex))) false false)
  (bind (_direction _opacity _scale _loca _locz) (Timeline|Timeline_SlimeBall PlayFromStart)
    (:Update
      (Transformation|SetRelativeScale3D (Variables|Default|GetAnim_RotationScale) _scale)
      (Rendering|Material|SetScalarParameterValueonMaterials (Variables|Default|GetStaticMesh) "Opacity" _opacity)
      (Transformation|SetActorLocation (+ (Math|Vector|Lerp(Vector) (.location (CallFunction|GetTileTransform (Variables|Default|GetOriginIndex))) (.location (CallFunction|GetTileTransform (Variables|Default|GetTargetIndex))) _loca) (Math|Vector|MakeVector 0.0 0.0 _locz)) false false))
    (:Finished
      (CallFunction|EventCompleteSpellAnim))))

(fn ConstructionScript
  (|CallParentFunction)
  (Rendering|Material|SetVectorParameterValueonMaterials (Variables|Default|GetStaticMesh) "Color" (Math|Conversions|ToVector(LinearColor) "(R=0.334918,G=0.645833,B=0.312153,A=1.000000)"))
  (Rendering|Material|SetVectorParameterValueonMaterials (Variables|Default|GetStaticMesh1) "Color" (Math|Conversions|ToVector(LinearColor) "(R=0.244777,G=0.550000,B=0.201667,A=1.000000)"))
  (Rendering|Material|SetVectorParameterValueonMaterials (Variables|Default|GetStaticMesh2) "Color" (Math|Conversions|ToVector(LinearColor) "(R=0.149427,G=0.683333,B=0.093958,A=1.000000)")))