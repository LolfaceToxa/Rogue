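; Spell animation Blueprint for Wind Gust, showing gusts blowing outward from the target tile to the other attacked tiles.
; EventPlaySpellAnim spawns a BP_AnimatedWindGust for each attacked index except the target, oriented along that direction, growing from half to full scale at a random play rate.
; A DoOnce binds only the first gust's completion delegate, which calls EventCompleteSpellAnim, so the spell completes without waiting for the other gusts.
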(event Custom|OnShapeAnimComplete
  (params (AnimatedShape :type BP%20Animated%20Wind%20Gust%20Object%20Reference))
  (CallFunction|EventCompleteSpellAnim))

(event EventBeginPlay
  (|CallParentFunction) ; This node is disabled and will not be called.\nDrag off pins to build functionality.
)

(event Collision|EventActorBeginOverlap
  (params (OtherActor :type Actor%20Object%20Reference)))

(event EventTick
  (params (DeltaSeconds :type Float%20%28single-precision%29)))

(event EventEventPlaySpellAnim
  (bind _targetindex (Variables|Default|GetTargetIndex))
  (bind _transform (CallFunction|GetTileTransform _targetindex))
  (for _array_element (Variables|Default|GetAttackedIndexes)
    (if (!= _array_element _targetindex)
      (bind _returnvalue (Game|SpawnActorfromClass "/Game/Rogue/Blueprints/Core/Combat/Spells/Anims/Components/BP_AnimatedWindGust.BP_AnimatedWindGust_C" (Math|Transform|MakeTransform "0, 0, 0" "0, 0, 0" "1.000000,1.000000,1.000000") "AlwaysSpawn" "MultiplyWithRoot" 0 (Math|Transform|MakeTransform (.location _transform) (Math|Rotator|FindLookatRotation (.location _transform) (.location (CallFunction|GetTileTransform _array_element))) "0.500000,0.500000,0.500000") (Math|Transform|MakeTransform (.location (CallFunction|GetTileTransform _array_element)) (Math|Rotator|FindLookatRotation (.location _transform) (.location (CallFunction|GetTileTransform _array_element)))) (Math|Random|RandomFloatinRange 0.8 1.5) 0))
      (Utilities|FlowControl|DoOnce false
        (:Completed
          (EventDispatchers|BindEventtoOnShapeAnimCompleted _returnvalue (delegate Custom|OnShapeAnimComplete)))))))

(fn ConstructionScript
  (|CallParentFunction))