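; Spell animation Blueprint for a short-range arrow that flies from an origin tile to a target tile on the grid.
; On play, it snaps to the origin facing the target, computing yaw from the grid indices.
; A timeline lerps it between tiles with curve-driven height, pitch and scale.
; Partway through playback it reports the tile hit once, then completes the spell animation when the timeline finishes.
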(event EventBeginPlay
  (|CallParentFunction) ; This node is disabled and will not be called.\nDrag off pins to build functionality.
)

(event EventEventPlaySpellAnim
  (Transformation|SetActorLocationAndRotation (.location (CallFunction|GetTileTransform (Variables|Default|GetOriginIndex))) (Math|Rotator|FindLookatRotation (Math|Conversions|ToVector(Vector2D) (Math|Conversions|ToVector2D(IntPoint) (Variables|Default|GetOriginIndex))) (Math|Conversions|ToVector(Vector2D) (Math|Conversions|ToVector2D(IntPoint) (Variables|Default|GetTargetIndex)))))
  (bind (_direction _actorlocalpha _locz _roty _scale) (Timeline|Timeline_Arrow PlayFromStart)
    (:Update
      (Transformation|SetActorLocation (+ (Math|Vector|Lerp(Vector) (.location (CallFunction|GetTileTransform (Variables|Default|GetOriginIndex))) (.location (CallFunction|GetTileTransform (Variables|Default|GetTargetIndex))) _actorlocalpha) (Math|Vector|MakeVector 0.0 0.0 _locz)) false false)
      (Transformation|SetRelativeRotation (Variables|Default|GetAnim_RotationScale) (Math|Rotator|MakeRotator 0.0 _roty 0.0) false false)
      (Transformation|SetRelativeScale3D (Variables|Default|GetAnim_RotationScale) (Math|Conversions|ToVector(Float) _scale))
      (if (>= (Components|Timeline|GetPlaybackPosition (Variables|Default|GetTimeline_Arrow)) 0.2)
        (Utilities|FlowControl|DoOnce false
          (:Completed
            (Default|CallOnSpellAnimHitTIle self (Variables|Default|GetTargetIndex))))))
    (:Finished
      (CallFunction|EventCompleteSpellAnim))))

(fn ConstructionScript
  (|CallParentFunction))