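; Player action for combat setup that assigns a team index to the unit standing on a targeted grid tile.
; ExecuteAction looks up the tile by index in the grid, checks that its unit is valid, then passes that unit and the action's TeamIndex to the combat system's SetUnitTeamIndex.
; The event graph holds only disabled default events.
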(event EventBeginPlay
  (|CallParentFunction) ; This node is disabled and will not be called.\nDrag off pins to build functionality.
)

(event Collision|EventActorBeginOverlap
  (params (OtherActor :type Actor%20Object%20Reference))
  (|CallParentFunction OtherActor) ; This node is disabled and will not be called.\nDrag off pins to build functionality.
)

(event EventTick
  (params (DeltaSeconds :type Float%20%28single-precision%29))
  (|CallParentFunction DeltaSeconds) ; This node is disabled and will not be called.\nDrag off pins to build functionality.
)

(fn ConstructionScript
  (|CallParentFunction))

(fn ExecuteAction
  (params (Index :type Int%20Point%20Structure))
  (bind _playeractions (Variables|Default|GetPlayerActions))
  (bind _grid (Variables|/Game/Rogue/Blueprints/Core/Player/BP_PlayerActions.BP_PlayerActions_C|GetGrid _playeractions))
  (bind _grid_tiles (Variables|/Game/Rogue/Blueprints/Core/Grid/BP_Grid.BP_Grid_C|GetGrid%20Tiles _grid))
  (bind _value (Utilities|Map|Find _grid_tiles Index))
  (bind _unitontile (Utilities|Struct|BreakS_TileData _value))
  (Utilities|IsValid _unitontile
    (:Is%20Valid
      (Default|SetUnitTeamIndex (Variables|/Game/Rogue/Blueprints/Core/Player/BP_PlayerActions.BP_PlayerActions_C|GetCombatSystem (Variables|Default|GetPlayerActions)) _unitontile (Variables|Default|GetTeamIndex)))))