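; Player action that adds or removes a unit on a grid tile during combat setup.
; When adding, it checks that the tile type is valid for the chosen unit type, removes any occupant, then spawns a BP_Unit and registers it with the combat system by team and AI flag.
; Otherwise it only removes the tile's occupant from combat, without requesting that the actor be destroyed.
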(event EventBeginPlay
  (|CallParentFunction) ; This node is disabled and will not be called.\nDrag off pins to build functionality.
)

(event Collision|EventActorBeginOverlap
  (params (OtherActor :type Actor%20Object%20Reference))
  (|CallParentFunction OtherActor) ; This node is disabled and will not be called.\nDrag off pins to build functionality.
)

(event EventTick
  (params (DeltaSeconds :type Float%20%28single-precision%29))
  (|CallParentFunction DeltaSeconds) ; This node is disabled and will not be called.\nDrag off pins to build functionality.
)

(fn ConstructionScript
  (|CallParentFunction))

(fn ExecuteAction
  (params (Index :type Int%20Point%20Structure))
  (bind _playeractions (Variables|Default|GetPlayerActions))
  (bind _grid (Variables|/Game/Rogue/Blueprints/Core/Player/BP_PlayerActions.BP_PlayerActions_C|GetGrid _playeractions))
  (bind _grid_tiles (Variables|/Game/Rogue/Blueprints/Core/Grid/BP_Grid.BP_Grid_C|GetGrid%20Tiles _grid))
  (bind _value (Utilities|Map|Find _grid_tiles Index))
  (bind _unitontile (Utilities|Struct|BreakS_TileData _value))
  (if (Variables|Default|GetisAddingUnit)
    (bind _unit_data (CallFunction|GetDefUnitDatafromUnitType (Variables|Default|GetUnitType)))
    (if (Utilities|Array|ContainsItem (.ValidTileTypes (Utilities|Struct|BreakS_UnitDataStats (.stats _unit_data))) (.type (.Value (Utilities|Map|Find (Variables|/Game/Rogue/Blueprints/Core/Grid/BP_Grid.BP_Grid_C|GetGrid%20Tiles (Variables|/Game/Rogue/Blueprints/Core/Player/BP_PlayerActions.BP_PlayerActions_C|GetGrid (Variables|Default|GetPlayerActions))) Index))))
      (Utilities|FlowControl|Sequence
        (:then_0
          (Utilities|IsValid _unitontile :!label _label
            (:Is%20Valid
              (Default|RemoveUnitfromCombat (Variables|/Game/Rogue/Blueprints/Core/Player/BP_PlayerActions.BP_PlayerActions_C|GetCombatSystem (Variables|Default|GetPlayerActions)) _unitontile false))))
        (:then_1
          (bind _returnvalue (Game|SpawnActorfromClass "/Game/Rogue/Blueprints/Core/Units/BP_Unit.BP_Unit_C" (Math|Transform|MakeTransform "0, 0, 0" "0, 0, 0" "1.000000,1.000000,1.000000") "Undefined" "OverrideRootScale" 0 (Variables|Default|GetUnitType) 0))
          (Default|AddUnitinCombat (Variables|/Game/Rogue/Blueprints/Core/Player/BP_PlayerActions.BP_PlayerActions_C|GetCombatSystem (Variables|Default|GetPlayerActions)) _returnvalue Index (Variables|Default|GetTeamIndex) (Variables|Default|GetUse%20AI)))))
    (else
      (goto _label))))