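; Player action that adds or removes units in the overworld, depending on the IsAddingUnit flag.
; When adding with a valid index, it spawns a BP_Unit of the chosen type at the cursor hit, projected onto the navmesh and raised by capsule height.
; The new unit gets its context set and joins a group through OverworldUnitGroupsManager.
; When removing, it destroys the hovered unit.
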(event EventBeginPlay
  (|CallParentFunction) ; This node is disabled and will not be called.\nDrag off pins to build functionality.
)

(event Collision|EventActorBeginOverlap
  (params (OtherActor :type Actor%20Object%20Reference))
  (|CallParentFunction OtherActor) ; This node is disabled and will not be called.\nDrag off pins to build functionality.
)

(event EventTick
  (params (DeltaSeconds :type Float%20%28single-precision%29))
  (|CallParentFunction DeltaSeconds) ; This node is disabled and will not be called.\nDrag off pins to build functionality.
)

(fn ConstructionScript
  (|CallParentFunction))

(fn ExecuteAction
  (params (Index :type Int%20Point%20Structure))
  (bind _returnvalue (Game|GetPlayerController 0))
  (bind _playeractions (Variables|Default|GetPlayerActions))
  (bind (_hitresult _returnvalue_2) (Game|Player|GetHitResultUnderCursorbyChannel _returnvalue "TraceTypeQuery3" true))
  (bind _hoveredunit (Variables|/Game/Rogue/Blueprints/Core/Player/BP_PlayerActions.BP_PlayerActions_C|GetHoveredUnit _playeractions))
  (if (Variables|Default|GetisAddingUnit)
    (if (!= Index (Utilities|Struct|MakeIntPoint -999 -999))
      (if _returnvalue_2
        (LocalVariables|SetHit%20Location (.Location (Collision|BreakHitResult _hitresult)))
        (bind _returnvalue_3 (Game|SpawnActorfromClass "/Game/Rogue/Blueprints/Core/Units/BP_Unit.BP_Unit_C" (Math|Transform|MakeTransform "0, 0, 0" "0, 0, 0" "1.000000,1.000000,1.000000") "AlwaysSpawn" "MultiplyWithRoot" 0 (Variables|Default|GetUnitType) 0))
        (bind _output_get (LocalVariables|SetUnit _returnvalue_3))
        (Transformation|SetActorLocation _output_get (Default|AddCapsuleHeight _output_get (.ProjectedLocation (AI|Navigation|ProjectPointtoNavigation (LocalVariables|GetHit%20Location) (Variables|/Game/Rogue/Blueprints/Core/Units/BP_Unit.BP_Unit_C|GetNav%20Data _output_get) 0 "0, 0, 0"))) false false)
        (Default|SetUnitContext (LocalVariables|GetUnit) "NewEnumerator1")
        (Default|AddUnittoGroup (Variables|/Game/Rogue/Blueprints/Core/Player/BP_PlayerActions.BP_PlayerActions_C|GetOverworldUnitGroupsManager (Variables|Default|GetPlayerActions)) (LocalVariables|GetUnit) (Variables|Default|GetGroupID))))
    (else
      (Utilities|IsValid _hoveredunit
        (:Is%20Valid
          (Actor|DestroyActor _hoveredunit))))))