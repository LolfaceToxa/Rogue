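; BP_UnitAI runs a unit's turn in turn-based combat as a timed sequence of AI states.
; AIPlayTurn starts a chain of events for choosing a spell, moving, casting, choosing an end position and moving there, then calls CombatSystem.NextUnit.
; Each step uses a macro that sets AIState, broadcasts OnAIStateChanged and waits DelayBetweenStates.
; The steps are placeholders, with no decision, movement or casting logic in this graph.
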(event EventBeginPlay)

(event Custom|RunAILogic
  (Utilities|SetAIStatewithDelay "NewEnumerator1"
    (:Completed
      (CallFunction|DecideWhichSpelltoCast))))

(event Custom|CastSpell
  (Utilities|SetAIStatewithDelay "NewEnumerator4"
    (:Completed
      (CallFunction|CastSpellDone))))

(event Custom|CastSpell_Done
  (CallFunction|DecideWheretoEndTurn))

(event Custom|DecideWhereToEndTurn
  (Utilities|SetAIStatewithDelay "NewEnumerator5"
    (:Completed
      (CallFunction|DecideWheretoEndTurnDone))))

(event Custom|DecideWhereToEndTurn_Done
  (CallFunction|MovetoEndTurnLoc))

(event Custom|MoveToEndTurnLoc
  (Utilities|SetAIStatewithDelay "NewEnumerator6"
    (:Completed
      (CallFunction|MovetoEndTurnLocDone))))

(event Custom|MoveToEndTurnLoc_Done
  (Utilities|SetAIStatewithDelay "NewEnumerator7"
    (:Completed
      (CallFunction|AIEndTurn))))

(event Custom|DecideWhichSpellToCast
  (Utilities|SetAIStatewithDelay "NewEnumerator2"
    (:Completed
      (CallFunction|DecideWhichSpelltoCastDone))))

(event Custom|DecideWhichSpellToCast_Done
  (CallFunction|MovetoSpellCastLoc))

(event Custom|MoveToSpellCastLoc
  (Utilities|SetAIStatewithDelay "NewEnumerator3"
    (:Completed
      (CallFunction|MovetoSpellCastLocDone))))

(event Custom|MoveToSpellCastLoc_Done
  (CallFunction|CastSpell))

(fn ConstructionScript)

(fn AIPlayTurn
  (CallFunction|RunAILogic))

(fn AIEndTurn
  (Default|NextUnit (Variables|Default|GetCombatSystem)))