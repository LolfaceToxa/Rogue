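; Manages groups of overworld units so that members share hover state and move together.
; Units join a map of groups keyed by ID, and leave on regrouping or destruction, with empty groups dropped.
; When one unit walks, encounter groups scatter around its target while others follow in a chain, and toggling encounter state halts the group.
; Hover and walk handlers briefly unbind each affected member to avoid recursive propagation.
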(event EventBeginPlay)

(event Collision|EventActorBeginOverlap
  (params (OtherActor :type Actor%20Object%20Reference)))

(event EventTick
  (params (DeltaSeconds :type Float%20%28single-precision%29)))

(fn ConstructionScript)

(fn AddUnittoGroup
  (params (UnitToAdd :type BP%20Unit%20Object%20Reference) (GroupID :type Integer))
  (if (!= GroupID (Variables|/Game/Rogue/Blueprints/Core/Units/BP_Unit.BP_Unit_C|GetOverworldGroupID UnitToAdd))
    (CallFunction|RemoveUnitfromCurGroup UnitToAdd)
    (if (!= GroupID -999)
      (bind _output_get (LocalVariables|SetGroup (.Value (Utilities|Map|Find (Variables|Default|GetUnitGroups) GroupID))))
      (Utilities|Array|Add (.Units (Utilities|Struct|BreakS_OverworldUnitGroup _output_get)) UnitToAdd)
      (Utilities|Map|Add (Variables|Default|GetUnitGroups) GroupID (LocalVariables|GetGroup))
      (Variables|/Game/Rogue/Blueprints/Core/Units/BP_Unit.BP_Unit_C|SetOverworldGroupID UnitToAdd GroupID)
      (Game|BindEventtoOnDestroyed UnitToAdd (EventDispatchers|CreateEvent :!event OnUnitDestroyed))
      (EventDispatchers|BindEventtoOnUnitHoveredChanged UnitToAdd (EventDispatchers|CreateEvent :!event OnUnitHoveredChanged))
      (EventDispatchers|BindEventtoOnUnitStartedWalkingOverworld UnitToAdd (EventDispatchers|CreateEvent :!event OnUnitStartedWalkinginOverworld)))))

(fn RemoveUnitfromCurGroup
  (params (UnitToRemove :type BP%20Unit%20Object%20Reference))
  (if (!= (Variables|/Game/Rogue/Blueprints/Core/Units/BP_Unit.BP_Unit_C|GetOverworldGroupID UnitToRemove) -999)
    (LocalVariables|SetGroup (.Value (Utilities|Map|Find (Variables|Default|GetUnitGroups) (Variables|/Game/Rogue/Blueprints/Core/Units/BP_Unit.BP_Unit_C|GetOverworldGroupID UnitToRemove))))
    (Utilities|Array|RemoveItem (Utilities|Struct|BreakS_OverworldUnitGroup (LocalVariables|GetGroup)) UnitToRemove)
    (if (> (Utilities|Array|Length (Utilities|Struct|BreakS_OverworldUnitGroup (LocalVariables|GetGroup))) 0)
      (Utilities|Map|Add (Variables|Default|GetUnitGroups) (Variables|/Game/Rogue/Blueprints/Core/Units/BP_Unit.BP_Unit_C|GetOverworldGroupID UnitToRemove) (LocalVariables|GetGroup))
      (else
        (Utilities|Map|Remove (Variables|Default|GetUnitGroups) (Variables|/Game/Rogue/Blueprints/Core/Units/BP_Unit.BP_Unit_C|GetOverworldGroupID UnitToRemove))))
    (Variables|/Game/Rogue/Blueprints/Core/Units/BP_Unit.BP_Unit_C|SetOverworldGroupID UnitToRemove -999)
    (EventDispatchers|UnbindEventfromOnUnitHoveredChanged UnitToRemove (EventDispatchers|CreateEvent :!event OnUnitHoveredChanged))
    (EventDispatchers|UnbindEventfromOnUnitStartedWalkingOverworld UnitToRemove (EventDispatchers|CreateEvent :!event OnUnitStartedWalkinginOverworld))))

(fn OnUnitDestroyed
  (params (DestroyedActor :type Actor%20Object%20Reference))
  (bind _asbp_unit (Utilities|Casting|CastToBP_Unit DestroyedActor))
  (CallFunction|RemoveUnitfromCurGroup _asbp_unit))

(fn OnUnitHoveredChanged
  (params (Cur%20Unit :type BP%20Unit%20Object%20Reference))
  (bind _unitgroups (Variables|Default|GetUnitGroups))
  (bind _overworldgroupid (Variables|/Game/Rogue/Blueprints/Core/Units/BP_Unit.BP_Unit_C|GetOverworldGroupID Cur%20Unit))
  (bind (_value _returnvalue) (Utilities|Map|Find _unitgroups _overworldgroupid))
  (if _returnvalue
    (bind _output_get (LocalVariables|SetGroup _value))
    (for _array_element (.Units (Utilities|Struct|BreakS_OverworldUnitGroup _output_get))
      (bind _output_get_2 (LocalVariables|SetU _array_element))
      (if (!= _output_get_2 Cur%20Unit)
        (EventDispatchers|UnbindEventfromOnUnitHoveredChanged (LocalVariables|GetU) (EventDispatchers|CreateEvent :!event OnUnitHoveredChanged))
        (Default|SetIsHovered (LocalVariables|GetU) (Variables|/Game/Rogue/Blueprints/Core/Units/BP_Unit.BP_Unit_C|GetIsHovered Cur%20Unit))
        (EventDispatchers|BindEventtoOnUnitHoveredChanged (LocalVariables|GetU) (EventDispatchers|CreateEvent :!event OnUnitHoveredChanged))))))

(fn OnUnitStartedWalkinginOverworld
  (params (Unit :type BP%20Unit%20Object%20Reference))
  (if (Utilities|Struct|BreakS_OverworldUnitGroup (.Value (Utilities|Map|Find (Variables|Default|GetUnitGroups) (Variables|/Game/Rogue/Blueprints/Core/Units/BP_Unit.BP_Unit_C|GetOverworldGroupID Unit))))
    (for _array_element (Utilities|Struct|BreakS_OverworldUnitGroup (.Value (Utilities|Map|Find (Variables|Default|GetUnitGroups) (Variables|/Game/Rogue/Blueprints/Core/Units/BP_Unit.BP_Unit_C|GetOverworldGroupID Unit))))
      (LocalVariables|SetU _array_element)
      (if (!= (LocalVariables|GetU) Unit)
        (EventDispatchers|UnbindEventfromOnUnitStartedWalkingOverworld (LocalVariables|GetU) (EventDispatchers|CreateEvent :!event OnUnitStartedWalkinginOverworld))
        (bind _randomlocation (Default|GetRandomReachableLocinRadius (LocalVariables|GetU) (Variables|/Game/Rogue/Blueprints/Core/Units/BP_Unit.BP_Unit_C|GetTargetLocInOverworld Unit) "(X=100.000000,Y=400.000000)"))
        (Default|EventMoveUnitinOverworld (LocalVariables|GetU) _randomlocation 0 false)
        (EventDispatchers|BindEventtoOnUnitStartedWalkingOverworld (LocalVariables|GetU) (EventDispatchers|CreateEvent :!event OnUnitStartedWalkinginOverworld))))
    (else
      (LocalVariables|SetPrevious%20Unit Unit)
      (for _array_element_2 (Utilities|Struct|BreakS_OverworldUnitGroup (.Value (Utilities|Map|Find (Variables|Default|GetUnitGroups) (Variables|/Game/Rogue/Blueprints/Core/Units/BP_Unit.BP_Unit_C|GetOverworldGroupID Unit))))
        (bind _output_get (LocalVariables|SetU _array_element_2))
        (if (!= _output_get Unit)
          (EventDispatchers|UnbindEventfromOnUnitStartedWalkingOverworld (LocalVariables|GetU) (EventDispatchers|CreateEvent :!event OnUnitStartedWalkinginOverworld))
          (Default|EventMoveUnitinOverworld (LocalVariables|GetU) "0, 0, 0" (LocalVariables|GetPrevious%20Unit) false)
          (LocalVariables|SetPrevious%20Unit (LocalVariables|GetU))
          (EventDispatchers|BindEventtoOnUnitStartedWalkingOverworld (LocalVariables|GetU) (EventDispatchers|CreateEvent :!event OnUnitStartedWalkinginOverworld)))))))

(fn SetGroupIsEncounter
  (params (IsEncounter :type Boolean) (GroupID :type Integer))
  (bind _unitgroups (Variables|Default|GetUnitGroups))
  (bind (_value _returnvalue) (Utilities|Map|Find _unitgroups GroupID))
  (if _returnvalue
    (bind _output_get (LocalVariables|SetGroup _value))
    (if (!= (Utilities|Struct|BreakS_OverworldUnitGroup _output_get) IsEncounter)
      (Utilities|Struct|SetmembersinS_OverworldUnitGroup (LocalVariables|GetGroup) IsEncounter)
      (Utilities|Map|Add (Variables|Default|GetUnitGroups) GroupID (LocalVariables|GetGroup))
      (for _array_element (.Units (Utilities|Struct|BreakS_OverworldUnitGroup (LocalVariables|GetGroup)))
        (Default|EventStopMovingUnitinOverworld _array_element))
      (if (.IsEncounter (Utilities|Struct|BreakS_OverworldUnitGroup (LocalVariables|GetGroup)))
        (Default|EventMoveUnitinOverworld (Utilities|Array|Get(acopy) (.Units (Utilities|Struct|BreakS_OverworldUnitGroup (LocalVariables|GetGroup)))) "0, 0, 0" 0 true)))))